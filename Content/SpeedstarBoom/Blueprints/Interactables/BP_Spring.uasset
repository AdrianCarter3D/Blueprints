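; BP_Spring is an interactable spring that launches BP_SpeedstarBoom on overlap.
; It stops the character's movement, then applies a velocity-change impulse so prior speed does not affect the launch.
; The impulse adds EggSpringPower on Z to the forward vector and rotates it by the actor's rotation, so it mostly follows the spring's local up axis.
; Two spring sounds play at its location with attenuation.
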(event Collision|EventActorBeginOverlap
  (params (OtherActor :type Actor%20Object%20Reference))
  (bind _returnvalue (Transformation|GetActorLocation))
  (bind _asbp_third_person_character (Utilities|Casting|CastToBP_SpeedstarBoom OtherActor))
  ;[0.4323 0.4323 0.4323] Stop players movment when in contact and then add an impulse to push the character in the direction that the spring's forward vector is facing.
  (Components|Movement|StopMovementImmediately (Variables|/Script/Engine.Character|GetCharacterMovement _asbp_third_person_character))
  (Physics|AddImpulse (Variables|/Script/Engine.Character|GetCharacterMovement _asbp_third_person_character) (Math|Vector|RotateVector (+ (Transformation|GetActorForwardVector) (Math|Vector|MakeVector 0.0 0.0 (Variables|Default|GetEgg%20Spring%20Power))) (Transformation|GetActorRotation)) true)
  ;[0.4323 0.4323 0.4323] Triggering two sounds at location
  (Audio|PlaySoundatLocation "/Game/Common/Audio/Sounds/SFX/SE_Spring.SE_Spring" _returnvalue "0, 0, 0" 1.0 1.0 0.0 "/Game/BombBombLand/Audio/Attenuation/SoundAttenuation_Normal.SoundAttenuation_Normal" 0 0 0)
  (Audio|PlaySoundatLocation "/Game/Common/Audio/Sounds/SFX/SE_Eggman_Spring.SE_Eggman_Spring" _returnvalue "0, 0, 0" 1.0 1.0 0.0 "/Game/BombBombLand/Audio/Attenuation/SoundAttenuation_Normal.SoundAttenuation_Normal" 0 0 0))

(fn ConstructionScript)