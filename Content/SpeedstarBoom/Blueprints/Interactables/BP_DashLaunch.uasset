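; BP_DashLaunch is a dash launch pad that flings the player character when they overlap it.
; The launch velocity adds the forward and up power values to the pad's forward vector, then rotates the sum by the pad's rotation.
; The launch overrides existing XY and Z velocity, and an attenuated jumpboard sound plays at the pad's location.
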(event Collision|EventActorBeginOverlap
  (params (OtherActor :type Actor%20Object%20Reference))
  (bind _returnvalue (Game|GetPlayerCharacter 0))
  (if (== OtherActor _returnvalue)
    ;[0.4323 0.4323 0.4323] Launching player based off the direction of the dash launcher. So we grab the forward vector of the pad and break that vector to move in the directions we want.
    (Character|LaunchCharacter _returnvalue (Math|Vector|RotateVector (+ (Transformation|GetActorForwardVector) (Math|Vector|MakeVector (Variables|Default|GetForwardPower) 0.0 (Variables|Default|GetUp%20Power))) (Transformation|GetActorRotation)) true true)
    (Audio|PlaySoundatLocation "/Game/Common/Audio/Sounds/SFX/SE_Jumpboard.SE_Jumpboard" (Transformation|GetActorLocation) "0, 0, 0" 1.0 1.0 0.0 "/Game/BombBombLand/Audio/Attenuation/SoundAttenuation_Normal.SoundAttenuation_Normal" 0 0 0)))

(fn ConstructionScript)