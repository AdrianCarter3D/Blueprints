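; BP_HandPully is a hand pulley that carries the BP_SpeedstarBoom character vertically when it overlaps the trigger box.
; Overlap stops the character, switches it to Flying and plays a timeline lerping the cube's height between bottom and top arrow markers.
; While grabbed, the character follows at a fixed offset below that height.
; Leaving the box restores Walking, releases the character and reverses the timeline to return the cube.
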(event OnComponentBeginOverlap(Box)
  (params (OverlappedComponent :type Primitive%20Component%20Object%20Reference) (OtherActor :type Actor%20Object%20Reference) (OtherComp :type Primitive%20Component%20Object%20Reference) (OtherBodyIndex :type Integer) (bFromSweep :type Boolean) (SweepResult :type Hit%20Result%20Structure%20%28by%20ref%29))
  (bind _cube (Variables|Default|GetCube))
  (bind _returnvalue (Transformation|GetWorldLocation _cube))
  (bind _asbp_speedstar_boom (Utilities|Casting|CastToBP_SpeedstarBoom OtherActor))
  (Pawn|Components|CharacterMovement|SetMovementMode (Variables|/Script/Engine.Character|GetCharacterMovement _asbp_speedstar_boom) "MOVE_Flying" 0)
  (Components|Movement|StopMovementImmediately (Variables|/Script/Engine.Character|GetCharacterMovement _asbp_speedstar_boom))
  (Variables|Default|SetGrabbed? true)
  (bind _handpullymovement (Timeline|Timeline Play)
    (:Update
      (Transformation|SetWorldLocation _cube (Math|Vector|MakeVector (.x _returnvalue) (.y _returnvalue) (Math|Float|Lerp (.z (Transformation|GetWorldLocation (Variables|Default|GetArrowBottom))) (.z (Transformation|GetWorldLocation (Variables|Default|GetArrowTop))) _handpullymovement)) false false)
      (if (Variables|Default|GetGrabbed?)
        (Transformation|SetActorLocation _asbp_speedstar_boom (Math|Vector|MakeVector (.x (Transformation|GetActorLocation _asbp_speedstar_boom)) (.y (Transformation|GetActorLocation _asbp_speedstar_boom)) (- (Math|Float|Lerp (.z (Transformation|GetWorldLocation (Variables|Default|GetArrowBottom))) (.z (Transformation|GetWorldLocation (Variables|Default|GetArrowTop))) _handpullymovement) 1e+02)) false false)))))

(event OnComponentEndOverlap(Box)
  (params (OverlappedComponent :type Primitive%20Component%20Object%20Reference) (OtherActor :type Actor%20Object%20Reference) (OtherComp :type Primitive%20Component%20Object%20Reference) (OtherBodyIndex :type Integer))
  (bind _cube (Variables|Default|GetCube))
  (bind _returnvalue (Transformation|GetWorldLocation _cube))
  (bind _asbp_speedstar_boom (Utilities|Casting|CastToBP_SpeedstarBoom OtherActor))
  (Pawn|Components|CharacterMovement|SetMovementMode (Variables|/Script/Engine.Character|GetCharacterMovement _asbp_speedstar_boom) "MOVE_Walking" 0)
  (Variables|Default|SetGrabbed? false)
  (bind _handpullymovement (Timeline|Timeline Reverse)
    (:Update
      (Transformation|SetWorldLocation _cube (Math|Vector|MakeVector (.x _returnvalue) (.y _returnvalue) (Math|Float|Lerp (.z (Transformation|GetWorldLocation (Variables|Default|GetArrowBottom))) (.z (Transformation|GetWorldLocation (Variables|Default|GetArrowTop))) _handpullymovement)) false false)
      (if (Variables|Default|GetGrabbed?)
        (Transformation|SetActorLocation (stale OnComponentBeginOverlap(Box) _asbp_speedstar_boom) (Math|Vector|MakeVector (.x (Transformation|GetActorLocation (stale OnComponentBeginOverlap(Box) _asbp_speedstar_boom))) (.y (Transformation|GetActorLocation (stale OnComponentBeginOverlap(Box) _asbp_speedstar_boom))) (- (Math|Float|Lerp (.z (Transformation|GetWorldLocation (Variables|Default|GetArrowBottom))) (.z (Transformation|GetWorldLocation (Variables|Default|GetArrowTop))) _handpullymovement) 1e+02)) false false)))))

(event EventBeginPlay)

(event Collision|EventActorBeginOverlap
  (params (OtherActor :type Actor%20Object%20Reference)))

(event EventTick
  (params (DeltaSeconds :type Float%20%28single-precision%29)))

(fn ConstructionScript)