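; BP_DashPanel is a boost pad that launches an overlapping BP_ThirdPersonCharacter.
; On overlap it overwrites the character's velocity with a vector built from the panel's forward direction, power and rotation, then plays a booster sound and Niagara effect.
; A separate branch, outside the cast, snaps player 0 to the panel's rotation.
; DoOnce gates limit effects and rotation until end overlap resets them after a short retriggerable delay.
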(event Collision|EventActorBeginOverlap
  (params (OtherActor :type Actor%20Object%20Reference))
  (Utilities|FlowControl|Sequence
    (:then_0
      ;[0.4323 0.4323 0.4323] On collision overlap grab character and its movement component
      (bind _asbp_third_person_character (Utilities|Casting|CastToBP_ThirdPersonCharacter OtherActor))
      ;[0.4323 0.4323 0.4323] After obtaining the characters movment component we can set the velocity of the character by checking the forward direction of the dash panel and add some power to its push.
      (Variables|/Script/Engine.MovementComponent|SetVelocity (Variables|/Script/Engine.Character|GetCharacterMovement _asbp_third_person_character) (Math|Vector|RotateVector (+ (Transformation|GetActorForwardVector) (Math|Vector|MakeVector (Variables|Default|GetDash%20Panel%20Power) 0.0 0.0)) (Transformation|GetActorRotation)))
      ;[0.4323 0.4323 0.4323] Now lets play a sound for the dash pad and spawn a visual effect by using this actors location and scale to spawn them!
      (Utilities|FlowControl|DoOnce false ; This node is nice because itll only trigger once per fire
        (:Completed
          (Audio|PlaySoundatLocation "/Game/Common/Audio/Sounds/SFX/SE_Booster.SE_Booster" (Transformation|GetActorLocation) "0, 0, 0" 1.0 1.0 0.0 "/Game/BombBombLand/Audio/Attenuation/SoundAttenuation_Loud.SoundAttenuation_Loud" 0 0 0)
          (Niagara|SpawnSystematLocation "/Game/SpeedstarBoom/Effects/NiagaraSystem_DashRamp.NiagaraSystem_DashRamp" (Transformation|GetActorLocation) "0, 0, 0" (Transformation|GetActorScale3D)))))
    (:then_1
      ;[0.4323 0.4323 0.4323] Setting player rotation to the dash pads rotation
      (Utilities|FlowControl|DoOnce false
        (:Completed
          (Transformation|SetActorRotation (Game|GetPlayerCharacter 0) (Transformation|GetActorRotation)))))))

(event Collision|EventActorEndOverlap
  (params (OtherActor :type Actor%20Object%20Reference))
  (Utilities|FlowControl|RetriggerableDelay 0.2)
  (Utilities|FlowControl|Sequence
    (:then_0
      ;[0.4323 0.4323 0.4323] Now lets play a sound for the dash pad and spawn a visual effect by using this actors location and scale to spawn them!
      (Utilities|FlowControl|DoOnce false) ; enters at Reset
    )
    (:then_1
      ;[0.4323 0.4323 0.4323] Setting player rotation to the dash pads rotation
      (Utilities|FlowControl|DoOnce false) ; enters at Reset
    )))

(fn ConstructionScript)