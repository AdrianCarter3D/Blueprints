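; BP_MoveTo is a trigger actor that switches the view to its own tracking camera when BP_SpeedstarBoom enters its box.
; Entry disables the character's input, blends the view over and starts a self-recalling delay loop that keeps the camera aimed at the character.
; Exit only re-enables input; the view and tracking are never reset.
; Despite the name, the SimpleMoveToLocation and UnPossess nodes are never run.
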(event OnComponentBeginOverlap(Box)
  (params (OverlappedComponent :type Primitive%20Component%20Object%20Reference) (OtherActor :type Actor%20Object%20Reference) (OtherComp :type Primitive%20Component%20Object%20Reference) (OtherBodyIndex :type Integer) (bFromSweep :type Boolean) (SweepResult :type Hit%20Result%20Structure%20%28by%20ref%29))
  (bind _returnvalue (Game|GetPlayerController 0))
  (bind _asbp_speedstar_boom (Utilities|Casting|CastToBP_SpeedstarBoom OtherActor))
  (Input|DisableInput _asbp_speedstar_boom _returnvalue)
  (Game|Player|SetViewTargetwithBlend _returnvalue self 1.0 "VTBlend_Linear" 0.0 false)
  (Variables|Default|SetCanTrack? true)
  (CallFunction|TrackPlayer))

(event OnComponentEndOverlap(Box)
  (params (OverlappedComponent :type Primitive%20Component%20Object%20Reference) (OtherActor :type Actor%20Object%20Reference) (OtherComp :type Primitive%20Component%20Object%20Reference) (OtherBodyIndex :type Integer))
  (bind _returnvalue (Game|GetPlayerController 0))
  (bind _asbp_speedstar_boom (Utilities|Casting|CastToBP_SpeedstarBoom OtherActor))
  (Input|EnableInput _returnvalue _returnvalue))

(event Custom|TrackPlayer
  (if (Variables|Default|GetCanTrack?)
    (Transformation|SetWorldRotation (Variables|Default|GetCamera) (Math|Rotator|FindLookatRotation (Transformation|GetWorldLocation (Variables|Default|GetCamera)) (Transformation|GetActorLocation (stale OnComponentBeginOverlap(Box) _asbp_speedstar_boom))) false false)
    (Utilities|FlowControl|Delay 0.005)
    (CallFunction|TrackPlayer)))

(fn ConstructionScript)