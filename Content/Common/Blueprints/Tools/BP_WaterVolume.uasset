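; BP_WaterVolume is a box trigger that gives the BP_SpeedstarBoom character underwater movement and visuals while inside it.
; On BeginPlay it caches the player's gravity scale, acceleration, braking deceleration and walk speed.
; Entering applies underwater values, shows its own fog and post-process, and hides the fog referenced by GameMode_Sonic.
; Leaving restores the cached movement values and swaps the visibility back.
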(event OnComponentBeginOverlap(Box)
  (params (OverlappedComponent :type Primitive%20Component%20Object%20Reference) (OtherActor :type Actor%20Object%20Reference) (OtherComp :type Primitive%20Component%20Object%20Reference) (OtherBodyIndex :type Integer) (bFromSweep :type Boolean) (SweepResult :type Hit%20Result%20Structure%20%28by%20ref%29))
  (bind _asbp_speedstar_boom (Utilities|Casting|CastToBP_SpeedstarBoom OtherActor))
  (Rendering|SetVisibility (Variables|Default|GetExponentialHeightFog) true false)
  (Rendering|SetVisibility (Variables|Default|GetPostProcess) true false)
  (bind _asgame_mode_sonic (Utilities|Casting|CastToGameMode_Sonic (Game|GetGameMode)))
  (Rendering|SetVisibility (Variables|/Script/Engine.ExponentialHeightFog|GetComponent (Variables|/Game/SpeedstarBoom/Blueprints/GameModes/GameMode_Sonic.GameMode_Sonic_C|GetExponentialHeightFog _asgame_mode_sonic)) false false)
  (Variables|/Script/Engine.CharacterMovementComponent|SetMaxAcceleration (Variables|/Script/Engine.Character|GetCharacterMovement _asbp_speedstar_boom) (Variables|Default|GetUnderwaterMaxAcceleration))
  (Variables|/Script/Engine.CharacterMovementComponent|SetBrakingDecelerationWalking (Variables|/Script/Engine.Character|GetCharacterMovement _asbp_speedstar_boom) (Variables|Default|GetUnderwaterBrakingDecelerationWalking))
  (Variables|/Script/Engine.CharacterMovementComponent|SetGravityScale (Variables|/Script/Engine.Character|GetCharacterMovement _asbp_speedstar_boom) (Variables|Default|GetUnderwaterGravityScale))
  (Variables|/Script/Engine.CharacterMovementComponent|SetMaxWalkSpeed (Variables|/Script/Engine.Character|GetCharacterMovement _asbp_speedstar_boom) (Variables|Default|GetUnderwaterMaxWalkSpeed)))

(event OnComponentEndOverlap(Box)
  (params (OverlappedComponent :type Primitive%20Component%20Object%20Reference) (OtherActor :type Actor%20Object%20Reference) (OtherComp :type Primitive%20Component%20Object%20Reference) (OtherBodyIndex :type Integer))
  (bind _asbp_speedstar_boom (Utilities|Casting|CastToBP_SpeedstarBoom OtherActor))
  (Rendering|SetVisibility (Variables|Default|GetExponentialHeightFog) false false)
  (Rendering|SetVisibility (Variables|Default|GetPostProcess) false false)
  (bind _asgame_mode_sonic (Utilities|Casting|CastToGameMode_Sonic (Game|GetGameMode)))
  (Rendering|SetVisibility (Variables|/Script/Engine.ExponentialHeightFog|GetComponent (Variables|/Game/SpeedstarBoom/Blueprints/GameModes/GameMode_Sonic.GameMode_Sonic_C|GetExponentialHeightFog _asgame_mode_sonic)) true false)
  (Variables|/Script/Engine.CharacterMovementComponent|SetMaxAcceleration (Variables|/Script/Engine.Character|GetCharacterMovement _asbp_speedstar_boom) (Variables|Default|GetMax%20Acceleration))
  (Variables|/Script/Engine.CharacterMovementComponent|SetBrakingDecelerationWalking (Variables|/Script/Engine.Character|GetCharacterMovement _asbp_speedstar_boom) (Variables|Default|GetBraking%20Deceleration%20Walking))
  (Variables|/Script/Engine.CharacterMovementComponent|SetGravityScale (Variables|/Script/Engine.Character|GetCharacterMovement _asbp_speedstar_boom) (Variables|Default|GetGravity%20Scale))
  (Variables|/Script/Engine.CharacterMovementComponent|SetMaxWalkSpeed (Variables|/Script/Engine.Character|GetCharacterMovement _asbp_speedstar_boom) (Variables|Default|GetMax%20Walk%20Speed)))

(event EventBeginPlay
  (bind _asbp_speedstar_boom (Utilities|Casting|CastToBP_SpeedstarBoom (Game|GetPlayerCharacter 0)))
  (Variables|Default|SetGravity%20Scale (Variables|/Script/Engine.CharacterMovementComponent|GetGravityScale (Variables|/Script/Engine.Character|GetCharacterMovement _asbp_speedstar_boom)))
  (Variables|Default|SetMax%20Acceleration (Variables|/Script/Engine.CharacterMovementComponent|GetMaxAcceleration (Variables|/Script/Engine.Character|GetCharacterMovement _asbp_speedstar_boom)))
  (Variables|Default|SetBraking%20Deceleration%20Walking (Variables|/Script/Engine.CharacterMovementComponent|GetBrakingDecelerationWalking (Variables|/Script/Engine.Character|GetCharacterMovement _asbp_speedstar_boom)))
  (Variables|Default|SetMax%20Walk%20Speed (Variables|/Script/Engine.CharacterMovementComponent|GetMaxWalkSpeed (Variables|/Script/Engine.Character|GetCharacterMovement _asbp_speedstar_boom))))

(fn ConstructionScript)