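; Pressure plate door prop that opens with a short camera cutaway when its OpenDoor event is called.
; The event disables player input, stops movement and blends the view to the door while a timeline lowers the cube mesh into its open position.
; After a brief delay it restores input, returns the view to the player character and turns off the mesh's collision.
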(event Custom|OpenDoor
  (bind _returnvalue (Game|GetPlayerController 0))
  (bind _returnvalue_2 (Game|GetPlayerController 0))
  (Input|DisableInput _returnvalue 0)
  (AI|Navigation|StopMovement _returnvalue)
  (Game|Player|SetViewTargetwithBlend _returnvalue self 0.0 "VTBlend_Linear" 0.0 false)
  (bind _newtrack_0 (Timeline|Timeline Play)
    (:Update
      (Transformation|SetRelativeLocation (Variables|Default|GetSM_Cube) (Math|Vector|Lerp(Vector) "0, 0, 0" "0.000000,0.000000,-250.000000" _newtrack_0) false false))
    (:Finished
      (Utilities|FlowControl|Delay 1.0)
      (Input|EnableInput _returnvalue_2 0)
      (Game|Player|SetViewTargetwithBlend _returnvalue_2 (Game|GetPlayerCharacter 0) 0.0 "VTBlend_Linear" 0.0 false)
      (Collision|SetCollisionEnabled (Variables|Default|GetSM_Cube) "NoCollision"))))

(fn ConstructionScript)