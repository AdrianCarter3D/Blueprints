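; Mario-style warp pipe prop that teleports the player to another pipe sharing its PipeID.
; Box overlap shows a prompt widget, enables input and opens a gate so Interact only works in range.
; Interact disables movement, lerps the player down between two arrows on a timeline, fades the camera, then searches all pipe actors for the match.
; The player rises from the destination pipe on a reversed timeline before walking resumes.
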(event OnComponentBeginOverlap(Box)
  (params (OverlappedComponent :type Primitive%20Component%20Object%20Reference) (OtherActor :type Actor%20Object%20Reference) (OtherComp :type Primitive%20Component%20Object%20Reference) (OtherBodyIndex :type Integer) (bFromSweep :type Boolean) (SweepResult :type Hit%20Result%20Structure%20%28by%20ref%29))
  (Variables|Default|SetREF_Player OtherActor)
  (Input|EnableInput (Game|GetPlayerController 0))
  (Rendering|SetVisibility (Variables|Default|GetWidget) true false)
  (Utilities|FlowControl|Gate true) ; enters at Open
)

(event OnComponentEndOverlap(Box)
  (params (OverlappedComponent :type Primitive%20Component%20Object%20Reference) (OtherActor :type Actor%20Object%20Reference) (OtherComp :type Primitive%20Component%20Object%20Reference) (OtherBodyIndex :type Integer))
  (bind _ref_player (Variables|Default|GetREF_Player))
  (bind _ref_player_2 (Variables|Default|GetREF_Player))
  (bind _returnvalue (Transformation|GetActorLocation _ref_player_2))
  (bind _returnvalue_2 (Transformation|GetActorLocation _ref_player))
  (Input|DisableInput (Game|GetPlayerController 0))
  (Rendering|SetVisibility (Variables|Default|GetWidget) false false)
  (Utilities|FlowControl|Gate true) ; enters at Close
)

(event EventInteract
  (bind _ref_player (Variables|Default|GetREF_Player))
  (bind _ref_player_2 (Variables|Default|GetREF_Player))
  (bind _returnvalue (Transformation|GetActorLocation _ref_player_2))
  (bind _returnvalue_2 (Transformation|GetActorLocation _ref_player))
  (Utilities|FlowControl|Gate true
    (:Exit
      ;[0.4323 0.4323 0.4323] Getting reference to any playable character
      (bind _ascharacter (Utilities|Casting|CastToCharacter (Variables|Default|GetREF_Player)))
      (bind _output_get (Variables|Default|SetREF_CurrentCharacter _ascharacter))
      (Pawn|Components|CharacterMovement|DisableMovement (Variables|/Script/Engine.Character|GetCharacterMovement _output_get)) ; Disabling movement of current character
      (Audio|PlaySoundatLocation "/Game/Common/Audio/Sounds/SFX/8d82b5_Super_Mario_Bros_Pipe_Sound_Effect.8d82b5_Super_Mario_Bros_Pipe_Sound_Effect" (Transformation|GetActorLocation) "0, 0, 0" 1.0 1.0 0.0 "/Game/BombBombLand/Audio/Attenuation/SoundAttenuation_Normal.SoundAttenuation_Normal" 0 0 0)
      ;[0.4323 0.4323 0.4323] Setting pipe transfer animation and lerping between two points being arrow top and arrow bottom.
      (bind _trackpipe (Timeline|Enter%20Pipe PlayFromStart)
        (:Update
          (Transformation|SetActorLocation _ref_player_2 (Math|Vector|MakeVector (.x _returnvalue) (.y _returnvalue) (Math|Float|Lerp (.z (Transformation|GetWorldLocation (Variables|Default|GetArrow_Top))) (.z (Transformation|GetWorldLocation (Variables|Default|GetArrow_Bottom))) _trackpipe)) false false))
        (:Finished
          ;[0.4323 0.4323 0.4323] Camera fade for transition
          (CameraFades|StartCameraFade :self (Game|GetPlayerCameraManager 0) :ToAlpha 1.0 :Duration 1.0 :bShouldFadeAudio true)
          (Utilities|FlowControl|Delay 1.0)
          ;[0.4323 0.4323 0.4323] Finding all instances of this blueprint and turning it into an array. Then with a branch looking to see what instances of this blueprint match the pipe id so we can link them and travel between.
          (bind _outactors (Actor|GetAllActorsOfClass "BP_PipeTransfer_C"))
          (bind _array_element (Utilities|Array|ForEachLoopwithBreak _outactors :!label _label)
            (:LoopBody
              (if (and (== (Variables|BP_PipeTransfer_C|GetPipeID _array_element) (Variables|Default|GetPipeID)) (!= _array_element self))
                (Utilities|FlowControl|Sequence ; Looping search for matching pipe ids
                  (:then_0
                    (goto _label Break))
                  (:then_1
                    (Transformation|SetActorLocation (Variables|Default|GetREF_Player) (Transformation|GetWorldLocation (Variables|BP_PipeTransfer_C|GetArrow_Bottom _array_element)) false false)
                    ;[0.4323 0.4323 0.4323] Camera fade for transition
                    (CameraFades|StartCameraFade :self (Game|GetPlayerCameraManager 0) :FromAlpha 1.0 :Duration 1.0 :bShouldFadeAudio true)
                    (Audio|PlaySoundatLocation "/Game/Common/Audio/Sounds/SFX/8d82b5_Super_Mario_Bros_Pipe_Sound_Effect.8d82b5_Super_Mario_Bros_Pipe_Sound_Effect" (Transformation|GetActorLocation) "0, 0, 0" 1.0 1.0 0.0 "/Game/BombBombLand/Audio/Attenuation/SoundAttenuation_Normal.SoundAttenuation_Normal" 0 0 0)
                    ;[0.4323 0.4323 0.4323] Setting animation for exiting pipe using the same arrow locations. Then on animation finished allow the player to move again.
                    (bind _trackpipe_2 (Timeline|ExitPipe ReverseFromEnd)
                      (:Update
                        (Transformation|SetActorLocation _ref_player (Math|Vector|MakeVector (.x _returnvalue_2) (.y _returnvalue_2) (Math|Float|Lerp (.z (Transformation|GetWorldLocation (Variables|BP_PipeTransfer_C|GetArrow_Top _array_element))) (.z (Transformation|GetWorldLocation (Variables|BP_PipeTransfer_C|GetArrow_Bottom _array_element))) _trackpipe_2)) false false))
                      (:Finished
                        (Pawn|Components|CharacterMovement|SetMovementMode (Variables|/Script/Engine.Character|GetCharacterMovement (Variables|Default|GetREF_CurrentCharacter)) "MOVE_Walking" 0)))))))))))))

(fn ConstructionScript)