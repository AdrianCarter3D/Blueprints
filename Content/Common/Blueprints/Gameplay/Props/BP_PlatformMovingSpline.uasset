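; Moving platform prop that carries a configurable mesh along a spline track.
; While movement is enabled, Tick advances a clamped time value by the current direction and places the platform at that point on the spline at constant velocity.
; At an endpoint it either stops or, when looping, reverses direction with an optional timed pause.
; The construction script applies mesh, scale and track duration, and previews the start position.
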(event EventTick
  (params (DeltaSeconds :type Float%20%28single-precision%29))
  (Variables|Default|SetDelta%20Seconds DeltaSeconds)
  (if (Variables|Public|GetMovePlatform)
    (Utilities|FlowControl|Sequence
      (:then_0
        (CallFunction|UpdatePlatform)
        (CallFunction|SetPlatformLocationandDirection))
      (:then_1
        (bind _lreturn (CallFunction|EndPointReached))
        (if _lreturn
          (if (Variables|Default|GetLoop)
            (Variables|Default|SetPlatformDirection (* (Variables|Default|GetPlatformDirection) -1))
            (if (Variables|Public|GetWaitAtEndpoint)
              (Variables|Public|SetMovePlatform false)
              (Utilities|FlowControl|Delay (Variables|Public|GetPlatformWaitTime))
              (CallFunction|UpdatePlatform)
              (CallFunction|SetPlatformLocationandDirection)
              (Variables|Public|SetMovePlatform true))
            (else
              (Variables|Public|SetMovePlatform false))))))))

(fn ConstructionScript
  (Components|StaticMesh|SetStaticMesh (Variables|Default|GetPlatform) (Variables|Public|GetNewMesh))
  (Transformation|SetWorldScale3D (Variables|Default|GetPlatform) (Variables|Public|GetPlatformScale))
  (Variables|/Script/Engine.SplineComponent|SetDuration (Variables|Default|GetSpline) (Variables|Public|GetTrackDuration))
  (Variables|Default|SetPlatformTime (Variables|Default|GetPlatformStartTime))
  (CallFunction|SetPlatformLocationandDirection))

(fn SetPlatformLocationandDirection
  (Transformation|SetWorldLocation (Variables|Default|GetPlatform) (Spline|GetLocationatTime (Variables|Default|GetSpline) (Variables|Default|GetPlatformTime) "World" true) false false))

(fn UpdatePlatform
  (Variables|Default|SetCachedPlatformTime (Variables|Default|GetPlatformTime))
  (Variables|Default|SetPlatformTime (Math|Float|Clamp(Float) (+ (* (Variables|Default|GetDelta%20Seconds) (Variables|Default|GetPlatformDirection)) (Variables|Default|GetPlatformTime)) 0.0 (Variables|/Script/Engine.SplineComponent|GetDuration (Variables|Default|GetSpline))))
  (return))

(fn EndPointReached
  (Math|Integer|CompareInt (Variables|Default|GetPlatformDirection)
    (:>
      (Variables|Default|SetLReturn (Math|Float|NearlyEqual(Float) (Variables|Default|GetPlatformTime) (Variables|/Script/Engine.SplineComponent|GetDuration (Variables|Default|GetSpline)) 1e-06)))
    (:<
      (Variables|Default|SetLReturn (Math|Float|NearlyEqual(Float) (Variables|Default|GetPlatformTime) 0.0 1e-06))))
  (return (Variables|Default|GetLReturn)))