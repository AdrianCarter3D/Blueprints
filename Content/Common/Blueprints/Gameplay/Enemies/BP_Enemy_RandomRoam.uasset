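; Roaming enemy with a Paper2D flipbook sprite, set at construction, that damages the player on box overlap through the player's health component.
; RandomRoam loops AI moves to random nearby reachable points, pausing randomly after each successful move.
; Non-lethal hits stop movement, launch the enemy using the hero's Directionality, then restart roaming after a delay.
; At zero health it spawns a poof effect, plays a sound and destroys itself.
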(event OnComponentBeginOverlap(Box)
  (params (OverlappedComponent :type Primitive%20Component%20Object%20Reference) (OtherActor :type Actor%20Object%20Reference) (OtherComp :type Primitive%20Component%20Object%20Reference) (OtherBodyIndex :type Integer) (bFromSweep :type Boolean) (SweepResult :type Hit%20Result%20Structure%20%28by%20ref%29))
  (bind _returnvalue (Game|GetPlayerCharacter 0))
  (if (== OtherActor _returnvalue)
    (Default|DamageCall (Actor|GetComponentbyClass _returnvalue "/Game/MythOfLegndrule/Blueprints/Player/BPComponent_HealthSystem.BPComponent_HealthSystem_C") (Variables|Default|GetDamage))))

(event Custom|RandomRoam
  (bind _returnvalue (Transformation|GetActorLocation))
  (bind _randomlocation (AI|Navigation|GetRandomReachablePointinRadius _returnvalue 5e+02 0 0))
  (AI|AIMoveTo self (Math|Vector|MakeVector (.x _randomlocation) (.y _randomlocation) 0.0) 0 5.0 false
    (:OnSuccess
      (Utilities|FlowControl|Delay (Math|Random|RandomFloatinRange (Variables|Default|GetMovementDelayMin) (Variables|Default|GetMovementDelayMax)))
      (CallFunction|RandomRoam))))

(event EventBeginPlay
  (CallFunction|RandomRoam)
  (Variables|Default|SetCurrentHealth (Variables|Default|GetMaxHealth)))

(event Game|Damage|EventAnyDamage
  (params (Damage :type Float%20%28single-precision%29) (DamageType :type Damage%20Type%20Object%20Reference) (InstigatedBy :type Controller%20Object%20Reference) (DamageCauser :type Actor%20Object%20Reference))
  (Variables|Default|SetCurrentHealth (Math|Float|Truncate (- (Variables|Default|GetCurrentHealth) Damage)))
  (if (<= (Variables|Default|GetCurrentHealth) 0)
    (Niagara|SpawnSystematLocation "/Game/MythOfLegndrule/Effects/P_Poof.P_Poof" (Transformation|GetActorLocation))
    (Audio|PlaySoundatLocation 0 (Transformation|GetActorLocation) "0, 0, 0" 1.0 1.0 0.0 0 0 0 0)
    (Actor|DestroyActor)
    (else
      (Components|Movement|StopMovementImmediately (Variables|Character|GetCharacterMovement self))
      (bind _asbp_hero (Utilities|Casting|CastToBP_Hero (Game|GetPlayerCharacter 0)))
      (Character|LaunchCharacter (Math|Vector|MakeVector (* (.X (Math|Vector2D|BreakVector2D (Variables|/Game/MythOfLegndrule/Blueprints/Player/BP_Hero.BP_Hero_C|GetDirectionality _asbp_hero))) 1e+03) (* (* (.Y (Math|Vector2D|BreakVector2D (Variables|/Game/MythOfLegndrule/Blueprints/Player/BP_Hero.BP_Hero_C|GetDirectionality _asbp_hero))) 1e+03) -1.0) 0.0) false false)
      (Audio|PlaySoundatLocation 0 (Transformation|GetActorLocation) "0, 0, 0" 1.0 1.0 0.0 0 0 0 0)
      (Utilities|FlowControl|Delay 1.5)
      (CallFunction|RandomRoam))))

(fn ConstructionScript
  (Sprite|SetFlipbook (Variables|Default|GetSprite) (Variables|Default|GetEnemy%20Flipbook)))