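; BP_Unlock is a barrier objective that registers with BP_ThirdPersonGameMode's objective count on BeginPlay and unlocks through a matching orb.
; When the player character enters its box, it loops Orbs with an empty body, then compares BlockID to the remaining element's OrbID.
; A match freezes input, plays the barrier-break sequence between camera fades, and destroys the orb.
; It then restores input, disables box collision and decrements the objective count.
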(event OnComponentBeginOverlap(Box)
  (params (OverlappedComponent :type Primitive%20Component%20Object%20Reference) (OtherActor :type Actor%20Object%20Reference) (OtherComp :type Primitive%20Component%20Object%20Reference) (OtherBodyIndex :type Integer) (bFromSweep :type Boolean) (SweepResult :type Hit%20Result%20Structure%20%28by%20ref%29))
  (bind _returnvalue (Game|GetPlayerController 0))
  (bind _returnvalue_2 (Game|GetPlayerCameraManager 0))
  (bind _asbp_third_person_character_1 (Utilities|Casting|CastToBP_ThirdPersonCharacter1 OtherActor))
  (for _array_element (Variables|Default|GetOrbs)
    _)
  (if (== (Variables|Default|GetBlockID) (Variables|/Game/BombBombLand/Blueprints/BP_OrbObjective.BP_OrbObjective_C|GetOrbID _array_element))
    (Components|Movement|StopMovementImmediately (Variables|/Script/Engine.Character|GetCharacterMovement _asbp_third_person_character_1))
    (Input|DisableInput _asbp_third_person_character_1 _returnvalue)
    (CameraFades|StartCameraFade :self _returnvalue_2 :ToAlpha 1.0 :Duration 2.0)
    (Utilities|FlowControl|Delay 2.0)
    (bind _returnvalue_3 (Sequencer|Player|CreateLevelSequencePlayer "/Game/BombBombLand/Sequencer/LVLSeq_BarrierBreak.LVLSeq_BarrierBreak"))
    (Sequencer|Player|Play _returnvalue_3 :!class /Script/MovieScene.MovieSceneSequencePlayer)
    (Utilities|FlowControl|Delay 3.0)
    (Actor|DestroyActor _array_element)
    (Utilities|FlowControl|Delay 3.0)
    (CameraFades|StartCameraFade :self _returnvalue_2 :FromAlpha 1.1 :Duration 2.0)
    (Utilities|FlowControl|Delay 2.0)
    (Input|EnableInput _asbp_third_person_character_1 _returnvalue)
    (Collision|SetCollisionEnabled (Variables|Default|GetBox) "NoCollision")
    (bind _asbp_third_person_game_mode (Utilities|Casting|CastToBP_ThirdPersonGameMode (Game|GetGameMode)))
    (Variables|/Game/BombBombLand/ThirdPerson/Blueprints/BP_ThirdPersonGameMode.BP_ThirdPersonGameMode_C|SetObjectives _asbp_third_person_game_mode (- (Variables|/Game/BombBombLand/ThirdPerson/Blueprints/BP_ThirdPersonGameMode.BP_ThirdPersonGameMode_C|GetObjectives _asbp_third_person_game_mode) 1))))

(event EventBeginPlay
  (Variables|Default|SetBlockID (Variables|Default|GetBlockID))
  (bind _returnvalue (Actor|GetActorOfClass "/Game/BombBombLand/Blueprints/BP_OrbObjective.BP_OrbObjective_C"))
  (Variables|Default|SetOrb%20ID (Variables|/Game/BombBombLand/Blueprints/BP_OrbObjective.BP_OrbObjective_C|GetOrbID _returnvalue))
  (bind _asbp_third_person_game_mode (Utilities|Casting|CastToBP_ThirdPersonGameMode (Game|GetGameMode)))
  (Variables|/Game/BombBombLand/ThirdPerson/Blueprints/BP_ThirdPersonGameMode.BP_ThirdPersonGameMode_C|SetObjectives _asbp_third_person_game_mode (+ (Variables|/Game/BombBombLand/ThirdPerson/Blueprints/BP_ThirdPersonGameMode.BP_ThirdPersonGameMode_C|GetObjectives _asbp_third_person_game_mode) 1)))

(event Collision|EventActorBeginOverlap
  (params (OtherActor :type Actor%20Object%20Reference)))

(event EventTick
  (params (DeltaSeconds :type Float%20%28single-precision%29)))

(fn ConstructionScript)