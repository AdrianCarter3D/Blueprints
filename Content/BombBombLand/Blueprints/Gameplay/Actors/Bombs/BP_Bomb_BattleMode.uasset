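; BP_Bomb_BattleMode is the battle-mode bomb actor, handling spawn overlap detection and blast pre-spawning.
; On BeginPlay, a multi box trace around the bomb collects hit actors, intended to be players standing in it, into ActorsToIgnore.
; SpawnBlast creates BP_BombBlast actors along the four horizontal axes and stores them in SpawnedBlasts.
; Pre-spawning offsets particle initialization delay so blasts appear simultaneously for all players.
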(event EventBeginPlay
  (bind _returnvalue (Transformation|GetActorLocation))
  (bind _returnvalue_2 (+ (.z _returnvalue) 5e+01))
  ;[0.1979 0.1979 0.1979] Handle Bomb collissions
  ;;[1 1 1] 1. When this actor (this bomb) gets spawned into the world, then the Beginplay event fires off a MultiBoxTrace which detects which players were in the bomb upon the bomb being spawned. Those that were get added to the actor to ignore. Once this MultiboxTrace check completed we fire off MC_Set_Collision_ActorsToIgnore
  (bind _outhits (Class|KismetSystemLibrary|BoxTraceMulti (Math|Vector|MakeVector (.x _returnvalue) (.y _returnvalue) _returnvalue_2) (Math|Vector|MakeVector (.x _returnvalue) (.y _returnvalue) _returnvalue_2) "50.000000,50.000000,50.000000" "0, 0, 0" "TraceTypeQuery1" false 0 "None" true "(R=0.000000,G=1.000000,B=0.022676,A=1.000000)"))
  (for _array_element _outhits
    (Utilities|Array|AddUnique (Variables|Default|GetActorsToIgnore) (.HitActor (Collision|BreakHitResult _array_element)))))

(fn ConstructionScript)

(fn SpawnBlast
  (bind _returnvalue (Transformation|GetActorLocation))
  ;[0.4375 0.4375 0.4375] Spawns a BombBlast_BP in 4 directions (x, x-, y, y-) and adds them to the array of [SpawnedBlasts]
  ;
  ; It's necessary that we pre-spawn these, since when the actor initializes (BombBlast_BP actor) the particle system takes a bit longer to initiate. Hence we pre-spawn these blasts so that once we set the particle to appear, it's visible to all players at the same time.
  (for _array_element (Utilities|Array|MakeArray "1.000000,0.000000,0.000000" "0.000000,1.000000,0.000000" "-1.000000,0.000000,0.000000" "0.000000,-1.000000,0.000000")
    (bind _returnvalue_2 (Game|SpawnActorfromClass "/Game/BombBombLand/Blueprints/Gameplay/Actors/Bombs/BP_BombBlast.BP_BombBlast_C" (Math|Transform|MakeTransform (Math|Vector|MakeVector (.x _returnvalue) (.y _returnvalue) (+ (.z _returnvalue) 5e+01)) (Math|Conversions|RotationFromXVector _array_element) "1.000000,1.000000,1.000000") "AlwaysSpawn" "OverrideRootScale" 0 0))
    (Utilities|Array|Add (Variables|Default|GetSpawnedBlasts) _returnvalue_2)))