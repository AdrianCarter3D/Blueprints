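; BP_LootSpawner is an unfinished loot spawner actor that contains a weighted random rarity roll.
; ChoooseRarity totals the weights in the BPInstance_Loot game instance's RarityMap, rolls within that sum, then subtracts weights until one covers the roll.
; The chosen rarity is only printed, as the return node is unwired.
; BeginPlay is empty, and the disconnected roll-and-spawn chain has unset random class options, so nothing spawns.
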(event EventBeginPlay)

(fn ConstructionScript)

(fn ChoooseRarity
  (bind _asbpinstance_loot (Utilities|Casting|CastToBPInstance_Loot (Game|GetGameInstance)))
  (bind _keys (Utilities|Map|Keys (Variables|/Game/BombBombLand/Blueprints/Loot/BPInstance_Loot.BPInstance_Loot_C|GetRarityMap _asbpinstance_loot)))
  (for _array_element _keys
    (LocalVariables|SetSum%20of%20Rarity (+ (.Value (Utilities|Map|Find (Variables|/Game/BombBombLand/Blueprints/Loot/BPInstance_Loot.BPInstance_Loot_C|GetRarityMap _asbpinstance_loot) _array_element)) (LocalVariables|GetSum%20of%20Rarity))))
  (LocalVariables|SetLootRoll (Math|Random|RandomFloatinRange 0.0 (LocalVariables|GetSum%20of%20Rarity)))
  (bind _keys_2 (Utilities|Map|Keys (Variables|/Game/BombBombLand/Blueprints/Loot/BPInstance_Loot.BPInstance_Loot_C|GetRarityMap _asbpinstance_loot)))
  (bind _array_element_2 (Utilities|Array|ForEachLoopwithBreak _keys_2 :!label _label)
    (:LoopBody
      (if (>= (.Value (Utilities|Map|Find (Variables|/Game/BombBombLand/Blueprints/Loot/BPInstance_Loot.BPInstance_Loot_C|GetRarityMap _asbpinstance_loot) _array_element_2)) (LocalVariables|GetLootRoll))
        (LocalVariables|SetRarityOut _array_element_2)
        (goto _label Break)
        (else
          (LocalVariables|SetLootRoll (- (LocalVariables|GetLootRoll) (.Value (Utilities|Map|Find (Variables|/Game/BombBombLand/Blueprints/Loot/BPInstance_Loot.BPInstance_Loot_C|GetRarityMap _asbpinstance_loot) _array_element_2)))))))
    (:Completed
      (Development|PrintString (Utilities|String|EnumtoString (LocalVariables|GetRarityOut))))))