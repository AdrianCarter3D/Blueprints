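; Blueprint function library for BombBombLand that puts transition and loading screens on the first player's viewport.
; Three functions each create a new black WB_TransitionFadeScreen and call its fade in, fade out, or fade-in-then-travel with level name and options.
; Only the travel function checks for a valid local player controller first.
; CreateLoadingScreen shows WB_LoadingScreen but never uses its text parameter.
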(fn OpenLevelFadeinTransitionScreen
  (params (LevelName :type Name) (Options :type String))
  (bind _returnvalue (Game|GetPlayerController 0))
  (Utilities|IsValid _returnvalue
    (:Is%20Valid
      (if (Pawn|IsLocalPlayerController _returnvalue)
        (bind _returnvalue_2 (UserInterface|CreateWidget "/Game/BombBombLand/Wigets/LoadingScreens/WB_TransitionFadeScreen.WB_TransitionFadeScreen_C" _returnvalue))
        (UserInterface|Viewport|AddtoViewport _returnvalue_2 0)
        (Default|FadeinTravel _returnvalue_2 LevelName Options)))))

(fn CreateLoadingScreen
  (params (LoadingScreenText :type Text))
  (bind _returnvalue (UserInterface|CreateWidget "/Game/BombBombLand/Wigets/LoadingScreens/WB_LoadingScreen.WB_LoadingScreen_C" (Game|GetPlayerController 0)))
  (UserInterface|Viewport|AddtoViewport _returnvalue 0))

(fn FadeinTransitions
  (bind _returnvalue (UserInterface|CreateWidget "/Game/BombBombLand/Wigets/LoadingScreens/WB_TransitionFadeScreen.WB_TransitionFadeScreen_C" (Game|GetPlayerController 0)))
  (UserInterface|Viewport|AddtoViewport _returnvalue 0)
  (Default|Fadein _returnvalue))

(fn FadeOutTransition
  (bind _returnvalue (UserInterface|CreateWidget "/Game/BombBombLand/Wigets/LoadingScreens/WB_TransitionFadeScreen.WB_TransitionFadeScreen_C" (Game|GetPlayerController 0)))
  (UserInterface|Viewport|AddtoViewport _returnvalue 0)
  (Default|FadeOut _returnvalue))