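; BP_TrackPlayer_Camera is a trigger-zone camera that takes over player 0's view and follows BP_ThirdPersonCharacter2 by rotating.
; Entering the Box switches the view target to this actor, prints a debug "Hello" and starts TrackPlayer.
; TrackPlayer re-aims the CineCamera at the character through a self-calling short Delay loop rather than Tick.
; Leaving the Box returns the view to the character and clears CanTrack, ending the loop.
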(event OnComponentBeginOverlap(Box)
  (params (OverlappedComponent :type Primitive%20Component%20Object%20Reference) (OtherActor :type Actor%20Object%20Reference) (OtherComp :type Primitive%20Component%20Object%20Reference) (OtherBodyIndex :type Integer) (bFromSweep :type Boolean) (SweepResult :type Hit%20Result%20Structure%20%28by%20ref%29))
  (bind _asbp_third_person_character_2 (Utilities|Casting|CastToBP_ThirdPersonCharacter2 OtherActor))
  (Game|Player|SetViewTargetwithBlend (Game|GetPlayerController 0) self 0.0 "VTBlend_Linear" 0.0 false)
  (Development|PrintString "Hello")
  (Variables|Default|SetCanTrack true)
  (CallFunction|TrackPlayer))

(event OnComponentEndOverlap(Box)
  (params (OverlappedComponent :type Primitive%20Component%20Object%20Reference) (OtherActor :type Actor%20Object%20Reference) (OtherComp :type Primitive%20Component%20Object%20Reference) (OtherBodyIndex :type Integer))
  (bind _asbp_third_person_character_2 (Utilities|Casting|CastToBP_ThirdPersonCharacter2 OtherActor))
  (Game|Player|SetViewTargetwithBlend (Game|GetPlayerController 0) _asbp_third_person_character_2 0.0 "VTBlend_Linear" 0.0 false)
  (Variables|Default|SetCanTrack false))

(event Custom|TrackPlayer
  (bind _cinecamera (Variables|Default|GetCineCamera))
  (if (Variables|Default|GetCanTrack)
    (Transformation|SetWorldRotation _cinecamera (Math|Rotator|FindLookatRotation (Transformation|GetWorldLocation _cinecamera) (Transformation|GetActorLocation (stale OnComponentBeginOverlap(Box) _asbp_third_person_character_2))) false false)
    (Utilities|FlowControl|Delay 0.005)
    (CallFunction|TrackPlayer)))

(event EventBeginPlay)

(event Collision|EventActorBeginOverlap
  (params (OtherActor :type Actor%20Object%20Reference)))

(fn ConstructionScript)