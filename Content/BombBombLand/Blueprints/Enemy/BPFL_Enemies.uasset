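; Blueprint function library for enemies, with a LootOnDeath function that picks which drops a loot table yields.
; It sums the entries' probabilities, rolls a random float up to that total, then walks the entries subtracting each weight until one covers the roll.
; The chosen entry's drops are returned, and the roll and picked table are printed on screen for debugging.
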(fn LootonDeath
  (params (LootTable :type Array%20of%20BPS%20Loot%20Table%20Array%20Structures))
  (for _array_element LootTable
    (LocalVariables|SetSumOfProbabilities (+ (.LootTableProbability (Utilities|Struct|BreakBPS_LootTableArray _array_element)) (LocalVariables|GetSumOfProbabilities))))
  (bind _output_get (LocalVariables|SetLootRoll (Math|Random|RandomFloatinRange 0.0 (LocalVariables|GetSumOfProbabilities))))
  ;[1 1 1] Debug
  (Development|PrintString 0 (Utilities|String|ToString(Float) _output_get) true true "(R=0.000000,G=1.000000,B=0.029616,A=1.000000)" 1e+01)
  (bind _array_element_2 (Utilities|Array|ForEachLoopwithBreak LootTable :!label _label)
    (:LoopBody
      (if (>= (.LootTableProbability (Utilities|Struct|BreakBPS_LootTableArray _array_element_2)) (LocalVariables|GetLootRoll))
        (LocalVariables|SetChosenTable (.LootTableDrops (Utilities|Struct|BreakBPS_LootTableArray _array_element_2)))
        (Development|PrintText 0 (.LootTable (Utilities|Struct|BreakBPS_LootTableArray _array_element_2)) true true "(R=0.783538,G=0.198069,B=0.396755,A=1.000000)" 1e+01)
        (goto _label Break)
        (else
          (LocalVariables|SetLootRoll (- (LocalVariables|GetLootRoll) (.LootTableProbability (Utilities|Struct|BreakBPS_LootTableArray _array_element_2)))))))
    (:Completed
      (return (LocalVariables|GetChosenTable)))))