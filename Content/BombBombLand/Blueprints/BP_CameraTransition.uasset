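; BP_CameraTransition is an unfinished camera transition actor whose logic is all unconnected, so it currently does nothing.
; The disconnected nodes would take the CineCamera from BP_ThirdPersonCharacter1 and ease it with VInterpTo toward the point on SplineREF's spline closest to this actor.
; A stray 0.1-second timer node is also present, while BeginPlay and the construction script are empty.
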(event EventBeginPlay)

(fn ConstructionScript)