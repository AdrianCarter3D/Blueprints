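; BP_Crates is the arena crate in BombBombLand that can leave a pickup behind when it is removed from play.
; On EndPlay it checks GMB_BomberArenaMode and skips the drop while GameSetup is set.
; Otherwise, on authority only, a weighted 20% roll spawns a random upgrade or downgrade pickup for bombs, fire power or speed at the crate's location.
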(event EventBeginPlay)

(event Collision|EventActorBeginOverlap
  (params (OtherActor :type Actor%20Object%20Reference)))

(event EventTick
  (params (DeltaSeconds :type Float%20%28single-precision%29)))

(event EventEndPlay
  (params (EndPlayReason :type EEndPlayReason%20Enum :default "Destroyed"))
  (bind _asgmb_bomber_arena_mode (Utilities|Casting|CastToGMB_BomberArenaMode (Game|GetGameMode)))
  (if (not (Variables|/Game/BombBombLand/Blueprints/GameMode/GMB_BomberArenaMode.GMB_BomberArenaMode_C|GetGameSetup _asgmb_bomber_arena_mode))
    (Networking|SwitchHasAuthority
      (:Authority
        (if (Math|Random|RandomBoolwithWeight 0.2)
          (Game|SpawnActorfromClass (.OutItem (Utilities|Array|Random (Utilities|Array|MakeArray "/Game/BombBombLand/Blueprints/Items/BP_UpgradePickup_Bomb.BP_UpgradePickup_Bomb_C" "/Game/BombBombLand/Blueprints/Items/BP_UpgradePickup_FirePow.BP_UpgradePickup_FirePow_C" "/Game/BombBombLand/Blueprints/Items/BP_UpgradePickup_Speed.BP_UpgradePickup_Speed_C" "/Game/BombBombLand/Blueprints/Items/BP_DowngradePickup_Bomb.BP_DowngradePickup_Bomb_C" "/Game/BombBombLand/Blueprints/Items/BP_DowngradePickup_FirePow.BP_DowngradePickup_FirePow_C" "/Game/BombBombLand/Blueprints/Items/BP_DowngradePickup_Speed.BP_DowngradePickup_Speed_C"))) (Math|Transform|MakeTransform (Transformation|GetActorLocation) "0, 0, 0" "1.000000,1.000000,1.000000") "Undefined" "MultiplyWithRoot" 0 0))))))

(fn ConstructionScript)