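; BP_UpgradePickup_Speed_2 is an Adventure Mode pickup that upgrades the speed of the BP_BombBombCharacter that touches it.
; On BeginPlay it picks a random direction, drifts that way on a looping timer using local offsets without sweep, and destroys itself after six seconds.
; Two of the four direction options are both +Y, so -Y never occurs.
; Overlap is handled on authority only: upgrade, 2D sound, then destroy.
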(event Custom|RandomDirection
  (Transformation|AddActorLocalOffset (Utilities|Select :Index (Variables|Default|GetRandomInt) :Option%200 "1.000000,0.000000,0.000000" :Option%201 "-1.000000,0.000000,0.000000" :Option%202 "0.000000,1.000000,0.000000" :Option%203 "0.000000,1.000000,0.000000") false false))

(event EventBeginPlay
  (|CallParentFunction)
  (Variables|Default|SetRandomInt (Math|Random|RandomIntegerinRange 0 3))
  (Utilities|Time|SetTimerbyEvent (delegate Custom|RandomDirection) 0.05 true)
  (Utilities|FlowControl|Delay 6.0)
  (Actor|DestroyActor))

(event Collision|EventActorBeginOverlap
  (params (OtherActor :type Actor%20Object%20Reference))
  (|CallParentFunction OtherActor)
  (Networking|SwitchHasAuthority
    (:Authority
      (bind _asbp_third_person_character_1 (Utilities|Casting|CastToBP_BombBombCharacter OtherActor))
      (Default|UpgradeSpeed _asbp_third_person_character_1)
      (Audio|PlaySound2D "/Game/BombBombLand/Audio/Sounds/FX/PickupSound_Cue.PickupSound_Cue" 1.0 1.0 0.0 0 0)
      (Actor|DestroyActor))))

(event EventTick
  (params (DeltaSeconds :type Float%20%28single-precision%29))
  (|CallParentFunction DeltaSeconds) ; This node is disabled and will not be called.\nDrag off pins to build functionality.
)

(fn ConstructionScript
  (|CallParentFunction))