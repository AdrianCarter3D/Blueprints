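; BP_Bullet is a projectile Blueprint that damages what it hits and can knock back 2D platformer enemies.
; When its Sphere overlaps an actor not tagged "Ignore", it spawns BP_Impact, applies its Damage value and destroys itself.
; If that actor is a BPChild_Platformer2DEnemy with Pushback enabled, it is then launched upward and along the bullet's forward X direction.
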(event OnComponentBeginOverlap(Sphere)
  (params (OverlappedComponent :type Primitive%20Component%20Object%20Reference) (OtherActor :type Actor%20Object%20Reference) (OtherComp :type Primitive%20Component%20Object%20Reference) (OtherBodyIndex :type Integer) (bFromSweep :type Boolean) (SweepResult :type Hit%20Result%20Structure%20%28by%20ref%29))
  (if (not (Actor|ActorHasTag OtherActor "Ignore"))
    (Game|SpawnActorfromClass "/Game/Assets/PaperZD/Textures/SuperVania/sprites/Fx/impact/BP_Impact.BP_Impact_C" (Transformation|GetActorTransform) "Undefined" "MultiplyWithRoot" 0 0)
    (Game|Damage|ApplyDamage OtherActor (Math|Conversions|ToFloat(Integer) (Variables|Default|GetDamage)) 0 self)
    (Actor|DestroyActor)
    (bind _asbpchild_platformer_2denemy (Utilities|Casting|CastToBPChild_Platformer2DEnemy OtherActor))
    (if (Variables|/Game/Blueprints/Core/Gameplay/Player/BP_Platformer2D.BP_Platformer2D_C|GetPushback? _asbpchild_platformer_2denemy)
      (Character|LaunchCharacter _asbpchild_platformer_2denemy (Math|Vector|MakeVector (.x (* (Transformation|GetActorForwardVector) 400)) 0.0 5e+02) true true))))

(event EventBeginPlay
  (Variables|Default|SetDamage (Variables|Default|GetDamage)))

(fn ConstructionScript)