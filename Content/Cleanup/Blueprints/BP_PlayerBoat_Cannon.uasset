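; Cannon actor for the player boat that aims at the boat's target and fires cannon shots.
; A looping timer, used in place of Tick, eases the actor's rotation toward the boat's target coordinate while the boat is aiming.
; The fire event spawns a shot at the Arrow component's transform.
; An aim query line-traces forward from the Arrow, ignoring the boat, and returns the impact point or the trace's far end.
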(event Custom|Event_UpdateAim
  (bind _returnvalue (Transformation|GetActorLocation))
  (bind _returnvalue_2 (Transformation|GetActorRotation))
  (bind _boat (Variables|Default|GetBoat))
  (bind _targetcoor (Variables|/Game/Cleanup/Blueprints/BP_Boat.BP_Boat_C|GetTargetCoor _boat))
  (bind _returnvalue_3 (Math|Rotator|FindLookatRotation _returnvalue _targetcoor))
  (bind _returnvalue_4 (Math|Interpolation|RInterpTo _returnvalue_2 _returnvalue_3 0.1 1.0))
  (bind (_roll _pitch _yaw) (Math|Rotator|BreakRotator _returnvalue_4))
  (Utilities|IsValid _boat
    (:Is%20Valid
      (if (Variables|/Game/Cleanup/Blueprints/BP_Boat.BP_Boat_C|GetAiming _boat)
        (Transformation|SetActorRotation (Math|Rotator|MakeRotator _roll _pitch _yaw))))))

(event Custom|Event_Fire
  (Game|SpawnActorfromClass "/Game/Cleanup/Blueprints/BP_PlayerCannonShot.BP_PlayerCannonShot_C" (Transformation|GetWorldTransform (Variables|Default|GetArrow)) "Undefined" "MultiplyWithRoot" 0 0))

(event EventBeginPlay
  (Utilities|Time|SetTimerbyEvent (delegate Custom|Event_UpdateAim) 0.1 true false 1.0))

(event Collision|EventActorBeginOverlap
  (params (OtherActor :type Actor%20Object%20Reference)))

(event EventTick
  (params (DeltaSeconds :type Float%20%28single-precision%29)))

(fn ConstructionScript)

(fn EventGetCannonAimDirection
  (bind _returnvalue (Math|Float|MakeLiteralFloat 3e+04))
  (bind _arrow (Variables|Default|GetArrow))
  (bind _returnvalue_2 (Math|Vector|GetForwardVector _arrow))
  (bind _returnvalue_3 (Transformation|GetWorldLocation _arrow))
  (bind _returnvalue_4 (* _returnvalue_2 _returnvalue))
  (bind _returnvalue_5 (+ _returnvalue_3 _returnvalue_4))
  (bind (_outhit _returnvalue_6) (Collision|LineTraceByChannel _returnvalue_3 _returnvalue_5 "TraceTypeQuery2" false (Utilities|Array|MakeArray (Variables|Default|GetBoat)) "None"))
  (if _returnvalue_6
    (bind _output_get (Variables|Default|SetAimDirection (.ImpactPoint (Collision|BreakHitResult _outhit))))
    (return _output_get)
    (else
      (bind _output_get_2 (Variables|Default|SetAimDirection _returnvalue_5))
      (return _output_get_2))))