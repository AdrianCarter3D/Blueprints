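; BP_NPC_Class is an NPC class that provides simple dialogue when a player interacts with it.
; On BeginPlay it picks one random entry from NPCSimpleDialogues and stores its dialogue as NPCDailyText.
; OnInteract switches the player into simple dialogue mode with this NPC, provided that text is not empty.
; A "They seem busy" HUD message exists in OnInteract but is disconnected and never runs.
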(event EventBeginPlay
  (bind _npcsimpledialogues (Variables|Default|GetNPCSimpleDialogues))
  (bind _returnvalue (Utilities|Array|Length _npcsimpledialogues))
  (if (> _returnvalue 0)
    (Variables|Default|SetNPCDailyText (Utilities|Struct|BreakStruct_SimpleDialogue (Utilities|Array|Get(acopy) _npcsimpledialogues (Math|Random|RandomIntegerinRange 0 (- _returnvalue 1)))))))

(event Collision|EventActorBeginOverlap
  (params (OtherActor :type Actor%20Object%20Reference)))

(event EventTick
  (params (DeltaSeconds :type Float%20%28single-precision%29)))

(fn ConstructionScript)

(fn OnInteract
  (params (Player :type BP%20Third%20Person%20Character%20Object%20Reference))
  (if (> (Utilities|Array|Length (Variables|Default|GetNPCDailyText)) 0)
    (Default|EventSimpleDialogueMode Player true self)))