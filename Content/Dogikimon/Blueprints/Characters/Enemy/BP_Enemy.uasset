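; BP_Enemy is an enemy character Blueprint for Dogikimon with basic health tracking.
; On BeginPlay it sets the BPHealth component's MaxHealth from HP, then copies that component's CurrentHealth into its own variable.
; AnyDamage sets the local CurrentHealth to the truncated result of Damage minus CurrentHealth (operands reversed from usual subtraction) and prints it.
; It neither writes damage back to BPHealth nor handles death.
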(event EventBeginPlay
  (bind _bp_health (Variables|Default|GetBP_Health))
  (Variables|/Game/Dogikimon/Blueprints/Characters/Enemy/BP_Health.BP_Health_C|SetMaxHealth _bp_health (Variables|Default|GetHP))
  (Variables|Default|SetCurrent%20Health (Variables|/Game/Dogikimon/Blueprints/Characters/Enemy/BP_Health.BP_Health_C|GetCurrentHealth _bp_health)))

(event Collision|EventActorBeginOverlap
  (params (OtherActor :type Actor%20Object%20Reference)))

(event EventTick
  (params (DeltaSeconds :type Float%20%28single-precision%29)))

(event Game|Damage|EventAnyDamage
  (params (Damage :type Float%20%28single-precision%29) (DamageType :type Damage%20Type%20Object%20Reference) (InstigatedBy :type Controller%20Object%20Reference) (DamageCauser :type Actor%20Object%20Reference))
  (bind _output_get (Variables|Default|SetCurrent%20Health (Math|Float|Truncate (- Damage (Variables|Default|GetCurrent%20Health)))))
  (Development|PrintString (Utilities|String|ToString(Integer) _output_get)))

(fn ConstructionScript)