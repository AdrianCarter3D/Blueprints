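; BP_Der is a player-controlled top-down character that moves and interacts with objects in the world.
; On begin play it adds the top-down Enhanced Input context and caches the GM_Digokemon game mode.
; Move input drives world-axis movement and stores the direction.
; Interact shows the first overlapping BPI_Interact actor's message on the game mode's HUD, then hides it after a retriggerable delay.
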(event Input|EnhancedActionEvents|EnhancedInputActionIA_Move
  (params (ActionValue :type Vector%202D%20Structure) (ElapsedSeconds :type Float%20%28double-precision%29) (TriggeredSeconds :type Float%20%28double-precision%29) (InputAction :type Input%20Action%20Object%20Reference :default "/Game/Dogikimon/Input/Actions/IA_Move.IA_Move"))
  (Variables|Default|SetDirectionality ActionValue)
  ;[1 1 1] Movement Left and Right
  (Pawn|Input|AddMovementInput "1.000000,0.000000,0.000000" (.X (Math|Vector2D|BreakVector2D ActionValue)) false)
  ;[1 1 1] Movement Up and Down
  (Pawn|Input|AddMovementInput "0.000000,1.000000,0.000000" (.Y (Math|Vector2D|BreakVector2D ActionValue)) false))

(event Input|EnhancedActionEvents|EnhancedInputActionIA_Interact
  (params (ActionValue :type Boolean) (ElapsedSeconds :type Float%20%28double-precision%29) (TriggeredSeconds :type Float%20%28double-precision%29) (InputAction :type Input%20Action%20Object%20Reference :default "/Game/Dogikimon/Input/Actions/IA_Interact.IA_Interact"))
  (:Started
    (bind _array_element (Utilities|Array|ForEachLoopwithBreak (Collision|GetOverlappingActors (Variables|Default|GetInteractCheck) 0 :!class /Script/Engine.PrimitiveComponent) :!label _label)
      (:LoopBody
        (if (Utilities|DoesObjectImplementInterface _array_element "/Game/Dogikimon/Blueprints/Interface/BPI_Interact.BPI_Interact_C")
          (bind _text (Class|BPIInteract|Interact(Message) _array_element))
          (Default|SetDialogueText (Variables|/Game/Dogikimon/Blueprints/GameMode/GM_Digokemon.GM_Digokemon_C|GetMainHUD (Variables|Default|GetAs%20GM%20Digokemon)) _text)
          (goto _label Break)))
      (:Completed
        (Utilities|FlowControl|RetriggerableDelay (Variables|Default|GetHideMessageDelay))
        (Default|HideMessage (Variables|/Game/Dogikimon/Blueprints/GameMode/GM_Digokemon.GM_Digokemon_C|GetMainHUD (Variables|Default|GetAs%20GM%20Digokemon)))))))

(event EventBeginPlay
  (Utilities|FlowControl|Sequence
    (:then_0
      (bind _asplayer_controller (Utilities|Casting|CastToPlayerController (Pawn|GetController)))
      (Input|AddMappingContext (PlayerController|LocalPlayerSubsystems|GetEnhancedInputLocalPlayerSubsystem _asplayer_controller) "/Game/Dogikimon/Input/IMC_TopDown.IMC_TopDown" 0 "(bIgnoreAllPressedKeysUntilRelease=True,bForceImmediately=False,bNotifyUserSettings=False)"))
    (:then_1
      (bind _asgm_digokemon (Utilities|Casting|CastToGM_Digokemon (Game|GetGameMode)))
      (Variables|Default|SetAs%20GM%20Digokemon _asgm_digokemon))))

(event Collision|EventActorBeginOverlap
  (params (OtherActor :type Actor%20Object%20Reference)))

(event EventTick
  (params (DeltaSeconds :type Float%20%28single-precision%29)))

(fn ConstructionScript)