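; Trigger volume that starts a random battle while the player stays inside its box.
; Entering the box starts a one-shot timer of random length, and leaving clears it.
; When the timer fires, it saves the player's location to BP_GameInstance_General and opens the battle map after a short delay.
; Player movement is not considered, as the velocity check is unconnected.
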(event OnComponentBeginOverlap(Box)
  (params (OverlappedComponent :type Primitive%20Component%20Object%20Reference) (OtherActor :type Actor%20Object%20Reference) (OtherComp :type Primitive%20Component%20Object%20Reference) (OtherBodyIndex :type Integer) (bFromSweep :type Boolean) (SweepResult :type Hit%20Result%20Structure%20%28by%20ref%29))
  (if (== OtherActor (Game|GetPlayerCharacter 0))
    (if (not (Variables|Default|GetRandomEncounter))
      (bind _returnvalue (Utilities|Time|SetTimerbyEvent (delegate Custom|Encounter) (Math|Random|RandomFloatinRange 1.0 15.0))))))

(event OnComponentEndOverlap(Box)
  (params (OverlappedComponent :type Primitive%20Component%20Object%20Reference) (OtherActor :type Actor%20Object%20Reference) (OtherComp :type Primitive%20Component%20Object%20Reference) (OtherBodyIndex :type Integer))
  (if (== OtherActor (Game|GetPlayerCharacter 0))
    (Variables|Default|SetRandomEncounter false)
    (Utilities|Time|ClearandInvalidateTimerbyHandle (stale OnComponentBeginOverlap(Box) _returnvalue))
    (Development|PrintString "reset")))

(event Custom|Encounter
  (Variables|Default|SetRandomEncounter true)
  (Utilities|FlowControl|Delay 0.2)
  (Development|PrintString "random encounter")
  (Variables|Default|SetRandomEncounter false)
  (bind _output_get (Variables|/Game/Common/Blueprints/Instance/BP_GameInstance_General.BP_GameInstance_General_C|SetPlayerLocation (Variables|Default|GetAs%20BP%20Game%20Instance%20General) (Transformation|GetActorLocation (Game|GetPlayerCharacter 0))))
  (Development|PrintString (Utilities|String|ToString(Vector) _output_get))
  (Game|OpenLevel(byObjectReference) "/Game/Dogikimon/Maps/BattleMap.BattleMap"))

(event EventBeginPlay
  (bind _asbp_game_instance_general (Utilities|Casting|CastToBP_GameInstance_General (Game|GetGameInstance)))
  (Variables|Default|SetAs%20BP%20Game%20Instance%20General _asbp_game_instance_general))

(event Collision|EventActorBeginOverlap
  (params (OtherActor :type Actor%20Object%20Reference)))

(event EventTick
  (params (DeltaSeconds :type Float%20%28single-precision%29)))

(fn ConstructionScript)