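; BP_EnvironmentalDamage is a hazard actor that damages the BP_PaperMarino player on overlap with its CollisionCheck component.
; A non-immune player is bounced upward, loses PlayerDamaged health, gets floating damage text overhead and is flagged immune.
; After a one-second delay it sets IsImmune to true again, never clearing it here, then opens the game-over level if health is depleted.
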(event OnComponentBeginOverlap(CollisionCheck)
  (params (OverlappedComponent :type Primitive%20Component%20Object%20Reference) (OtherActor :type Actor%20Object%20Reference) (OtherComp :type Primitive%20Component%20Object%20Reference) (OtherBodyIndex :type Integer) (bFromSweep :type Boolean) (SweepResult :type Hit%20Result%20Structure%20%28by%20ref%29))
  (bind _returnvalue (Game|GetPlayerCharacter 0))
  (bind _asbp_paper_marino (Utilities|Casting|CastToBP_PaperMarino _returnvalue))
  (if (== OtherActor _returnvalue)
    (if (not (Variables|/Game/PaperTopia/Blueprints/BP_PaperMarino.BP_PaperMarino_C|GetIsImmune _asbp_paper_marino))
      (Default|BounceUp _asbp_paper_marino "0,0,1200.000000")
      (Variables|/Game/PaperTopia/Blueprints/BP_PaperMarino.BP_PaperMarino_C|SetCurrentHealth _asbp_paper_marino (Math|Float|Truncate (- (Math|Conversions|ToFloat(Integer) (Variables|/Game/PaperTopia/Blueprints/BP_PaperMarino.BP_PaperMarino_C|GetCurrentHealth _asbp_paper_marino)) (Variables|Default|GetPlayerDamaged))))
      (bind _returnvalue_2 (Game|SpawnActorfromClass "/Game/PaperTopia/UI/BP_FloatingText_Environmental.BP_FloatingText_Environmental_C" (Math|Conversions|ToTransform(Vector) (+ (Transformation|GetActorLocation _asbp_paper_marino) "0, 0,100.000000")) "Undefined" "OverrideRootScale" 0 0))
      (Default|GetTextEnvironmental _returnvalue_2 self)
      (Variables|/Game/PaperTopia/Blueprints/BP_PaperMarino.BP_PaperMarino_C|SetIsImmune _asbp_paper_marino true)
      (Utilities|FlowControl|Delay 1.0)
      (Variables|/Game/PaperTopia/Blueprints/BP_PaperMarino.BP_PaperMarino_C|SetIsImmune _asbp_paper_marino true)
      (if (<= (Variables|/Game/PaperTopia/Blueprints/BP_PaperMarino.BP_PaperMarino_C|GetCurrentHealth _asbp_paper_marino) 0)
        (Input|DisableInput 0)
        (Game|OpenLevel(byName) "Level_GameOver")))))

(event EventBeginPlay)

(event Collision|EventActorBeginOverlap
  (params (OtherActor :type Actor%20Object%20Reference)))

(event EventTick
  (params (DeltaSeconds :type Float%20%28single-precision%29)))

(fn ConstructionScript)