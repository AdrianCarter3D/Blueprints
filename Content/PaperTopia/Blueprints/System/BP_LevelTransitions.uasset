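; BP_LevelTransitions is a trigger actor that sends the player to another level after a dialogue prompt.
; When ThirdPersonCharacter overlaps the Box, it stores its TransferID in MyGameInstance, disables character input and switches to UI-only input.
; It then shows Widget_TransitionDialogue and binds its button to an event that opens the level named by the Destination enum value.
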(event OnComponentBeginOverlap(Box)
  (params (OverlappedComponent :type Primitive%20Component%20Object%20Reference) (OtherActor :type Actor%20Object%20Reference) (OtherComp :type Primitive%20Component%20Object%20Reference) (OtherBodyIndex :type Integer) (bFromSweep :type Boolean) (SweepResult :type Hit%20Result%20Structure%20%28by%20ref%29))
  (bind _returnvalue (Game|GetPlayerController 0))
  ;[1 1 1] Level Transition and Widget
  ;;[1 1 1] Setting up level id for level transitioning
  (bind _asthird_person_character (Utilities|Casting|CastToThirdPersonCharacter OtherActor))
  (bind _asmy_game_instance (Utilities|Casting|CastToMyGameInstance (Game|GetGameInstance)))
  (Variables|/Game/PaperTopia/Blueprints/System/MyGameInstance.MyGameInstance_C|SetTransferID _asmy_game_instance (Variables|Default|GetTransferID))
  (Input|DisableInput _asthird_person_character _returnvalue)
  (Input|SetInputModeUIOnly _returnvalue 0 "DoNotLock" false)
  (bind _returnvalue_2 (UserInterface|CreateWidget "/Game/PaperTopia/UI/Widget_TransitionDialogue.Widget_TransitionDialogue_C"))
  (UserInterface|Viewport|AddtoViewport _returnvalue_2 0)
  (EventDispatchers|BindEventtoOnClicked (Variables|/Game/PaperTopia/UI/Widget_TransitionDialogue.Widget_TransitionDialogue_C|GetButton_121 _returnvalue_2) (delegate Custom|OnClickedTransition)) ; Event Dispatcher Call
)

(event Custom|OnClickedTransition
  ;[1 1 1] Level Transition and Widget
  ;;[1 1 1] Custom Event that feeds into the event dispatcher call. Listening for OnClicked event from Widget
  (Game|OpenLevel(byName) (Utilities|String|StringToName (Utilities|String|EnumtoString (Variables|Default|GetDestination)))))

(fn ConstructionScript)