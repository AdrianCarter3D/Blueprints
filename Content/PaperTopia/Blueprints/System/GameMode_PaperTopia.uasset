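; PaperTopia game mode that sets up the HUD, detects player inactivity and picks the spawn point after level transitions.
; BeginPlay creates the main HUD and a separate player stats HUD.
; Tick counts idle time and shows the animated stats once past a threshold; any key resets the timer, reverses the animation and removes that widget.
; ChoosePlayerStart matches PlayerStart tags to the game instance's TransferID, falling back to the first start.
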(event Custom|AnyKeyPressed?
  (bind _playerhud (Variables|Default|GetPlayerHUD))
  ;[1 1 1] PlayerAFK
  (Variables|Default|SetAFKTimer 0.0)
  (Class|UserWidget|PlayAnimationReverse _playerhud (Variables|/Game/PaperTopia/UI/Widget_PlayerHeadsUpDisplay.Widget_PlayerHeadsUpDisplay_C|GetAnim_CharacterStats _playerhud) 1.0 true)
  (Utilities|FlowControl|Delay 1.0)
  (Widget|RemovefromParent _playerhud))

(event EventTick
  (params (DeltaSeconds :type Float%20%28single-precision%29))
  (bind _playerhud (Variables|Default|GetPlayerHUD))
  ;[1 1 1] PlayerAFK
  (bind _output_get (Variables|Default|SetAFKTimer (+ DeltaSeconds (Variables|Default|GetAFKTimer))))
  (if (> _output_get 15.0)
    (Utilities|FlowControl|DoOnce false :!label _label
      (:Completed
        (UserInterface|Viewport|AddtoViewport _playerhud 0)
        (Default|PlayAnimCharacterStats _playerhud)))
    (else
      (goto _label Reset))))

(event EventBeginPlay
  (bind _returnvalue (UserInterface|CreateWidget "/Game/PaperTopia/UI/Widget_HUD.Widget_HUD_C"))
  (bind _output_get (Variables|Default|SetHeads%20UpDisplay _returnvalue))
  (UserInterface|Viewport|AddtoViewport _output_get 0)
  (bind _asthird_person_character (Utilities|Casting|CastToThirdPersonCharacter (Game|GetPlayerCharacter 0)))
  (Variables|Default|SetAs%20Third%20Person%20Character _asthird_person_character)
  (bind _returnvalue_2 (UserInterface|CreateWidget "/Game/PaperTopia/UI/Widget_PlayerHeadsUpDisplay.Widget_PlayerHeadsUpDisplay_C"))
  (Variables|Default|SetPlayerHUD _returnvalue_2))

(fn ConstructionScript)

(fn ChoosePlayerStart
  (params (Player :type Controller%20Object%20Reference))
  ;[1 1 1] Find the transfer id from the bp level transitions and the player tag from the player start in the levels. Choose which one to spawn in.
  (bind _asmy_game_instance (Utilities|Casting|CastToMyGameInstance (Game|GetGameInstance)))
  (bind _outactors (Actor|GetAllActorsOfClass "/Script/Engine.PlayerStart"))
  (for _array_element _outactors
    (if (Utilities|Name|Equal(Name) (Variables|/Script/Engine.PlayerStart|GetPlayerStartTag _array_element) (Variables|/Game/PaperTopia/Blueprints/System/MyGameInstance.MyGameInstance_C|GetTransferID _asmy_game_instance))
      (return _array_element)))
  (return (Utilities|Array|Get(acopy) _outactors)))