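; Game instance for PaperTopia that manages save slots, storing the player's location and level.
; LoadGame loads or creates a SaveGameObject for the named slot, which the save and load functions use to read from or write to the player character.
; It can also delete the current slot or return any slot's player data.
; AutoSaveData wraps the save, but its five-minute timer setup is unconnected and never runs.
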(event Custom|LoadGame
  (params (SaveSlotName :type String))
  (bind _output_get (Variables|Default|SetSlotSlotName SaveSlotName))
  (bind _returnvalue (SaveGame|DoesSaveGameExist _output_get))
  (if _returnvalue
    (bind _returnvalue_2 (SaveGame|LoadGamefromSlot (Variables|Default|GetSlotSlotName)))
    (bind _assave_game_object (Utilities|Casting|CastToSaveGameObject _returnvalue_2))
    (Variables|Default|SetSaveGameData _assave_game_object)
    (else
      (bind _returnvalue_3 (SaveGame|CreateSaveGameObject "/Game/PaperTopia/Blueprints/System/SaveGameObject.SaveGameObject_C"))
      (Variables|Default|SetSaveGameData _returnvalue_3))))

(fn SavePlayerData
  (bind _asthird_person_paper_topia (Utilities|Casting|CastToThirdPerson_PaperTopia (Game|GetPlayerCharacter 0)))
  (bind _output_get (LocalVariables|SetREF_Player _asthird_person_paper_topia))
  (Variables|/Game/PaperTopia/Blueprints/System/SaveGameObject.SaveGameObject_C|SetPlayerData (Variables|Default|GetSaveGameData) (Utilities|Struct|MakeStructure_PlayerSaveData (Transformation|GetActorLocation _output_get) (Variables|/Game/PaperTopia/Blueprints/ThirdPerson_PaperTopia.ThirdPerson_PaperTopia_C|GetLevel _output_get)))
  (SaveGame|SaveGametoSlot (Variables|Default|GetSaveGameData) (Variables|Default|GetSlotSlotName)))

(fn LoadPlayerData
  (bind _asthird_person_paper_topia (Utilities|Casting|CastToThirdPerson_PaperTopia (Game|GetPlayerCharacter 0)))
  (bind _output_get (LocalVariables|SetREF_Player _asthird_person_paper_topia))
  (bind _savegamedata (Variables|Default|GetSaveGameData)
    (:then
      (Transformation|SetActorLocation _output_get (.location (Variables|/Game/PaperTopia/Blueprints/System/SaveGameObject.SaveGameObject_C|GetPlayerData _savegamedata)) false false)
      (Variables|/Game/PaperTopia/Blueprints/ThirdPerson_PaperTopia.ThirdPerson_PaperTopia_C|SetLevel _output_get (.levels (Variables|/Game/PaperTopia/Blueprints/System/SaveGameObject.SaveGameObject_C|GetPlayerData _savegamedata))))
    (:else)))

(fn ClearSaveData
  (SaveGame|DeleteGameinSlot (Variables|Default|GetSlotSlotName)))

(fn AutoSaveData
  (CallFunction|SavePlayerData))

(fn RetrieveSaveData
  (params (LOCAL_SaveSlotName :type String))
  (bind _returnvalue (SaveGame|DoesSaveGameExist LOCAL_SaveSlotName))
  (if _returnvalue
    (bind _returnvalue_2 (SaveGame|LoadGamefromSlot LOCAL_SaveSlotName))
    (bind _assave_game_object (Utilities|Casting|CastToSaveGameObject _returnvalue_2))
    (return (Variables|/Game/PaperTopia/Blueprints/System/SaveGameObject.SaveGameObject_C|GetPlayerData _assave_game_object))))