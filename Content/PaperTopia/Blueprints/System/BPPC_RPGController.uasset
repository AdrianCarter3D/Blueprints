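; Player controller Blueprint for the RPG that opens the pause menu when the Menu input action is pressed.
; It creates the pause menu widget, stores it, adds it to the viewport, switches input to UI-only with the menu focused and pauses the game.
; A gamepad key check splits the flow so the mouse cursor is shown only when the menu is opened from a non-gamepad key.
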(event EventBeginPlay)

(event EventTick
  (params (DeltaSeconds :type Float%20%28single-precision%29)))

(event Input|ActionEvents|InputActionMenu
  (params (Key :type Key%20Structure))
  (:Pressed
    (if (Class|KismetInputLibrary|KeyIsGamepadKey Key)
      (bind _returnvalue (UserInterface|CreateWidget "/Game/PaperTopia/UI/Widget_PauseMenu.Widget_PauseMenu_C"))
      (bind _output_get (Variables|Default|SetPlayer%20Menu _returnvalue))
      (UserInterface|Viewport|AddtoViewport _output_get 0)
      (Input|SetInputModeUIOnly self (Variables|Default|GetPlayer%20Menu) "DoNotLock" false)
      (Game|SetGamePaused true)
      (else
        (bind _returnvalue_2 (UserInterface|CreateWidget "/Game/PaperTopia/UI/Widget_PauseMenu.Widget_PauseMenu_C"))
        (bind _output_get_2 (Variables|Default|SetPlayer%20Menu _returnvalue_2))
        (UserInterface|Viewport|AddtoViewport _output_get_2 0)
        (Input|SetInputModeUIOnly self (Variables|Default|GetPlayer%20Menu) "DoNotLock" false)
        (Variables|Default|SetbShowMouseCursor true)
        (Game|SetGamePaused true)))))

(fn ConstructionScript)