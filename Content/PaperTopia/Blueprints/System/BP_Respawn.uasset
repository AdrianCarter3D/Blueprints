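; BP_Respawn is a trigger volume that penalizes the ThirdPerson_PaperTopia character on overlapping its Box.
; It disables player input, then either opens the level named by the Levels enum if health is already zero or below, or subtracts one health and restores input after a brief delay.
; The health check precedes the decrement, and the SetActorLocation reposition node is unconnected, so the character is never moved.
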(event OnComponentBeginOverlap(Box)
  (params (OverlappedComponent :type Primitive%20Component%20Object%20Reference) (OtherActor :type Actor%20Object%20Reference) (OtherComp :type Primitive%20Component%20Object%20Reference) (OtherBodyIndex :type Integer) (bFromSweep :type Boolean) (SweepResult :type Hit%20Result%20Structure%20%28by%20ref%29))
  (bind _returnvalue (Game|GetPlayerController 0))
  (bind _asthird_person_paper_topia (Utilities|Casting|CastToThirdPerson_PaperTopia OtherActor))
  (Input|DisableInput _asthird_person_paper_topia _returnvalue)
  (if (<= (Variables|/Game/PaperTopia/Blueprints/ThirdPerson_PaperTopia.ThirdPerson_PaperTopia_C|GetCurrentHealth _asthird_person_paper_topia) 0)
    (Game|OpenLevel(byName) (Utilities|String|StringToName (Utilities|String|EnumtoString (Variables|Default|GetLevels))))
    (else
      (Variables|/Game/PaperTopia/Blueprints/ThirdPerson_PaperTopia.ThirdPerson_PaperTopia_C|SetCurrentHealth _asthird_person_paper_topia (- (Variables|/Game/PaperTopia/Blueprints/ThirdPerson_PaperTopia.ThirdPerson_PaperTopia_C|GetCurrentHealth _asthird_person_paper_topia) 1))
      (Utilities|FlowControl|Delay 0.2)
      (Input|EnableInput _asthird_person_paper_topia _returnvalue))))

(event EventBeginPlay)

(event Collision|EventActorBeginOverlap
  (params (OtherActor :type Actor%20Object%20Reference)))

(event EventTick
  (params (DeltaSeconds :type Float%20%28single-precision%29)))

(fn ConstructionScript)