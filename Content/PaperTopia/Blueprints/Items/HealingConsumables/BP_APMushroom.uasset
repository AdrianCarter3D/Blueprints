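; BP_APMushroom is a mushroom pickup that restores the player's AP.
; When its CollisionCheck component overlaps a ThirdPersonCharacter, it adds RestorativeAmount to CurrentAP, capped at MaxAP, and prints the new value on screen.
; The mushroom destroys itself on that overlap even if AP is already full, in which case it restores and prints nothing.
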(event OnComponentBeginOverlap(CollisionCheck)
  (params (OverlappedComponent :type Primitive%20Component%20Object%20Reference) (OtherActor :type Actor%20Object%20Reference) (OtherComp :type Primitive%20Component%20Object%20Reference) (OtherBodyIndex :type Integer) (bFromSweep :type Boolean) (SweepResult :type Hit%20Result%20Structure%20%28by%20ref%29))
  (bind _asthird_person_character (Utilities|Casting|CastToThirdPersonCharacter OtherActor))
  (if (>= (Variables|/Game/PaperTopia/Blueprints/ThirdPersonCharacter.ThirdPersonCharacter_C|GetCurrentAP _asthird_person_character) (Variables|/Game/PaperTopia/Blueprints/ThirdPersonCharacter.ThirdPersonCharacter_C|GetMaxAP _asthird_person_character))
    (Actor|DestroyActor)
    (else
      (bind _output_get (Variables|/Game/PaperTopia/Blueprints/ThirdPersonCharacter.ThirdPersonCharacter_C|SetCurrentAP _asthird_person_character (Math|Integer|Min(Integer) (+ (Variables|Default|GetRestorativeAmount) (Variables|/Game/PaperTopia/Blueprints/ThirdPersonCharacter.ThirdPersonCharacter_C|GetCurrentAP _asthird_person_character)) (Variables|/Game/PaperTopia/Blueprints/ThirdPersonCharacter.ThirdPersonCharacter_C|GetMaxAP _asthird_person_character))))
      (Development|PrintString (Utilities|String|ToString(Integer) _output_get) true true "(R=1.000000,G=0.957605,B=0.000000,A=1.000000)")
      (Actor|DestroyActor))))

(event EventBeginPlay
  (|CallParentFunction) ; This node is disabled and will not be called.\nDrag off pins to build functionality.
)

(event Collision|EventActorBeginOverlap
  (params (OtherActor :type Actor%20Object%20Reference))
  (|CallParentFunction OtherActor) ; This node is disabled and will not be called.\nDrag off pins to build functionality.
)

(event EventTick
  (params (DeltaSeconds :type Float%20%28single-precision%29))
  (|CallParentFunction DeltaSeconds) ; This node is disabled and will not be called.\nDrag off pins to build functionality.
)

(fn ConstructionScript
  (|CallParentFunction))