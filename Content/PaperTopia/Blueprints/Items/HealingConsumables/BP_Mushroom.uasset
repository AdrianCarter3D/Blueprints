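; BP_Mushroom is a healing consumable pickup in PaperTopia.
; When the ThirdPerson_PaperTopia character overlaps its CollisionCheck component, it adds RestorativeAmount to that character's CurrentHealth, clamped to MaxHealth, and prints the new value.
; The mushroom destroys itself on that overlap even when the character is already at full health, in which case it restores nothing.
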(event OnComponentBeginOverlap(CollisionCheck)
  (params (OverlappedComponent :type Primitive%20Component%20Object%20Reference) (OtherActor :type Actor%20Object%20Reference) (OtherComp :type Primitive%20Component%20Object%20Reference) (OtherBodyIndex :type Integer) (bFromSweep :type Boolean) (SweepResult :type Hit%20Result%20Structure%20%28by%20ref%29))
  (bind _asthird_person_paper_topia (Utilities|Casting|CastToThirdPerson_PaperTopia OtherActor))
  (if (>= (Variables|/Game/PaperTopia/Blueprints/ThirdPerson_PaperTopia.ThirdPerson_PaperTopia_C|GetCurrentHealth _asthird_person_paper_topia) (Variables|/Game/PaperTopia/Blueprints/ThirdPerson_PaperTopia.ThirdPerson_PaperTopia_C|GetMaxHealth _asthird_person_paper_topia))
    (Actor|DestroyActor)
    (else
      (bind _output_get (Variables|/Game/PaperTopia/Blueprints/ThirdPerson_PaperTopia.ThirdPerson_PaperTopia_C|SetCurrentHealth _asthird_person_paper_topia (Math|Integer|Min(Integer) (+ (Variables|Default|GetRestorativeAmount) (Variables|/Game/PaperTopia/Blueprints/ThirdPerson_PaperTopia.ThirdPerson_PaperTopia_C|GetCurrentHealth _asthird_person_paper_topia)) (Variables|/Game/PaperTopia/Blueprints/ThirdPerson_PaperTopia.ThirdPerson_PaperTopia_C|GetMaxHealth _asthird_person_paper_topia))))
      (Development|PrintString (Utilities|String|ToString(Integer) _output_get))
      (Actor|DestroyActor))))

(event EventBeginPlay
  (|CallParentFunction) ; This node is disabled and will not be called.\nDrag off pins to build functionality.
)

(event Collision|EventActorBeginOverlap
  (params (OtherActor :type Actor%20Object%20Reference))
  (|CallParentFunction OtherActor) ; This node is disabled and will not be called.\nDrag off pins to build functionality.
)

(event EventTick
  (params (DeltaSeconds :type Float%20%28single-precision%29))
  (|CallParentFunction DeltaSeconds) ; This node is disabled and will not be called.\nDrag off pins to build functionality.
)

(fn ConstructionScript
  (|CallParentFunction))