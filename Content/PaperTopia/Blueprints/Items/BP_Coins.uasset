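; BP_Coins is a coin pickup that adds to the currency of BP_PaperMarino.
; The Coin component spins by a fixed rotation step every tick, without delta-time scaling.
; When BP_PaperMarino overlaps the Sphere, it plays a 2D sound, adds CurrencyAmount to that character's Currency and destroys itself.
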(event OnComponentBeginOverlap(Sphere)
  (params (OverlappedComponent :type Primitive%20Component%20Object%20Reference) (OtherActor :type Actor%20Object%20Reference) (OtherComp :type Primitive%20Component%20Object%20Reference) (OtherBodyIndex :type Integer) (bFromSweep :type Boolean) (SweepResult :type Hit%20Result%20Structure%20%28by%20ref%29))
  (bind _asbp_paper_marino (Utilities|Casting|CastToBP_PaperMarino OtherActor))
  (Audio|PlaySound2D (Variables|Default|GetSound) 1.0 1.0 0.0 0 0)
  (Variables|/Game/PaperTopia/Blueprints/BP_PaperMarino.BP_PaperMarino_C|SetCurrency _asbp_paper_marino (+ (Variables|/Game/PaperTopia/Blueprints/BP_PaperMarino.BP_PaperMarino_C|GetCurrency _asbp_paper_marino) (Variables|Default|GetCurrencyAmount)))
  (Actor|DestroyActor))

(event EventTick
  (params (DeltaSeconds :type Float%20%28single-precision%29))
  (Transformation|AddRelativeRotation (Variables|Default|GetCoin) "0,1.000000, 0" false false))

(fn ConstructionScript)