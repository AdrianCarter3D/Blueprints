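; A shop pickup that the ThirdPersonCharacter buys automatically on overlapping its box, with sprite and price taken from a data table row.
; Construction sets the sprite; overlap shows the spinning mesh, price text and item widget, all hidden again on leaving.
; With enough Currency, it disables input, shows the sprite above the character between delays, then restores input, deducts the price and destroys itself.
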(event OnComponentBeginOverlap(Box)
  (params (OverlappedComponent :type Primitive%20Component%20Object%20Reference) (OtherActor :type Actor%20Object%20Reference) (OtherComp :type Primitive%20Component%20Object%20Reference) (OtherBodyIndex :type Integer) (bFromSweep :type Boolean) (SweepResult :type Hit%20Result%20Structure%20%28by%20ref%29))
  (bind _returnvalue (Game|GetPlayerController 0))
  (bind _papersprite (Variables|Default|GetPaperSprite))
  (bind _asthird_person_character (Utilities|Casting|CastToThirdPersonCharacter OtherActor))
  (Rendering|SetVisibility (Variables|Default|GetStaticMesh) true false)
  (Rendering|Components|TextRender|SetText (Variables|Default|GetTextRender) (Utilities|Text|ToText(Integer) (.Value (Utilities|Struct|BreakStructure_Items (stale EventBeginPlay _returnvalue)))))
  (Rendering|SetVisibility (Variables|Default|GetTextRender) true false)
  (bind _returnvalue_2 (UserInterface|CreateWidget "/Game/PaperTopia/UI/Widget_PurchasableItem.Widget_PurchasableItem_C" 0 "Header Here"))
  (UserInterface|Viewport|AddtoViewport _returnvalue_2 0)
  (if (>= (Variables|/Game/PaperTopia/Blueprints/ThirdPersonCharacter.ThirdPersonCharacter_C|GetCurrency _asthird_person_character) (.Value (Utilities|Struct|BreakStructure_Items (stale EventBeginPlay _returnvalue))))
    (Input|DisableInput _asthird_person_character _returnvalue)
    (Viewport|RemoveAllWidgets)
    (Rendering|SetVisibility _papersprite true false)
    (Rendering|SetVisibility (Variables|Default|GetStaticMesh) false false)
    (Rendering|SetVisibility (Variables|Default|GetTextRender) false false)
    (Utilities|FlowControl|Delay 1.0)
    (Transformation|SetWorldLocation (Variables|Default|GetDefaultSceneRoot) (Math|Vector|MakeVector (.x (Transformation|GetWorldLocation (Variables|/Game/PaperTopia/Blueprints/ThirdPersonCharacter.ThirdPersonCharacter_C|GetFB_Character _asthird_person_character))) (.y (Transformation|GetWorldLocation (Variables|/Game/PaperTopia/Blueprints/ThirdPersonCharacter.ThirdPersonCharacter_C|GetFB_Character _asthird_person_character))) (+ (.z (Transformation|GetWorldLocation (Variables|/Game/PaperTopia/Blueprints/ThirdPersonCharacter.ThirdPersonCharacter_C|GetFB_Character _asthird_person_character))) 8e+01)) false false)
    (Rendering|SetVisibility _papersprite true false)
    (Utilities|FlowControl|Delay 1.0)
    (Input|EnableInput _asthird_person_character _returnvalue)
    (Variables|/Game/PaperTopia/Blueprints/ThirdPersonCharacter.ThirdPersonCharacter_C|SetCurrency _asthird_person_character (- (Variables|/Game/PaperTopia/Blueprints/ThirdPersonCharacter.ThirdPersonCharacter_C|GetCurrency _asthird_person_character) (.Value (Utilities|Struct|BreakStructure_Items (stale EventBeginPlay _returnvalue)))))
    (Actor|DestroyActor)
    (else
      (bind _returnvalue_3 (UserInterface|CreateWidget "/Game/PaperTopia/UI/Widget_PurchasableItem.Widget_PurchasableItem_C" 0 "Header Here"))
      (UserInterface|Viewport|AddtoViewport _returnvalue_3 0))))

(event OnComponentEndOverlap(Box)
  (params (OverlappedComponent :type Primitive%20Component%20Object%20Reference) (OtherActor :type Actor%20Object%20Reference) (OtherComp :type Primitive%20Component%20Object%20Reference) (OtherBodyIndex :type Integer))
  (Viewport|RemoveAllWidgets)
  (Rendering|SetVisibility (Variables|Default|GetStaticMesh) false false)
  (Rendering|SetVisibility (Variables|Default|GetTextRender) false false))

(event EventBeginPlay
  (bind _items (Variables|Default|GetItems))
  (bind _item (Utilities|Struct|BreakStructure_Slots _items))
  (bind (_datatable _rowname) (Utilities|Struct|BreakDataTableRowHandle _item))
  (bind _returnvalue (Utilities|GetDataTableRow _datatable _rowname)))

(event EventTick
  (params (DeltaSeconds :type Float%20%28single-precision%29))
  (Transformation|AddLocalRotation (Variables|Default|GetStaticMesh) "0,1.000000, 0" false false))

(fn ConstructionScript
  (bind _items (Variables|Default|GetItems))
  (bind _papersprite (Variables|Default|GetPaperSprite))
  (bind _item (Utilities|Struct|BreakStructure_Slots _items))
  (bind (_datatable _rowname) (Utilities|Struct|BreakDataTableRowHandle _item))
  (bind _returnvalue (Utilities|GetDataTableRow _datatable _rowname)
    (:then
      (Rendering|Components|Sprite|SetSprite _papersprite (.Sprite (Utilities|Struct|BreakStructure_Items _returnvalue)))
      (Transformation|SetWorldRotation _papersprite "0,90.000000, 0" false false))))