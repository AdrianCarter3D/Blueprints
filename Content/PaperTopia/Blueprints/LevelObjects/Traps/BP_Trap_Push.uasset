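; BP_Trap_Push is a level trap that repeatedly moves its Scene component to push along a relative path, starting on BeginPlay.
; Smash waits a random delay, then plays a timeline that lerps the component's relative location between its origin and RelativeVector without sweeping.
; When the timeline finishes, a short pause precedes the next Smash call, so the cycle loops indefinitely with irregular timing.
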(event Custom|Smash
  (Utilities|FlowControl|Delay (Math|Random|RandomFloatinRange 0.0 4.0))
  (bind _newtrack_0 (Timeline|Timeline_0 PlayFromStart)
    (:Update
      (Transformation|SetRelativeLocation (Variables|Default|GetScene) (Math|Vector|Lerp(Vector) "0, 0, 0" (Variables|Default|GetRelativeVector) _newtrack_0) false false))
    (:Finished
      (Utilities|FlowControl|Delay 0.4)
      (CallFunction|Smash))))

(event EventBeginPlay
  (CallFunction|Smash))

(fn ConstructionScript)