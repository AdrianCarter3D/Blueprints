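; BP_DynamicMaterialTest is a test level object that animates a material parameter while the player stands in its trigger box.
; On BeginPlay it creates a dynamic material instance on the Cube from a source material.
; Player overlap plays one timeline that lerps the named scalar parameter from zero to a target value.
; Leaving plays a second timeline back to zero; both restart from the beginning, regardless of the current value.
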(event OnComponentBeginOverlap(Box)
  (params (OverlappedComponent :type Primitive%20Component%20Object%20Reference) (OtherActor :type Actor%20Object%20Reference) (OtherComp :type Primitive%20Component%20Object%20Reference) (OtherBodyIndex :type Integer) (bFromSweep :type Boolean) (SweepResult :type Hit%20Result%20Structure%20%28by%20ref%29))
  (if (== OtherActor (Game|GetPlayerCharacter 0))
    (bind _animmask (Timeline|Timeline_0 PlayFromStart)
      (:Update
        (Rendering|Material|SetScalarParameterValue (Variables|Default|GetMesh%20Material) (Variables|Default|GetParameterName) (Math|Float|Lerp 0.0 (Variables|Default|GetValue) _animmask) :!class /Script/Engine.MaterialInstanceDynamic)))))

(event OnComponentEndOverlap(Box)
  (params (OverlappedComponent :type Primitive%20Component%20Object%20Reference) (OtherActor :type Actor%20Object%20Reference) (OtherComp :type Primitive%20Component%20Object%20Reference) (OtherBodyIndex :type Integer))
  (if (== OtherActor (Game|GetPlayerCharacter 0))
    (bind _animmask (Timeline|Timeline_1 PlayFromStart)
      (:Update
        (Rendering|Material|SetScalarParameterValue (Variables|Default|GetMesh%20Material) (Variables|Default|GetParameterName) (Math|Float|Lerp (Variables|Default|GetValue) 0.0 _animmask) :!class /Script/Engine.MaterialInstanceDynamic)))))

(event EventBeginPlay
  (bind _returnvalue (Rendering|Material|CreateDynamicMaterialInstance (Variables|Default|GetCube) 0 (Variables|Default|GetSourceMaterial) "None" :!class /Script/Engine.PrimitiveComponent))
  (Variables|Default|SetMesh%20Material _returnvalue))

(fn ConstructionScript)