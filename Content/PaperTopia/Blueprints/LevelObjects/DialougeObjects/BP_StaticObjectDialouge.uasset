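; BP_StaticObjectDialouge is a level object that shows a dialogue box while the player character is near it.
; On BeginPlay it caches the Widget component's Widget_DialogueBox.
; When a ThirdPersonCharacter enters the Box trigger, it unhides the widget and passes its Text variable into the dialogue box.
; When the character leaves the trigger, it hides the widget again.
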(event OnComponentBeginOverlap(Box)
  (params (OverlappedComponent :type Primitive%20Component%20Object%20Reference) (OtherActor :type Actor%20Object%20Reference) (OtherComp :type Primitive%20Component%20Object%20Reference) (OtherBodyIndex :type Integer) (bFromSweep :type Boolean) (SweepResult :type Hit%20Result%20Structure%20%28by%20ref%29))
  (Utilities|Casting|CastToThirdPersonCharacter OtherActor)
  (Development|SetHiddeninGame (Variables|Default|GetWidget) false false)
  (Variables|/Game/PaperTopia/UI/Widget_DialogueBox.Widget_DialogueBox_C|SetDialogueText (Variables|Default|GetAs%20Widget%20Dialogue%20Box) (Variables|Default|GetText)))

(event OnComponentEndOverlap(Box)
  (params (OverlappedComponent :type Primitive%20Component%20Object%20Reference) (OtherActor :type Actor%20Object%20Reference) (OtherComp :type Primitive%20Component%20Object%20Reference) (OtherBodyIndex :type Integer))
  (Utilities|Casting|CastToThirdPersonCharacter OtherActor)
  (Development|SetHiddeninGame (Variables|Default|GetWidget) true false))

(event EventBeginPlay
  (bind _aswidget_dialogue_box (Utilities|Casting|CastToWidget_DialogueBox (UserInterface|GetWidget (Variables|Default|GetWidget))))
  (Variables|Default|SetAs%20Widget%20Dialogue%20Box _aswidget_dialogue_box))

(fn ConstructionScript)