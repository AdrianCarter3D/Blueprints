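; One-way platform that the ThirdPersonCharacter can jump up through from below and drop down through from on top.
; Overlapping the underneath trigger disables the Cube's collision, and leaving that trigger restores it.
; The above trigger enables input and opens a gate while occupied, so pressing Down there also disables the collision.
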(event OnComponentBeginOverlap(CollisionCheck_Underneath)
  (params (OverlappedComponent :type Primitive%20Component%20Object%20Reference) (OtherActor :type Actor%20Object%20Reference) (OtherComp :type Primitive%20Component%20Object%20Reference) (OtherBodyIndex :type Integer) (bFromSweep :type Boolean) (SweepResult :type Hit%20Result%20Structure%20%28by%20ref%29))
  ;[1 1 1] Jump up through platform
  (Utilities|Casting|CastToThirdPersonCharacter OtherActor)
  (Collision|SetCollisionEnabled (Variables|Default|GetCube) "NoCollision"))

(event OnComponentEndOverlap(CollisionCheck_Underneath)
  (params (OverlappedComponent :type Primitive%20Component%20Object%20Reference) (OtherActor :type Actor%20Object%20Reference) (OtherComp :type Primitive%20Component%20Object%20Reference) (OtherBodyIndex :type Integer))
  ;[1 1 1] Jump up through platform
  (Utilities|Casting|CastToThirdPersonCharacter OtherActor)
  (Collision|SetCollisionEnabled (Variables|Default|GetCube) "QueryAndPhysics"))

(event OnComponentBeginOverlap(CollisionCheck_Above)
  (params (OverlappedComponent :type Primitive%20Component%20Object%20Reference) (OtherActor :type Actor%20Object%20Reference) (OtherComp :type Primitive%20Component%20Object%20Reference) (OtherBodyIndex :type Integer) (bFromSweep :type Boolean) (SweepResult :type Hit%20Result%20Structure%20%28by%20ref%29))
  (Utilities|Casting|CastToThirdPersonCharacter OtherActor)
  (Input|EnableInput (Game|GetPlayerController 0))
  (Utilities|FlowControl|Gate true) ; enters at Open
)

(event OnComponentEndOverlap(CollisionCheck_Above)
  (params (OverlappedComponent :type Primitive%20Component%20Object%20Reference) (OtherActor :type Actor%20Object%20Reference) (OtherComp :type Primitive%20Component%20Object%20Reference) (OtherBodyIndex :type Integer))
  (Utilities|Casting|CastToThirdPersonCharacter OtherActor)
  (Input|DisableInput (Game|GetPlayerController 0))
  (Utilities|FlowControl|Gate true) ; enters at Close
)

(event Input|ActionEvents|InputActionDown
  (params (Key :type Key%20Structure))
  (:Pressed
    (Utilities|FlowControl|Gate true
      (:Exit
        (Collision|SetCollisionEnabled (Variables|Default|GetCube) "NoCollision")))))

(event Input|ActionEvents|InputActionJump
  (params (Key :type Key%20Structure)))

(fn ConstructionScript)