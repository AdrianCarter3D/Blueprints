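; BP_SpawnerPlanet is a level object that repeatedly spawns BP_RandomScalePlanet actors inside a box volume.
; The construction script sizes the box from the BoxScale variable.
; On BeginPlay it starts a looping timer whose interval is randomized once between the min and max spawn rates.
; Each tick of that timer places a planet at a random point within the box extents with a random rotation.
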(event Custom|SpawnBox
  (Game|SpawnActorfromClass "/Game/PaperTopia/Blueprints/LevelObjects/BP_RandomScalePlanet.BP_RandomScalePlanet_C" (Math|Transform|MakeTransform (Math|Random|RandomPointinBoundingBox (Transformation|GetWorldLocation (Variables|Default|GetScene)) (Components|Box|GetScaledBoxExtent (Variables|Default|GetBox))) (Math|Random|RandomRotator true) "1.000000,1.000000,1.000000") "Undefined" "OverrideRootScale" 0 0))

(event EventBeginPlay
  (Utilities|Time|SetTimerbyFunctionName 0 "SpawnBox" (Math|Random|RandomFloatinRange (Variables|Default|GetMinSpawnRate) (Variables|Default|GetMaxSpawnRate)) true))

(fn ConstructionScript
  (Transformation|SetWorldScale3D (Variables|Default|GetBox) (Variables|Default|GetBoxScale)))