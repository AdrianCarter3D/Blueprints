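; Save point actor that opens a save dialogue when the third-person character overlaps its trigger.
; The overlap disables the player's input, bobs the actor's root up and back down with latent component moves, then adds Widget_SaveDialogue to the viewport.
; Disconnected leftover logic for writing player location and a load flag to the "check" save slot never runs, so this Blueprint saves nothing itself.
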(event OnComponentBeginOverlap(Trigger)
  (params (OverlappedComponent :type Primitive%20Component%20Object%20Reference) (OtherActor :type Actor%20Object%20Reference) (OtherComp :type Primitive%20Component%20Object%20Reference) (OtherBodyIndex :type Integer) (bFromSweep :type Boolean) (SweepResult :type Hit%20Result%20Structure%20%28by%20ref%29))
  (bind _defaultsceneroot (Variables|Default|GetDefaultSceneRoot))
  (bind _returnvalue (Transformation|GetRelativeTransform _defaultsceneroot))
  (bind _asthird_person_character (Utilities|Casting|CastToThirdPersonCharacter OtherActor))
  (Input|DisableInput _asthird_person_character (Game|GetPlayerController 0))
  (Components|MoveComponentTo _defaultsceneroot (+ (.location _returnvalue) "0, 0,50.000000") (.rotation _returnvalue) false false 0.2 false)
  (Utilities|FlowControl|Delay 0.2)
  (Components|MoveComponentTo _defaultsceneroot (+ (.location _returnvalue) "0, 0,-50.000000") (.rotation _returnvalue) false false 0.1 false)
  (bind _returnvalue_2 (UserInterface|CreateWidget "/Game/PaperTopia/UI/Widget_SaveDialogue.Widget_SaveDialogue_C"))
  (UserInterface|Viewport|AddtoViewport _returnvalue_2 0))

(fn ConstructionScript)