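; BP_HealthBlock is a recovery block that restores a ThirdPersonCharacter to full health when it overlaps the Trigger.
; On overlap it disables player input, spawns heart and glitter particles, and bounces its root up and down with MoveComponentTo.
; It then refills health and returns input after a short delay.
; A final delayed "Ready" print is only a message, with no cooldown flag blocking re-triggering.
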(event OnComponentBeginOverlap(Trigger)
  (params (OverlappedComponent :type Primitive%20Component%20Object%20Reference) (OtherActor :type Actor%20Object%20Reference) (OtherComp :type Primitive%20Component%20Object%20Reference) (OtherBodyIndex :type Integer) (bFromSweep :type Boolean) (SweepResult :type Hit%20Result%20Structure%20%28by%20ref%29))
  (bind _returnvalue (Game|GetPlayerController 0))
  (bind _defaultsceneroot (Variables|Default|GetDefaultSceneRoot))
  (bind _defaultsceneroot_2 (Variables|Default|GetDefaultSceneRoot))
  (bind _returnvalue_2 (Transformation|GetRelativeTransform _defaultsceneroot))
  (bind _returnvalue_3 (Transformation|GetWorldLocation _defaultsceneroot_2))
  (bind _asthird_person_character (Utilities|Casting|CastToThirdPersonCharacter OtherActor))
  (Input|DisableInput _asthird_person_character _returnvalue)
  (Effects|SpawnEmitteratLocation "/Game/PaperTopia/Particles/Particle_RecoveryBlock_Heart.Particle_RecoveryBlock_Heart" (Transformation|GetWorldLocation (Variables|Default|GetDefaultSceneRoot)))
  (Effects|SpawnEmitteratLocation "/Game/PaperTopia/Particles/Particle_RecoveryBlock_Glitter.Particle_RecoveryBlock_Glitter" (Math|Vector|MakeVector (.x _returnvalue_3) (.y _returnvalue_3) (- (.z _returnvalue_3) 2.6e+02)))
  (Components|MoveComponentTo _defaultsceneroot (+ (.location _returnvalue_2) "0, 0,50.000000") (.rotation _returnvalue_2) false true 0.2 false)
  (Utilities|FlowControl|Delay 0.2)
  (Components|MoveComponentTo _defaultsceneroot (+ (.location _returnvalue_2) "0, 0,-50.000000") (.rotation _returnvalue_2) true false 0.1 false)
  (Variables|/Game/PaperTopia/Blueprints/ThirdPersonCharacter.ThirdPersonCharacter_C|SetCurrentHealth _asthird_person_character (Variables|/Game/PaperTopia/Blueprints/ThirdPersonCharacter.ThirdPersonCharacter_C|GetMaxHealth _asthird_person_character))
  (Utilities|FlowControl|Delay 1.0)
  (Input|EnableInput _asthird_person_character _returnvalue)
  (Utilities|FlowControl|Delay 5.0)
  (Development|PrintString "HealthBlock Ready!"))

(fn ConstructionScript)