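; Flying bat enemy that the player damages by stomping on its head.
; When a ThirdPersonCharacter overlaps the head collision while falling, the bat bounces the player upward and subtracts the player's attack power, reduced by its own defense, from its health.
; Each hit spawns floating text above the bat and prints debug health, and the bat is destroyed when health reaches zero.
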(event OnComponentBeginOverlap(Collision_Head)
  (params (OverlappedComponent :type Primitive%20Component%20Object%20Reference) (OtherActor :type Actor%20Object%20Reference) (OtherComp :type Primitive%20Component%20Object%20Reference) (OtherBodyIndex :type Integer) (bFromSweep :type Boolean) (SweepResult :type Hit%20Result%20Structure%20%28by%20ref%29))
  (bind _asthird_person_character (Utilities|Casting|CastToThirdPersonCharacter (Game|GetPlayerCharacter 0)))
  (if (and (== (Utilities|GetClass OtherActor) "/Game/PaperTopia/Blueprints/ThirdPersonCharacter.ThirdPersonCharacter_C") (< (.z (Transformation|GetVelocity _asthird_person_character)) 0.0))
    (Default|BounceUp _asthird_person_character "0,0,1200.000000")
    (bind _output_get (Variables|Default|SetTotalDamage (- (Variables|Default|GetCurrentHealth) (- (Variables|/Game/PaperTopia/Blueprints/ThirdPersonCharacter.ThirdPersonCharacter_C|GetAttackPower _asthird_person_character) (Variables|Default|GetDefense)))))
    (bind _output_get_2 (Variables|Default|SetCurrentHealth _output_get))
    (Game|SpawnActorfromClass "/Game/PaperTopia/UI/BP_FloatingText.BP_FloatingText_C" (Math|Conversions|ToTransform(Vector) (+ (Transformation|GetActorLocation) "0, 0,100.000000")) "Undefined" "OverrideRootScale" 0 0)
    (Development|PrintString (Utilities|String|ToString(Float) _output_get_2) true true "(R=1.000000,G=0.084098,B=0.000000,A=1.000000)")
    (if (<= _output_get_2 0.0)
      (Actor|DestroyActor))))

(event EventBeginPlay
  (bind _maxhealth (Variables|Default|GetMaxHealth))
  (bind _output_get (Variables|Default|SetCurrentHealth _maxhealth))
  (Development|PrintString (Utilities|String|ToString(Float) _maxhealth) true true "(R=0.109987,G=1.000000,B=0.000000,A=1.000000)")
  (Development|PrintString (Utilities|String|ToString(Float) _output_get) true true "(R=1.000000,G=0.956935,B=0.000000,A=1.000000)"))

(event Collision|EventActorBeginOverlap
  (params (OtherActor :type Actor%20Object%20Reference)))

(event EventTick
  (params (DeltaSeconds :type Float%20%28single-precision%29)))

(fn ConstructionScript)