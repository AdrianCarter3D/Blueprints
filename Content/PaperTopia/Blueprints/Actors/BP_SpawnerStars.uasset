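; BP_SpawnerStars is a spawner actor that repeatedly creates BP_RandomActor instances inside a box volume.
; BeginPlay starts a looping SpawnBox timer, picking its interval once between MinSpawnRate and MaxSpawnRate, so the rate stays fixed afterward.
; Each SpawnBox call spawns at a random point within the scaled Box extent around the Scene component's location, with fixed rotation and random uniform scale.
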(event Custom|SpawnBox
  ;[0.7799 0.09445 0.5057] Making a custom event that takes the world location and the collision box scaled boundings and spawning at a random point within the alotted space.
  (Game|SpawnActorfromClass "/Game/PaperTopia/Blueprints/Actors/BP_RandomActor.BP_RandomActor_C" (Math|Transform|MakeTransform (Math|Random|RandomPointinBoundingBox (Transformation|GetWorldLocation (Variables|Default|GetScene)) (Components|Box|GetScaledBoxExtent (Variables|Default|GetBox))) "0, 0,-145.000000" (Math|Conversions|ToVector(Float) (Math|Random|RandomFloatinRange 0.25 1.0))) "Undefined" "OverrideRootScale" 0 0))

(event EventBeginPlay
  ;[1 1 1] Calling the custom event with a timer that loops.
  (Utilities|Time|SetTimerbyFunctionName 0 "SpawnBox" (Math|Random|RandomFloatinRange (Variables|Default|GetMinSpawnRate) (Variables|Default|GetMaxSpawnRate)) true))

(fn ConstructionScript)