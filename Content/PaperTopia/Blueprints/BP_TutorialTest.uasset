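; BP_TutorialTest is a test tutorial trigger that starts a cutscene when the player character enters its Box.
; The overlap disables player input, then creates and plays NewLevelSequence, with no re-enable or one-shot guard here.
; Custom events Widget and Speech add UI to the viewport: a generic widget, and a sequencer dialogue box given speaker and line.
; Nothing here calls those events.
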(event OnComponentBeginOverlap(Box)
  (params (OverlappedComponent :type Primitive%20Component%20Object%20Reference) (OtherActor :type Actor%20Object%20Reference) (OtherComp :type Primitive%20Component%20Object%20Reference) (OtherBodyIndex :type Integer) (bFromSweep :type Boolean) (SweepResult :type Hit%20Result%20Structure%20%28by%20ref%29))
  (if (== OtherActor (Game|GetPlayerCharacter 0))
    (Input|DisableInput (Game|GetPlayerCharacter 0) (Game|GetPlayerController 0))
    (bind _outactor (Sequencer|Player|CreateLevelSequencePlayer "/Game/PaperTopia/Animations/LevelSequences/NewLevelSequence.NewLevelSequence"))
    (Sequencer|Player|Play (Variables|/Script/LevelSequence.LevelSequenceActor|GetSequencePlayer _outactor) :!class /Script/MovieScene.MovieSceneSequencePlayer)))

(event Custom|Widget
  (bind _returnvalue (UserInterface|CreateWidget "/Game/PaperTopia/Widgets/Menus/NewWidgetBlueprint.NewWidgetBlueprint_C"))
  (UserInterface|Viewport|AddtoViewport _returnvalue 0))

(event Custom|Speech
  (params (speaker :type Text) (dialogue :type Text))
  (bind _returnvalue (UserInterface|CreateWidget "/Game/MythOfLegndrule/Widgets/Menus/Widget_DialogueBoxSequencer.Widget_DialogueBoxSequencer_C" (Game|GetPlayerController 0) speaker dialogue))
  (UserInterface|Viewport|AddtoViewport _returnvalue 0))

(event EventBeginPlay)

(event Collision|EventActorBeginOverlap
  (params (OtherActor :type Actor%20Object%20Reference)))

(event EventTick
  (params (DeltaSeconds :type Float%20%28single-precision%29)))

(fn ConstructionScript)