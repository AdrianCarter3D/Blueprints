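; Enemy AI Blueprint that wanders a pawn at walk speed to random reachable points within its Battle territory.
; EnableAI, run on BeginPlay, loops a randomized pause and an AIMoveTo, using the Wait timeline's play rate to vary the delay.
; Territory comes from the Battle actor's location and scaled radius.
; The loop repeats only on successful moves, and StopAI halts both movement and timer.
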(event Custom|EnableAI
  (bind (_origin _radius) (CallFunction|GetAITerritory))
  (Variables|/Script/Engine.CharacterMovementComponent|SetMaxWalkSpeed (Variables|Character|GetCharacterMovement) (Variables|Default|GetwalkSpeed))
  (Components|Timeline|SetPlayRate (Variables|Default|GetWait) (/ 1.0 (Math|Random|RandomFloatinRange 2.0 5.0)) :!label _label)
  (Timeline|Wait PlayFromStart
    (:Finished
      (AI|AIMoveTo self (.RandomLocation (AI|Navigation|GetRandomReachablePointinRadius _origin _radius 0 0)) 0 5e+01 false
        (:OnSuccess
          (goto _label))))))

(event Custom|StopAI
  (bind (_origin _radius) (CallFunction|GetAITerritory))
  (AI|Navigation|StopMovement (AI|GetAIController self))
  (Timeline|Wait Stop
    (:Finished
      (AI|AIMoveTo self (.RandomLocation (AI|Navigation|GetRandomReachablePointinRadius _origin _radius 0 0)) 0 5e+01 false
        (:OnSuccess
          (Components|Timeline|SetPlayRate (Variables|Default|GetWait) (/ 1.0 (Math|Random|RandomFloatinRange 2.0 5.0)))
          (Timeline|Wait PlayFromStart))))))

(event EventBeginPlay
  (CallFunction|EnableAI))

(fn ConstructionScript)

(fn GetAITerritory
  (bind _battle (Variables|Default|GetBattle)
    (:then
      (return (Transformation|GetActorLocation _battle) (* (Variables|/Game/PaperTopia/Blueprints/AI/BP_BattleBase.BP_BattleBase_C|GetRadius _battle) 5e+01)))
    (:else)))