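; AI companion Blueprint for PaperTopia that joins the player on first trigger contact and then follows them.
; On first overlap by the player character, it disables their input, shows a widget, stores the character reference and marks itself joined.
; FollowPlayer re-calls itself on a short delay, moving to the character beyond PalDistance or targeting itself when closer.
; Later trigger overlaps by any actor call FollowPlayer again.
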(event OnComponentBeginOverlap(TriggerBox)
  (params (OverlappedComponent :type Primitive%20Component%20Object%20Reference) (OtherActor :type Actor%20Object%20Reference) (OtherComp :type Primitive%20Component%20Object%20Reference) (OtherBodyIndex :type Integer) (bFromSweep :type Boolean) (SweepResult :type Hit%20Result%20Structure%20%28by%20ref%29))
  (if (Variables|Default|GetHasJoined?)
    (CallFunction|FollowPlayer)
    (else
      (bind _asthird_person_paper_topia (Utilities|Casting|CastToThirdPerson_PaperTopia OtherActor))
      (Input|DisableInput _asthird_person_paper_topia (Game|GetPlayerController 0))
      (bind _returnvalue (UserInterface|CreateWidget (Variables|Default|GetClass)))
      (UserInterface|Viewport|AddtoViewport _returnvalue 0)
      (Variables|Default|SetCharacterReference _asthird_person_paper_topia)
      (CallFunction|FollowPlayer)
      (Variables|Default|SetHasJoined? true))))

(event Custom|Follow%20Player
  (bind _self self)
  (if (>= (Transformation|GetDistanceTo (Variables|Default|GetCharacterReference)) (Variables|Default|GetPalDistance))
    (AI|AIMoveTo self "0, 0, 0" (Variables|Default|GetCharacterReference) 5.0 false
      (:then
        _))
    (else
      (AI|AIMoveTo _self "0, 0, 0" _self 5.0 false
        (:then
          _))))
  (Utilities|FlowControl|Delay 0.2)
  (CallFunction|FollowPlayer))

(fn ConstructionScript)