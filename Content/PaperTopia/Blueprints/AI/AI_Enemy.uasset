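; Overworld enemy that patrols between two points and starts a battle when the player touches or stomps it.
; Sighting the player shows a reaction widget and starts a chase, while a retriggerable delay returns it to patrol once sight lapses.
; A capsule hit or downward box overlap, which also bounces the player, freezes the player, shows a transition widget and opens the Destination level.
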(event OnComponentHit(CapsuleComponent)
  (params (HitComponent :type Primitive%20Component%20Object%20Reference) (OtherActor :type Actor%20Object%20Reference) (OtherComp :type Primitive%20Component%20Object%20Reference) (NormalImpulse :type Vector :default "0, 0, 0") (Hit :type Hit%20Result%20Structure%20%28by%20ref%29))
  (Utilities|FlowControl|DoOnce false
    (:Completed
      (bind _asthird_person_character (Utilities|Casting|CastToThirdPersonCharacter OtherActor))
      (Collision|SetCollisionEnabled (Variables|Default|GetBox) "NoCollision")
      (Input|DisableInput _asthird_person_character (Game|GetPlayerController 0))
      (bind _returnvalue (AddComponent|AddAudioComponent false))
      (Audio|Components|Audio|FadeOut _returnvalue 2.5 0.0 "Linear" :!class /Script/Engine.AudioComponent)
      (Utilities|FlowControl|Delay 0.4)
      (Pawn|Components|CharacterMovement|SetMovementMode (Variables|/Script/Engine.Character|GetCharacterMovement _asthird_person_character) "MOVE_None" 0)
      (bind _returnvalue_2 (UserInterface|CreateWidget "/Game/PaperTopia/UI/Widget_BattleTransition.Widget_BattleTransition_C"))
      (UserInterface|Viewport|AddtoViewport _returnvalue_2 0)
      (Utilities|FlowControl|Delay 2.0)
      (Game|OpenLevel(byName) (Utilities|String|StringToName (Utilities|String|EnumtoString (Variables|Default|GetDestination))))
      (Actor|DestroyActor))))

(event OnSeePawn(PawnSensing)
  (params (Pawn :type Pawn%20Object%20Reference))
  (bind _asthird_person_character (Utilities|Casting|CastToThirdPersonCharacter Pawn))
  (Utilities|FlowControl|Sequence
    (:then_0
      (Variables|Default|SetSeeEnemy? true)
      (AI|AIMoveTo self "0, 0, 0" _asthird_person_character 5.0 false
        (:then
          (Rendering|SetVisibility (Variables|Default|GetWidgetComponent_Reaction) true false))))
    (:then_1
      (Utilities|FlowControl|RetriggerableDelay 0.6)
      (Variables|Default|SetSeeEnemy? false)
      (Components|Movement|StopMovementImmediately (Variables|Character|GetCharacterMovement))
      (Rendering|SetVisibility (Variables|Default|GetWidgetComponent_Reaction) false false)
      (CallFunction|Patrol))))

(event OnComponentBeginOverlap(Box)
  (params (OverlappedComponent :type Primitive%20Component%20Object%20Reference) (OtherActor :type Actor%20Object%20Reference) (OtherComp :type Primitive%20Component%20Object%20Reference) (OtherBodyIndex :type Integer) (bFromSweep :type Boolean) (SweepResult :type Hit%20Result%20Structure%20%28by%20ref%29))
  (bind _asthird_person_character (Utilities|Casting|CastToThirdPersonCharacter OtherActor))
  (if (and (== (Utilities|GetClass OtherActor) "/Game/PaperTopia/Blueprints/ThirdPersonCharacter.ThirdPersonCharacter_C") (< (.z (Transformation|GetVelocity _asthird_person_character)) 0.0))
    (Default|BounceUp _asthird_person_character (Math|Vector|MakeVector 0.0 0.0 (.z (Variables|Default|GetBounce%20Intensity))))
    (Collision|SetCollisionEnabled (Variables|Default|GetBox) "NoCollision")
    (Input|DisableInput _asthird_person_character (Game|GetPlayerController 0))
    (Utilities|FlowControl|Delay 0.4)
    (Pawn|Components|CharacterMovement|SetMovementMode (Variables|/Script/Engine.Character|GetCharacterMovement _asthird_person_character) "MOVE_None" 0)
    (bind _returnvalue (UserInterface|CreateWidget "/Game/PaperTopia/UI/Widget_BattleTransition.Widget_BattleTransition_C"))
    (UserInterface|Viewport|AddtoViewport _returnvalue 0)
    (Utilities|FlowControl|Delay 2.0)
    (Game|OpenLevel(byName) (Utilities|String|StringToName (Utilities|String|EnumtoString (Variables|Default|GetDestination))))))

(event Custom|Patrol
  (if (Variables|Patrol|GetPatrol%20Location%201)
    (Utilities|PatrolLocations true false
      (:Out
        (Utilities|FlowControl|Delay 2.0)
        (AI|AIMoveTo self (Variables|Default|GetLocation%20Vector%201) 0 5.0 false
          (:OnSuccess
            (Utilities|PatrolLocations false true :!label _label
              (:Out
                (Utilities|FlowControl|Delay 2.0)
                (AI|AIMoveTo self (Variables|Default|GetLocation%20Vector%202) 0 5.0 false
                  (:OnSuccess
                    (Utilities|PatrolLocations true false
                      (:Out
                        (CallFunction|Patrol)))))))))))
    (elif (Variables|Patrol|GetPatrol%20Location%202)
      (goto _label))))

(event EventBeginPlay
  (CallFunction|Patrol)
  (Rendering|SetVisibility (Variables|Default|GetWidgetComponent_Reaction) false false))

(fn ConstructionScript)