(event OnComponentBeginOverlap(Collision_Head)
  (params (OverlappedComponent :type Primitive%20Component%20Object%20Reference) (OtherActor :type Actor%20Object%20Reference) (OtherComp :type Primitive%20Component%20Object%20Reference) (OtherBodyIndex :type Integer) (bFromSweep :type Boolean) (SweepResult :type Hit%20Result%20Structure%20%28by%20ref%29))
  (bind _asthird_person_paper_topia (Utilities|Casting|CastToThirdPerson_PaperTopia (Game|GetPlayerCharacter 0)))
  (if (and (== (Utilities|GetClass OtherActor) "/Game/PaperTopia/Blueprints/ThirdPerson_PaperTopia.ThirdPerson_PaperTopia_C") (< (.z (Transformation|GetVelocity _asthird_person_paper_topia)) 0.0))
    (Default|BounceUp _asthird_person_paper_topia (Math|Vector|MakeVector 0.0 0.0 (.z (Variables|Default|GetBounce%20Intensity))))
    (Collision|SetCollisionEnabled (Variables|Default|GetCollision_Head) "NoCollision")
    (Input|DisableInput _asthird_person_paper_topia (Game|GetPlayerController 0))
    (Utilities|FlowControl|Delay 0.4)
    (Pawn|Components|CharacterMovement|SetMovementMode (Variables|/Script/Engine.Character|GetCharacterMovement _asthird_person_paper_topia) "MOVE_None" 0)
    (bind _returnvalue (UserInterface|CreateWidget "/Game/PaperTopia/UI/Widget_BattleTransition.Widget_BattleTransition_C"))
    (UserInterface|Viewport|AddtoViewport _returnvalue 0)
    (Utilities|FlowControl|Delay 2.0)
    (Game|LoadStreamLevel(byName) (Utilities|String|StringToName (Utilities|String|EnumtoString (Variables|Default|GetDestination))) true)
    (Game|UnloadStreamLevel(byName) (Utilities|String|StringToName (Utilities|String|EnumtoString (Variables|Default|GetUnloadCurrentLevel))) false)
    (Actor|DestroyActor)))

(event OnComponentHit(PaperFlipbook)
  (params (HitComponent :type Primitive%20Component%20Object%20Reference) (OtherActor :type Actor%20Object%20Reference) (OtherComp :type Primitive%20Component%20Object%20Reference) (NormalImpulse :type Vector :default "0, 0, 0") (Hit :type Hit%20Result%20Structure%20%28by%20ref%29))
  (bind _asthird_person_paper_topia (Utilities|Casting|CastToThirdPerson_PaperTopia (Game|GetPlayerCharacter 0)))
  (Collision|SetCollisionEnabled (Variables|Default|GetCollision_Head) "NoCollision")
  (Input|DisableInput _asthird_person_paper_topia (Game|GetPlayerController 0))
  (bind _returnvalue (AddComponent|AddAudioComponent false))
  (Audio|Components|Audio|FadeOut _returnvalue 2.5 0.0 "Linear" :!class /Script/Engine.AudioComponent)
  (Utilities|FlowControl|Delay 0.4)
  (Pawn|Components|CharacterMovement|SetMovementMode (Variables|/Script/Engine.Character|GetCharacterMovement _asthird_person_paper_topia) "MOVE_None" 0)
  (bind _returnvalue_2 (UserInterface|CreateWidget "/Game/PaperTopia/UI/Widget_BattleTransition.Widget_BattleTransition_C"))
  (UserInterface|Viewport|AddtoViewport _returnvalue_2 0)
  (Utilities|FlowControl|Delay 2.0)
  (Game|OpenLevel(byName) (Utilities|String|StringToName (Utilities|String|EnumtoString (Variables|Default|GetDestination)))))

(fn ConstructionScript)