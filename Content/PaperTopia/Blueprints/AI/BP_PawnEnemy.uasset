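; Paper2D enemy pawn that the player damages by falling onto its head, rewarding experience and coins when defeated.
; Head overlap bounces the player, subtracts attack minus defense from health and spawns floating damage text.
; On overlap end at zero health, it grants level-scaled XP, checks for level-up, then plays two rotation timelines.
; It then launches a physics coin and either shows level-up widgets or destroys itself.
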(event OnComponentBeginOverlap(Collision_Head)
  (params (OverlappedComponent :type Primitive%20Component%20Object%20Reference) (OtherActor :type Actor%20Object%20Reference) (OtherComp :type Primitive%20Component%20Object%20Reference) (OtherBodyIndex :type Integer) (bFromSweep :type Boolean) (SweepResult :type Hit%20Result%20Structure%20%28by%20ref%29))
  (if (> (Variables|Default|GetCurrentHealth) 0.0)
    (bind _asthird_person_character (Utilities|Casting|CastToThirdPersonCharacter (Game|GetPlayerCharacter 0)))
    (if (and (== (Utilities|GetClass OtherActor) "/Game/PaperTopia/Blueprints/ThirdPersonCharacter.ThirdPersonCharacter_C") (< (.z (Transformation|GetVelocity _asthird_person_character)) 0.0))
      (Sprite|SetFlipbook (Variables|Default|GetPaperFlipbook) (Variables|Default|GetAnim_Hit))
      (Default|BounceUp _asthird_person_character (Math|Vector|MakeVector 0.0 0.0 (.z (Variables|Default|GetBounce%20Intensity))))
      (bind _output_get (Variables|Default|SetTotalDamage (- (Variables|/Game/PaperTopia/Blueprints/ThirdPersonCharacter.ThirdPersonCharacter_C|GetAttackPower _asthird_person_character) (Variables|Default|GetDefense))))
      (Development|PrintString (Utilities|String|ToString(Float) _output_get) true true "(R=1.000000,G=0.202903,B=0.000000,A=1.000000)")
      (Variables|Default|SetCurrentHealth (- (Variables|Default|GetCurrentHealth) _output_get))
      (bind _returnvalue (Game|SpawnActorfromClass "/Game/PaperTopia/UI/BP_FloatingText.BP_FloatingText_C" (Math|Conversions|ToTransform(Vector) (+ (Transformation|GetActorLocation) "0, 0,100.000000")) "Undefined" "OverrideRootScale" 0 0))
      (Default|EventCreateText _returnvalue self)
      (Utilities|FlowControl|Delay 1.0)
      (Sprite|SetFlipbook (Variables|Default|GetPaperFlipbook) (Variables|Default|GetAnim_Idle)))))

(event OnComponentEndOverlap(Collision_Head)
  (params (OverlappedComponent :type Primitive%20Component%20Object%20Reference) (OtherActor :type Actor%20Object%20Reference) (OtherComp :type Primitive%20Component%20Object%20Reference) (OtherBodyIndex :type Integer))
  (bind _paperflipbook (Variables|Default|GetPaperFlipbook))
  (bind _returnvalue (Transformation|GetWorldLocation _paperflipbook))
  (if (<= (Variables|Default|GetCurrentHealth) 0.0)
    (Utilities|FlowControl|Delay 1.0)
    (Sprite|SetFlipbook (Variables|Default|GetPaperFlipbook) (Variables|Default|GetAnim_Death))
    (Utilities|FlowControl|DoOnce false
      (:Completed
        (bind _asthird_person_character (Utilities|Casting|CastToThirdPersonCharacter (Game|GetPlayerCharacter 0)))
        (if (>= (Variables|/Game/PaperTopia/Blueprints/ThirdPersonCharacter.ThirdPersonCharacter_C|GetLevel _asthird_person_character) (Variables|Default|Getexperience%20points%20))
          (Variables|Default|Setexperience%20points%20 1)
          (bind _rotation (Timeline|Timeline_0 Play)
            (:Update
              (Transformation|SetRelativeRotation (Variables|Default|GetDefaultSceneRoot) (Math|Rotator|MakeRotator 0.0 0.0 _rotation) false false))
            (:Finished
              (Effects|SpawnEmitteratLocation "/Game/PaperTopia/Particles/PS_XP.PS_XP" (Transformation|GetWorldLocation (Variables|Default|GetDefaultSceneRoot)))
              (Utilities|FlowControl|Delay 1.0)
              (bind _rotation_2 (Timeline|Timeline_1 Play)
                (:Update
                  (Transformation|SetRelativeRotation (Variables|Default|GetDefaultSceneRoot) (Math|Rotator|MakeRotator 0.0 _rotation_2 0.0) false false))
                (:Finished
                  ;[0.7799 0.1173 0.09445] Spawn Coins
                  (bind _returnvalue_2 (Game|SpawnActorfromClass "/Game/PaperTopia/Blueprints/Items/BP_Coins.BP_Coins_C" (Math|Transform|MakeTransform (Math|Vector|MakeVector (.x _returnvalue) (.y _returnvalue) (+ (.z _returnvalue) 2e+01)) "0, 0, 0" "1.000000,1.000000,1.000000") "Undefined" "OverrideRootScale" 0 "/Game/PaperTopia/Sounds/SFX/SoundCue_Coins.SoundCue_Coins" 0))
                  (Class|PrimitiveComponent|SetPhysMaterialOverride (Variables|/Game/PaperTopia/Blueprints/Items/BP_Coins.BP_Coins_C|GetCube _returnvalue_2) "/Game/PaperTopia/Materials/PhysicMat/PhysicalMaterial_Rubber.PhysicalMaterial_Rubber")
                  (Physics|AddImpulse (Variables|/Game/PaperTopia/Blueprints/Items/BP_Coins.BP_Coins_C|GetCube _returnvalue_2) (* (Math|Random|RandomUnitVectorinConeinDegrees "0, 0,1.000000" 2e+01) 5e+02) "None" true)
                  (Actor|SetLifeSpan _returnvalue_2 5.0)
                  (if (Variables|Default|GetLevelUP?)
                    (bind _returnvalue_3 (UserInterface|CreateWidget "/Game/PaperTopia/UI/Widget_LevelUp.Widget_LevelUp_C"))
                    (UserInterface|Viewport|AddtoViewport _returnvalue_3 0)
                    (Default|PlayLevelUpAnim _returnvalue_3)
                    (Utilities|FlowControl|Delay 2.0)
                    (Widget|RemovefromParent _returnvalue_3)
                    (bind _returnvalue_4 (UserInterface|CreateWidget "/Game/PaperTopia/UI/Widget_LevelUpUI.Widget_LevelUpUI_C"))
                    (UserInterface|Viewport|AddtoViewport _returnvalue_4 0)
                    (else
                      (Actor|DestroyActor)))))))
          (else
            (bind _output_get (Variables|Default|Setexperience%20points%20 (- (Variables|Default|Getexperience%20points%20) (- (Variables|/Game/PaperTopia/Blueprints/ThirdPersonCharacter.ThirdPersonCharacter_C|GetLevel _asthird_person_character) 1))))
            (bind _output_get_2 (Variables|/Game/PaperTopia/Blueprints/ThirdPersonCharacter.ThirdPersonCharacter_C|SetCurrent%20Experience _asthird_person_character (+ (Variables|/Game/PaperTopia/Blueprints/ThirdPersonCharacter.ThirdPersonCharacter_C|GetCurrent%20Experience _asthird_person_character) _output_get)))
            (if (>= _output_get_2 (Variables|/Game/PaperTopia/Blueprints/ThirdPersonCharacter.ThirdPersonCharacter_C|GetMax%20Experience _asthird_person_character))
              (Variables|/Game/PaperTopia/Blueprints/ThirdPersonCharacter.ThirdPersonCharacter_C|SetLevel _asthird_person_character (+ (Variables|/Game/PaperTopia/Blueprints/ThirdPersonCharacter.ThirdPersonCharacter_C|GetLevel _asthird_person_character) 1))
              (Variables|Default|SetLevelUP? true)
              (Variables|/Game/PaperTopia/Blueprints/ThirdPersonCharacter.ThirdPersonCharacter_C|SetCurrent%20Experience _asthird_person_character (- _output_get_2 (Variables|/Game/PaperTopia/Blueprints/ThirdPersonCharacter.ThirdPersonCharacter_C|GetMax%20Experience _asthird_person_character)))
              (Timeline|Timeline_0 Play)
              (else
                (Timeline|Timeline_0 Play)))))))))

(event EventBeginPlay
  ;[1 1 1] Look up on wake
  (Variables|Default|SetCurrentHealth (Variables|Default|GetMaxHealth))
  (bind _asthird_person_character (Utilities|Casting|CastToThirdPersonCharacter (Game|GetPlayerCharacter 0)))
  (bind _output_get (Variables|Default|SetAs%20Third%20Person%20Character _asthird_person_character))
  (if (>= (Variables|/Game/PaperTopia/Blueprints/ThirdPersonCharacter.ThirdPersonCharacter_C|GetLevel _output_get) (Variables|Default|Getexperience%20points%20))
    (Variables|Default|Setexperience%20points%20 1)
    (else
      (Variables|Default|Setexperience%20points%20 (- (Variables|Default|Getexperience%20points%20) (- (Variables|/Game/PaperTopia/Blueprints/ThirdPersonCharacter.ThirdPersonCharacter_C|GetLevel _output_get) 1))))))

(fn ConstructionScript)