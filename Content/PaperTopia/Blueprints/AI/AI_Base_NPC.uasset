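; AI_Base_NPC is a base NPC Blueprint that shows a talk icon while the player's character is nearby.
; When a ThirdPersonCharacter enters TalkIconTrigger, it applies the TalkIcon texture to the image in its Widget_TalkIcon component and unhides it.
; Leaving the trigger hides the widget again.
; The graph holds no dialogue or AI logic.
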(event OnComponentBeginOverlap(TalkIconTrigger)
  (params (OverlappedComponent :type Primitive%20Component%20Object%20Reference) (OtherActor :type Actor%20Object%20Reference) (OtherComp :type Primitive%20Component%20Object%20Reference) (OtherBodyIndex :type Integer) (bFromSweep :type Boolean) (SweepResult :type Hit%20Result%20Structure%20%28by%20ref%29))
  (bind _widget_talkicon (Variables|Default|GetWidget_TalkIcon))
  (Utilities|Casting|CastToThirdPersonCharacter OtherActor)
  (bind _aswidget_talk_icon (Utilities|Casting|CastToWidget_TalkIcon (UserInterface|GetUserWidgetObject _widget_talkicon)))
  (Appearance|SetBrushfromTexture (Variables|/Game/PaperTopia/UI/Widget_TalkIcon.Widget_TalkIcon_C|GetImage_33 _aswidget_talk_icon) "/Game/PaperTopia/Textures/TalkIcon.TalkIcon" true)
  (Development|SetHiddeninGame _widget_talkicon false false))

(event OnComponentEndOverlap(TalkIconTrigger)
  (params (OverlappedComponent :type Primitive%20Component%20Object%20Reference) (OtherActor :type Actor%20Object%20Reference) (OtherComp :type Primitive%20Component%20Object%20Reference) (OtherBodyIndex :type Integer))
  (Utilities|Casting|CastToThirdPersonCharacter OtherActor)
  (Development|SetHiddeninGame (Variables|Default|GetWidget_TalkIcon) true false))

(event EventBeginPlay)

(event Collision|EventActorBeginOverlap
  (params (OtherActor :type Actor%20Object%20Reference)))

(event EventTick
  (params (DeltaSeconds :type Float%20%28single-precision%29)))

(fn ConstructionScript)