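; Behavior tree task that asks the player a dialogue question and records the chosen response.
; On execute it gets the dialogue box widget from the Blackboard, sets its text to the question, and adds a response list holding one clickable widget per configured response.
; The task stays active until a response event writes the answer to a Blackboard string, removes the list, and finishes successfully.
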(event Custom|ResponseRecieved
  (params (ResponseRecieved :type Text))
  (Class|BTFunctionLibrary|SetBlackboardValueasString (Variables|Default|GetBB_Response) (Utilities|String|ToString(Text) ResponseRecieved))
  (Widget|RemovefromParent (Variables|Default|GetResponseList))
  (AI|BehaviorTree|FinishExecute true))

(event EventReceiveExecuteAI
  (params (OwnerController :type AI%20Controller%20Object%20Reference) (ControlledPawn :type Pawn%20Object%20Reference))
  (bind _aswidget_dialogue_box (Utilities|Casting|CastToWidget_DialogueBox (Class|BTFunctionLibrary|GetBlackboardValueasObject (Variables|Default|GetBB_DialogueUI))))
  (bind _output_get (Variables|Default|SetDialogue%20Box _aswidget_dialogue_box))
  (Variables|/Game/PaperTopia/UI/Widget_DialogueBox.Widget_DialogueBox_C|SetDialogueText _output_get (Variables|Default|GetQuestion))
  (CallFunction|PrepareResponses))

(fn PrepareResponses
  (bind _returnvalue (UserInterface|CreateWidget "/Game/PaperTopia/UI/Widget_ResponseList.Widget_ResponseList_C"))
  (bind _output_get (Variables|Default|SetResponseList _returnvalue))
  (Class|Overlay|AddChildtoOverlay (Variables|/Game/PaperTopia/UI/Widget_DialogueBox.Widget_DialogueBox_C|GetResponseListPanel (Variables|Default|GetDialogue%20Box)) _output_get)
  (for _array_element (Variables|Default|GetResponses)
    (bind _returnvalue_2 (UserInterface|CreateWidget "/Game/PaperTopia/UI/Widget_Responses.Widget_Responses_C" 0 _array_element))
    (Class|VerticalBox|AddChildtoVerticalBox (Variables|/Game/PaperTopia/UI/Widget_ResponseList.Widget_ResponseList_C|GetResponseList (Variables|Default|GetResponseList)) _returnvalue_2)
    (EventDispatchers|BindEventtoResponseClicked _returnvalue_2 (EventDispatchers|CreateEvent :!event Custom|ResponseRecieved))))