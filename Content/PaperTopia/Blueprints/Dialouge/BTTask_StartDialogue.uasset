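; Behavior tree task that opens the dialogue UI when an AI NPC begins a conversation.
; On execute, it sets the NPC's name as speaker on the dialogue box in the PaperTopia game mode's HUD and makes it visible.
; It stores that widget in a blackboard key, disables player character input, shows the mouse cursor and finishes successfully.
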(event EventReceiveExecuteAI
  (params (OwnerController :type AI%20Controller%20Object%20Reference) (ControlledPawn :type Pawn%20Object%20Reference))
  (bind _returnvalue (Game|GetPlayerController 0))
  (bind _asai_npc (Utilities|Casting|CastToAI_NPC ControlledPawn))
  (Variables|Default|SetNPCPawn _asai_npc)
  (bind _asgame_mode_paper_topia (Utilities|Casting|CastToGameMode_PaperTopia (Game|GetGameMode)))
  (Variables|/Game/PaperTopia/UI/Widget_DialogueBox.Widget_DialogueBox_C|SetSpeakerName (Variables|/Game/PaperTopia/UI/Widget_HUD.Widget_HUD_C|GetWidget_DialogueBox (Variables|/Game/PaperTopia/Blueprints/System/GameMode_PaperTopia.GameMode_PaperTopia_C|GetHeads%20UpDisplay _asgame_mode_paper_topia)) (Variables|/Game/PaperTopia/Blueprints/AI/AI_NPC.AI_NPC_C|GetNPCName (Variables|Default|GetNPCPawn)))
  (Widget|SetVisibility (Variables|/Game/PaperTopia/UI/Widget_HUD.Widget_HUD_C|GetWidget_DialogueBox (Variables|/Game/PaperTopia/Blueprints/System/GameMode_PaperTopia.GameMode_PaperTopia_C|GetHeads%20UpDisplay _asgame_mode_paper_topia)) "Visible")
  (Development|PrintString "ITS VISIBLE")
  (Class|BTFunctionLibrary|SetBlackboardValueasObject (Variables|Default|GetBB_DialogueUI) (Variables|/Game/PaperTopia/UI/Widget_HUD.Widget_HUD_C|GetWidget_DialogueBox (Variables|/Game/PaperTopia/Blueprints/System/GameMode_PaperTopia.GameMode_PaperTopia_C|GetHeads%20UpDisplay _asgame_mode_paper_topia)))
  (Input|DisableInput (Game|GetPlayerCharacter 0) _returnvalue)
  (Variables|/Script/Engine.PlayerController|SetbShowMouseCursor _returnvalue true)
  (AI|BehaviorTree|FinishExecute true))