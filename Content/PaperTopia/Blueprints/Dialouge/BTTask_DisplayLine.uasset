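; Behavior Tree task that shows one line of dialogue in the dialogue box widget and waits for the player to advance it.
; On execute it reads the widget from a blackboard key, casts it to Widget_DialogueBox and sets its DialogueText to the task's Text.
; Each tick it compares key presses against the "Inter" action mapping and finishes successfully when one of those keys is pressed.
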(event EventReceiveExecuteAI
  (params (OwnerController :type AI%20Controller%20Object%20Reference) (ControlledPawn :type Pawn%20Object%20Reference))
  (bind _aswidget_dialogue_box (Utilities|Casting|CastToWidget_DialogueBox (Class|BTFunctionLibrary|GetBlackboardValueasObject (Variables|Default|GetDialougeWidget))))
  (Variables|/Game/PaperTopia/UI/Widget_DialogueBox.Widget_DialogueBox_C|SetDialogueText _aswidget_dialogue_box (Variables|Default|GetText)))

(event EventTick
  (params (OwnerActor :type Actor%20Object%20Reference) (DeltaSeconds :type Float%20%28single-precision%29))
  (if (Game|Player|WasInputKeyJustPressed (Game|GetPlayerController 0) "AnyKey")
    (for _array_element (Class|InputSettings|GetActionMappingbyName (Class|InputSettings|GetInputSettings) "Inter")
      (if (Game|Player|WasInputKeyJustPressed (Game|GetPlayerController 0) (.Key (Utilities|Struct|BreakInputActionKeyMapping _array_element)))
        (AI|BehaviorTree|FinishExecute true)))))