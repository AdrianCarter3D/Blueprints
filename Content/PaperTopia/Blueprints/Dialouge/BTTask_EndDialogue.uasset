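; Behavior tree task that closes an NPC dialogue and hands control back to the player.
; It hides the dialogue widget stored on the blackboard and calls EndDialogue on the owning BP_AIController.
; It then hides the mouse cursor, switches to game-only input, re-enables player character input and finishes successfully.
; A failed widget or controller cast stops execution before FinishExecute is reached.
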(event EventReceiveExecuteAI
  (params (OwnerController :type AI%20Controller%20Object%20Reference) (ControlledPawn :type Pawn%20Object%20Reference))
  (bind _returnvalue (Game|GetPlayerController 0))
  (bind _aswidget (Utilities|Casting|CastToWidget (Class|BTFunctionLibrary|GetBlackboardValueasObject (Variables|Default|GetBB_DialougeUI))))
  (Widget|SetVisibility _aswidget "Hidden")
  (bind _asbp_aicontroller (Utilities|Casting|CastToBP_AIController OwnerController))
  (Default|EndDialogue _asbp_aicontroller)
  (Variables|/Script/Engine.PlayerController|SetbShowMouseCursor _returnvalue false)
  (Input|SetInputModeGameOnly _returnvalue false)
  (Input|EnableInput (Game|GetPlayerCharacter 0) _returnvalue)
  (AI|BehaviorTree|FinishExecute true))