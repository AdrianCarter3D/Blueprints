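; BP_Bot_Axe is a flying drone bot with a swinging axe and spinning gyro blades.
; On BeginPlay a timeline adds its swing curve to the axe's starting world pitch, with a whoosh sound on finish, and a quiet drone sound also plays.
; Tick spins the blades with a fixed yaw step per frame, unscaled by delta time, writing relative rotation plus that step as world rotation.
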(event EventBeginPlay
  (bind _returnvalue (Transformation|GetActorLocation))
  (Utilities|FlowControl|Sequence
    (:then_0
      (Variables|Default|SetRotation (Transformation|GetWorldRotation (Variables|Default|GetSM_Axe)))
      (bind _swing (Timeline|Timeline_AxeSwing Play)
        (:Update
          (Transformation|SetWorldRotation (Variables|Default|GetSM_Axe) (Math|Rotator|MakeRotator (.roll (Variables|Default|GetRotation)) (+ _swing (.pitch (Variables|Default|GetRotation))) (.yaw (Variables|Default|GetRotation))) false false))
        (:Finished
          (Audio|PlaySoundatLocation "/Game/2024SpaceBotdyssey/Models/Bot/sword-swing-whoosh-sound-effect-1-full-pack-on-gamesfxpackscom-241824_Cue.sword-swing-whoosh-sound-effect-1-full-pack-on-gamesfxpackscom-241824_Cue" _returnvalue "0, 0, 0" 1.0 1.0 0.0 "/Game/BombBombLand/Audio/Attenuation/SoundAttenuation_Normal.SoundAttenuation_Normal" 0 0 0))))
    (:then_1
      (Audio|PlaySoundatLocation "/Game/2024SpaceBotdyssey/Models/Bot/sound-of-flying-drone_02-166962_Cue.sound-of-flying-drone_02-166962_Cue" _returnvalue "0, 0, 0" 0.1 1.0 0.0 "/Game/BombBombLand/Audio/Attenuation/SoundAttenuation_Normal.SoundAttenuation_Normal" 0 0 0))))

(event Collision|EventActorBeginOverlap
  (params (OtherActor :type Actor%20Object%20Reference)))

(event EventTick
  (params (DeltaSeconds :type Float%20%28single-precision%29))
  (bind _gyroblades (Variables|Default|GetGyroBlades))
  (bind _relativerotation (Variables|/Script/Engine.SceneComponent|GetRelativeRotation _gyroblades))
  (Transformation|SetWorldRotation _gyroblades (Math|Rotator|MakeRotator (.roll _relativerotation) (.pitch _relativerotation) (+ 3e+01 (.yaw _relativerotation))) false false))

(fn ConstructionScript)