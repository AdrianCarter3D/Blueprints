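; BP_Projectile_BASE is the base projectile Blueprint in SuperVania, dealing damage to platformer characters of a different faction.
; Overlapping a BP_Platformer2D whose Faction differs from its own applies ProjectileDamage, plays the hit effect and destroys the projectile.
; A blocking hit on the Sphere plays the effect and destroys it without damage.
; PlayHitEffect spawns a BP_VFX_BASE_Child actor at the projectile's location and rotation.
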(event OnComponentHit(Sphere)
  (params (HitComponent :type Primitive%20Component%20Object%20Reference) (OtherActor :type Actor%20Object%20Reference) (OtherComp :type Primitive%20Component%20Object%20Reference) (NormalImpulse :type Vector :default "0, 0, 0") (Hit :type Hit%20Result%20Structure%20%28by%20ref%29))
  (CallFunction|PlayHitEffect)
  (Actor|DestroyActor))

(event OnComponentBeginOverlap(Sphere)
  (params (OverlappedComponent :type Primitive%20Component%20Object%20Reference) (OtherActor :type Actor%20Object%20Reference) (OtherComp :type Primitive%20Component%20Object%20Reference) (OtherBodyIndex :type Integer) (bFromSweep :type Boolean) (SweepResult :type Hit%20Result%20Structure%20%28by%20ref%29))
  (bind _asbp_platformer_2d (Utilities|Casting|CastToBP_Platformer2D OtherActor))
  (if (Utilities|Enum|NotEqual(Enum) (Variables|/Game/SuperVania/Blueprints/Player/BP_Platformer2D.BP_Platformer2D_C|GetFaction _asbp_platformer_2d) (Variables|Default|GetFaction))
    (Game|Damage|ApplyDamage _asbp_platformer_2d (Variables|Default|GetProjectileDamage) 0 0)
    (CallFunction|PlayHitEffect)
    (Actor|DestroyActor)))

(event EventTick
  (params (DeltaSeconds :type Float%20%28single-precision%29)))

(fn ConstructionScript)

(fn PlayHitEffect
  (Game|SpawnActorfromClass "/Game/SuperVania/Effects/BP_VFX_BASE_Child.BP_VFX_BASE_Child_C" (Math|Transform|MakeTransform (Transformation|GetActorLocation) (Transformation|GetActorRotation) "1.000000,1.000000,1.000000") "AlwaysSpawn" "MultiplyWithRoot" 0 0))