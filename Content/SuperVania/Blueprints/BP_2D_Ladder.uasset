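; BP_2D_Ladder is a ladder trigger for the 2D player character BPChild_SumasNara in SuperVania.
; When that character overlaps the Box, it sets the character's OnLadder flag and disables gravity on the capsule.
; When the overlap ends, it clears the flag, sets movement mode to Walking and re-enables gravity, with debug prints on both transitions.
; Climbing movement itself is not handled in this Blueprint.
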(event OnComponentBeginOverlap(Box)
  (params (OverlappedComponent :type Primitive%20Component%20Object%20Reference) (OtherActor :type Actor%20Object%20Reference) (OtherComp :type Primitive%20Component%20Object%20Reference) (OtherBodyIndex :type Integer) (bFromSweep :type Boolean) (SweepResult :type Hit%20Result%20Structure%20%28by%20ref%29))
  (bind _asbpchild_sumas_nara (Utilities|Casting|CastToBPChild_SumasNara OtherActor))
  (Variables|/Game/SuperVania/Blueprints/Player/BPChild_SumasNara.BPChild_SumasNara_C|SetOnLadder _asbpchild_sumas_nara true)
  (Development|PrintString "OnLadder")
  (Physics|SetEnableGravity (Variables|/Script/Engine.Character|GetCapsuleComponent _asbpchild_sumas_nara) false))

(event OnComponentEndOverlap(Box)
  (params (OverlappedComponent :type Primitive%20Component%20Object%20Reference) (OtherActor :type Actor%20Object%20Reference) (OtherComp :type Primitive%20Component%20Object%20Reference) (OtherBodyIndex :type Integer))
  (bind _asbpchild_sumas_nara (Utilities|Casting|CastToBPChild_SumasNara OtherActor))
  (Variables|/Game/SuperVania/Blueprints/Player/BPChild_SumasNara.BPChild_SumasNara_C|SetOnLadder _asbpchild_sumas_nara false)
  (Development|PrintString "OffLadder")
  (Pawn|Components|CharacterMovement|SetMovementMode (Variables|/Script/Engine.Character|GetCharacterMovement _asbpchild_sumas_nara) "MOVE_Walking" 0)
  (Physics|SetEnableGravity (Variables|/Script/Engine.Character|GetCapsuleComponent _asbpchild_sumas_nara) true))

(event EventBeginPlay)

(event Collision|EventActorBeginOverlap
  (params (OtherActor :type Actor%20Object%20Reference)))

(event EventTick
  (params (DeltaSeconds :type Float%20%28single-precision%29)))

(fn ConstructionScript)