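; BP_Bullet is a projectile fired by the BPChild_SumasNara character, which it caches from its owner on BeginPlay.
; Tick projects its location to screen space, with debug prints, and destroys it past the left or right viewport edge.
; Sphere overlaps with actors not tagged Ignore spawn BP_Impact, apply damage, destroy the bullet and launch enemies flagged for Pushback.
; Both destruction paths call RestoreShotEnergy on the owner.
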(event OnComponentBeginOverlap(Sphere)
  (params (OverlappedComponent :type Primitive%20Component%20Object%20Reference) (OtherActor :type Actor%20Object%20Reference) (OtherComp :type Primitive%20Component%20Object%20Reference) (OtherBodyIndex :type Integer) (bFromSweep :type Boolean) (SweepResult :type Hit%20Result%20Structure%20%28by%20ref%29))
  (if (not (Actor|ActorHasTag OtherActor "Ignore"))
    (Game|SpawnActorfromClass "/Game/SuperVania/PaperZD/Sprites/Fx/impact/BP_Impact.BP_Impact_C" (Transformation|GetActorTransform) "Undefined" "MultiplyWithRoot" 0 0)
    (Game|Damage|ApplyDamage OtherActor (Math|Conversions|ToFloat(Integer) (Variables|Default|GetDamage)) 0 self)
    (Actor|DestroyActor)
    (Default|RestoreShotEnergy (Variables|Default|GetAs%20BPChild%20Sumas%20Nara))
    (bind _asbpchild_platformer_2denemy (Utilities|Casting|CastToBPChild_Platformer2DEnemy OtherActor))
    (if (Variables|/Game/SuperVania/Blueprints/Player/BP_Platformer2D.BP_Platformer2D_C|GetPushback? _asbpchild_platformer_2denemy)
      (Character|LaunchCharacter _asbpchild_platformer_2denemy (Math|Vector|MakeVector (.x (* (Transformation|GetActorForwardVector) 400)) 0.0 5e+02) true true))))

(event EventBeginPlay
  (Variables|Default|SetDamage (Variables|Default|GetDamage))
  (bind _asbpchild_sumas_nara (Utilities|Casting|CastToBPChild_SumasNara (Components|GetOwner)))
  (Variables|Default|SetAs%20BPChild%20Sumas%20Nara _asbpchild_sumas_nara))

(event EventTick
  (params (DeltaSeconds :type Float%20%28single-precision%29))
  (bind _returnvalue (Game|GetPlayerController 0))
  (bind _returnvalue_2 (Transformation|GetActorLocation))
  (bind _screenlocation (Class|PlayerController|ProjectWorldLocationtoScreen _returnvalue _returnvalue_2 false))
  (Development|PrintString (Utilities|String|ToString(Float) (.x _screenlocation)))
  (if (or (<= (.x _screenlocation) 0.0) (>= (.x _screenlocation) (.x (Viewport|GetViewportSize))))
    (Development|PrintString "Destroy")
    (Actor|DestroyActor)
    (Default|RestoreShotEnergy (Variables|Default|GetAs%20BPChild%20Sumas%20Nara))))

(fn ConstructionScript)