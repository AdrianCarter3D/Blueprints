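; Water volume actor that switches the scene to an underwater look while the third-person player character is inside its box.
; On box begin overlap with BP_ThirdPersonCharacter, it shows its own height fog and post-process components and hides the global exponential height fog referenced by GameMode_Sonic.
; On end overlap it reverses this, hiding the local effects and restoring the game mode's fog.
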(event OnComponentBeginOverlap(Box)
  (params (OverlappedComponent :type Primitive%20Component%20Object%20Reference) (OtherActor :type Actor%20Object%20Reference) (OtherComp :type Primitive%20Component%20Object%20Reference) (OtherBodyIndex :type Integer) (bFromSweep :type Boolean) (SweepResult :type Hit%20Result%20Structure%20%28by%20ref%29))
  (Utilities|Casting|CastToBP_ThirdPersonCharacter OtherActor)
  (Rendering|SetVisibility (Variables|Default|GetExponentialHeightFog) true false)
  (Rendering|SetVisibility (Variables|Default|GetPostProcess) true false)
  (bind _asgame_mode_sonic (Utilities|Casting|CastToGameMode_Sonic (Game|GetGameMode)))
  (Rendering|SetVisibility (Variables|/Script/Engine.ExponentialHeightFog|GetComponent (Variables|/Game/Blueprints/Core/Gameplay/Gamemode/GameMode_Sonic.GameMode_Sonic_C|GetExponentialHeightFog _asgame_mode_sonic)) false false))

(event OnComponentEndOverlap(Box)
  (params (OverlappedComponent :type Primitive%20Component%20Object%20Reference) (OtherActor :type Actor%20Object%20Reference) (OtherComp :type Primitive%20Component%20Object%20Reference) (OtherBodyIndex :type Integer))
  (Utilities|Casting|CastToBP_ThirdPersonCharacter OtherActor)
  (Rendering|SetVisibility (Variables|Default|GetExponentialHeightFog) false false)
  (Rendering|SetVisibility (Variables|Default|GetPostProcess) false false)
  (bind _asgame_mode_sonic (Utilities|Casting|CastToGameMode_Sonic (Game|GetGameMode)))
  (Rendering|SetVisibility (Variables|/Script/Engine.ExponentialHeightFog|GetComponent (Variables|/Game/Blueprints/Core/Gameplay/Gamemode/GameMode_Sonic.GameMode_Sonic_C|GetExponentialHeightFog _asgame_mode_sonic)) true false))

(event EventBeginPlay)

(event Collision|EventActorBeginOverlap
  (params (OtherActor :type Actor%20Object%20Reference)))

(event EventTick
  (params (DeltaSeconds :type Float%20%28single-precision%29)))

(fn ConstructionScript)