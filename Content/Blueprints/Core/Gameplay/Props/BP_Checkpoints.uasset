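; A checkpoint gate prop that fires once when the third-person character overlaps its middle trigger, giving audiovisual feedback only.
; It plays a sound, starts both side skeletal montages at rates scaled by player speed, and hides the beam.
; As each montage completes, that side's orb takes a completed material and both lights turn orange.
; The construction script attaches each orb light to its mesh socket.
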(event OnComponentBeginOverlap(Middle)
  (params (OverlappedComponent :type Primitive%20Component%20Object%20Reference) (OtherActor :type Actor%20Object%20Reference) (OtherComp :type Primitive%20Component%20Object%20Reference) (OtherBodyIndex :type Integer) (bFromSweep :type Boolean) (SweepResult :type Hit%20Result%20Structure%20%28by%20ref%29))
  (bind _returnvalue (Game|GetPlayerCharacter 0))
  (bind _sk_checkpointleft (Variables|Default|GetSK_CheckPointLeft))
  (bind _sk_checkpointright (Variables|Default|GetSK_CheckPointRight))
  (bind _returnvalue_2 (Transformation|GetVelocity _returnvalue))
  (bind _returnvalue_3 (Math|Vector|VectorLength _returnvalue_2))
  (bind _returnvalue_4 (/ _returnvalue_3 2.5e+03))
  (bind _returnvalue_5 (Math|Float|Clamp(Float) _returnvalue_4 1.0 1e+04))
  (Utilities|Casting|CastToBP_ThirdPersonCharacter OtherActor)
  (Utilities|FlowControl|DoOnce false
    (:Completed
      (Utilities|FlowControl|Sequence
        (:then_0
          (Development|PrintString "checkpoint"))
        (:then_1
          (Audio|PlaySoundatLocation "/Game/Assets/Audio/Sounds/SFX/SE_Checkpoint.SE_Checkpoint" (Transformation|GetActorLocation) "0, 0, 0" 1.0 1.0 0.0 0 0 0 0)
          (Animation|Montage|PlayMontage _sk_checkpointleft "/Game/Assets/Animations/AnimationMongtage_CheckPointLeft.AnimationMongtage_CheckPointLeft" _returnvalue_5
            (:then
              (Animation|Montage|PlayMontage _sk_checkpointright "/Game/Assets/Animations/AnimationMontage_CheckPointRight.AnimationMontage_CheckPointRight" _returnvalue_5
                (:then
                  (Rendering|SetVisibility (Variables|Default|GetBeam) false false))
                (:OnCompleted
                  (Rendering|Material|SetMaterial _sk_checkpointright 1 "/Game/Materials/Master/MI_CheckpointsOrb_Completed.MI_CheckpointsOrb_Completed")
                  (Rendering|Components|Light|SetLightColor (Variables|Default|GetOrbLight1) "(R=1.000000,G=0.628884,B=0.000000,A=1.000000)" true :!label _label))))
            (:OnCompleted
              (Rendering|Material|SetMaterial _sk_checkpointleft 1 "/Game/Materials/Master/MI_CheckpointsOrb_Completed.MI_CheckpointsOrb_Completed")
              (goto _label))))))))

(event EventBeginPlay)

(event Collision|EventActorBeginOverlap
  (params (OtherActor :type Actor%20Object%20Reference)))

(event EventTick
  (params (DeltaSeconds :type Float%20%28single-precision%29)))

(fn ConstructionScript
  (Transformation|AttachComponentToComponent (Variables|Default|GetOrbLight) (Variables|Default|GetSK_CheckPointLeft) "effectpointL" "KeepRelative" "KeepRelative" "KeepRelative" true)
  (Transformation|AttachComponentToComponent (Variables|Default|GetOrbLight1) (Variables|Default|GetSK_CheckPointRight) "effectpointR" "KeepRelative" "KeepRelative" "KeepRelative" true))