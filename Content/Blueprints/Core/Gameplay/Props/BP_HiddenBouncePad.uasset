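; Hidden bounce pad prop that starts invisible and inert, then reveals itself temporarily when the third-person character enters its trigger.
; Overlapping Box shows the skeletal mesh and enables Box1 for VisibilityTimer, with a DoOnce blocking retriggers until it hides again.
; Overlapping Box1 launches the character with SpringPower along Z, rotated by the actor's rotation and overriding current velocity, and plays a spring sound.
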(event OnComponentBeginOverlap(Box)
  (params (OverlappedComponent :type Primitive%20Component%20Object%20Reference) (OtherActor :type Actor%20Object%20Reference) (OtherComp :type Primitive%20Component%20Object%20Reference) (OtherBodyIndex :type Integer) (bFromSweep :type Boolean) (SweepResult :type Hit%20Result%20Structure%20%28by%20ref%29))
  (bind _skeletalmesh (Variables|Default|GetSkeletalMesh))
  (Utilities|Casting|CastToBP_ThirdPersonCharacter OtherActor)
  (Utilities|FlowControl|DoOnce false :!label _label
    (:Completed
      (Rendering|SetVisibility _skeletalmesh true false)
      (Collision|SetCollisionEnabled (Variables|Default|GetBox1) "QueryOnly")
      (Utilities|FlowControl|Delay (Variables|Default|GetVisibilityTimer))
      (Rendering|SetVisibility _skeletalmesh false false)
      (Collision|SetCollisionEnabled (Variables|Default|GetBox1) "NoCollision")
      (goto _label Reset))))

(event OnComponentBeginOverlap(Box1)
  (params (OverlappedComponent :type Primitive%20Component%20Object%20Reference) (OtherActor :type Actor%20Object%20Reference) (OtherComp :type Primitive%20Component%20Object%20Reference) (OtherBodyIndex :type Integer) (bFromSweep :type Boolean) (SweepResult :type Hit%20Result%20Structure%20%28by%20ref%29))
  ;[1 1 1] Launching player straight up by splitting the vector and using the Z axis ( World Up)
  (bind _asbp_third_person_character (Utilities|Casting|CastToBP_ThirdPersonCharacter OtherActor))
  (Character|LaunchCharacter _asbp_third_person_character (Math|Vector|RotateVector (+ (Transformation|GetActorForwardVector) (Math|Vector|MakeVector 0.0 0.0 (Variables|Default|GetSpringPower))) (Transformation|GetActorRotation)) true true)
  (Audio|PlaySoundatLocation "/Game/Assets/Audio/Sounds/SFX/SE_Spring.SE_Spring" (Transformation|GetActorLocation) "0, 0, 0" 1.0 1.0 0.0 "/Game/Assets/Audio/Attenuation/SoundAttenuation_Normal.SoundAttenuation_Normal" 0 0 0))

(event EventBeginPlay
  (Rendering|SetVisibility (Variables|Default|GetSkeletalMesh) false false)
  (Collision|SetCollisionEnabled (Variables|Default|GetBox1) "NoCollision"))

(event Collision|EventActorBeginOverlap
  (params (OtherActor :type Actor%20Object%20Reference)))

(event EventTick
  (params (DeltaSeconds :type Float%20%28single-precision%29)))

(fn ConstructionScript)