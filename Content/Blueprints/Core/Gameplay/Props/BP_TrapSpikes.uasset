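; Spike trap prop that raises its spikes when the player enters a trigger sphere and lowers them when they leave.
; Tick interpolates the spikes if Animated, with DoOnce gates toggling CanDamagePlayer and playing sounds, plus an exclamation effect over the player on extension.
; While damage is enabled, a player overlapping the Box takes damage every tick.
; The construction script sets the trigger radius from a variable.
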(event EventTick
  (params (DeltaSeconds :type Float%20%28single-precision%29))
  (bind _returnvalue (Game|GetPlayerCharacter 0))
  (bind _returnvalue_2 (Transformation|GetActorLocation))
  (bind _returnvalue_3 (Utilities|Time|GetWorldDeltaSeconds))
  (bind _spikes (Variables|Default|GetSpikes))
  (bind _spikes_2 (Variables|Default|GetSpikes))
  (bind _interp_speed (Variables|Default|GetInterp%20Speed))
  (bind _relativelocation (Variables|/Script/Engine.SceneComponent|GetRelativeLocation _spikes_2))
  (Utilities|FlowControl|Sequence
    (:then_0
      (if (Variables|Default|GetAnimated?)
        (if (Collision|IsOverlappingActor (Variables|Default|GetSphere) (Game|GetPlayerCharacter 0) :!class /Script/Engine.PrimitiveComponent)
          (Transformation|SetRelativeLocation _spikes (Math|Interpolation|VInterpTo _relativelocation "0, 0, 0" _returnvalue_3 _interp_speed) false false)
          (Utilities|FlowControl|Sequence
            (:then_0
              (Utilities|FlowControl|DoOnce false :!label _label
                (:Completed
                  (Utilities|FlowControl|Delay (/ (Variables|Default|GetInterp%20Speed) 1.7e+02))
                  (Variables|Default|SetCanDamagePlayer? true)
                  (Audio|PlaySoundatLocation "/Game/Assets/Audio/Sounds/SFX/SE_Needle_Panel_Out.SE_Needle_Panel_Out" _returnvalue_2 "0, 0, 0" 0.25 2.0 0.0 "/Game/Assets/Audio/Attenuation/SoundAttenuation_Normal.SoundAttenuation_Normal" 0 0 0)
                  (Niagara|SpawnSystemAttached "/Game/Assets/NiagaraParticles/NiagaraSystem_Exclamation.NiagaraSystem_Exclamation" (Variables|/Script/Engine.Character|GetMesh (Game|GetPlayerCharacter 0)) "None" "0.000000,0.000000,210.000000" "0, 0, 0" "KeepRelativeOffset" true))))
            (:then_1
              (goto _label_2 Reset)))
          (else
            (Transformation|SetRelativeLocation _spikes (Math|Interpolation|VInterpTo _relativelocation "0.000000,0.000000,-100.000000" _returnvalue_3 _interp_speed) false false)
            (Utilities|FlowControl|Sequence
              (:then_0
                (Utilities|FlowControl|DoOnce false :!label _label_2
                  (:Completed
                    (Variables|Default|SetCanDamagePlayer? false)
                    (Audio|PlaySoundatLocation "/Game/Assets/Audio/Sounds/SFX/SE_Needle_Panel_Out.SE_Needle_Panel_Out" _returnvalue_2 "0, 0, 0" 0.25 2.0 0.0 "/Game/Assets/Audio/Attenuation/SoundAttenuation_Normal.SoundAttenuation_Normal" 0 0 0))))
              (:then_1
                (goto _label Reset)))))))
    (:then_1
      (if (and (Collision|IsOverlappingActor (Variables|Default|GetBox) _returnvalue :!class /Script/Engine.PrimitiveComponent) (Variables|Default|GetCanDamagePlayer?))
        (bind _asbp_third_person_character (Utilities|Casting|CastToBP_ThirdPersonCharacter _returnvalue))
        (bind _returnvalue_4 (Game|Damage|ApplyDamage _asbp_third_person_character 1.0 0 self))
        (Development|PrintString (Utilities|String|ToString(Float) _returnvalue_4))))))

(fn ConstructionScript
  (Components|Sphere|SetSphereRadius (Variables|Default|GetSphere) (Variables|Default|GetIn%20Sphere%20Radius) true))