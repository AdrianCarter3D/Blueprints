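; BP_SpawnFallingObjects is a prop spawner that periodically creates random objects at its own location, presumably to fall.
; BeginPlay picks one random interval between Min and Max for a looping timer, so the rate stays fixed afterward.
; Each tick of that timer shuffles ObjectsToSpawn and spawns a randomly indexed class with random rotation.
; The random index range includes the array length, so it can land out of bounds.
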(event Custom|SpawnObjects
  (bind _objectstospawn (Variables|Default|GetObjectsToSpawn))
  (Utilities|Array|Shuffle _objectstospawn)
  (Game|SpawnActorfromClass (Utilities|Array|Get(acopy) _objectstospawn (Math|Random|RandomIntegerinRange 0 (Utilities|Array|Length _objectstospawn))) (Math|Transform|MakeTransform (Transformation|GetActorLocation) (Math|Random|RandomRotator true) "1.000000,1.000000,1.000000") "Undefined" "MultiplyWithRoot" 0 0))

(event EventBeginPlay
  (Utilities|Time|SetTimerbyFunctionName 0 "SpawnObjects" (Math|Random|RandomFloatinRange (Variables|Default|GetMin) (Variables|Default|GetMax)) true))

(fn ConstructionScript)