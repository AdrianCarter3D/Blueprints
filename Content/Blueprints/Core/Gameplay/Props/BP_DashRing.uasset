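; BP_DashRing is a dash ring prop that boosts the player when they overlap it.
; On overlap by BP_ThirdPersonCharacter, it moves the character to the ring's location, then launches it with both XY and Z velocity overridden.
; The launch vector adds DashRingPower on X to the ring's forward vector, then rotates the sum by the ring's rotation.
; A booster sound plays at the ring.
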(event Collision|EventActorBeginOverlap
  (params (OtherActor :type Actor%20Object%20Reference))
  (bind _asbp_third_person_character (Utilities|Casting|CastToBP_ThirdPersonCharacter OtherActor))
  ;[0.4323 0.4323 0.4323] Launching player based off the dash rings forward vector and breaking the vector so we can add to that direction
  (Transformation|SetWorldLocation (Variables|/Script/Engine.Actor|GetRootComponent _asbp_third_person_character) (Transformation|GetActorLocation) false false)
  (Character|LaunchCharacter _asbp_third_person_character (Math|Vector|RotateVector (+ (Transformation|GetActorForwardVector) (Math|Vector|MakeVector (Variables|Default|GetDashRingPower) 0.0 0.0)) (Transformation|GetActorRotation)) true true)
  (Audio|PlaySoundatLocation "/Game/Assets/Audio/Sounds/SFX/SE_Ringbooster.SE_Ringbooster" (Transformation|GetActorLocation) "0, 0, 0" 1.0 1.0 0.0 "/Game/Assets/Audio/Attenuation/SoundAttenuation_Normal.SoundAttenuation_Normal" 0 0 0))

(fn ConstructionScript)