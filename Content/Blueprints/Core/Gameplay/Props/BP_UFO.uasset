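; BP_UFO is a spinning UFO prop that moves between its origin and a configurable point and tractor-beams the player upward.
; InterpToMovement gets its path, behaviour and duration in the construction script.
; Entering the Box switches the third-person character to Flying and plays the Tractor timeline, lerping its height toward the mesh while keeping the player's XY.
; Leaving the Box restores Walking and stops the timeline.
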(event OnComponentBeginOverlap(Box)
  (params (OverlappedComponent :type Primitive%20Component%20Object%20Reference) (OtherActor :type Actor%20Object%20Reference) (OtherComp :type Primitive%20Component%20Object%20Reference) (OtherBodyIndex :type Integer) (bFromSweep :type Boolean) (SweepResult :type Hit%20Result%20Structure%20%28by%20ref%29))
  (bind _returnvalue (Game|GetPlayerCharacter 0))
  (bind _returnvalue_2 (Transformation|GetActorLocation _returnvalue))
  (bind _asbp_third_person_character (Utilities|Casting|CastToBP_ThirdPersonCharacter OtherActor))
  (Pawn|Components|CharacterMovement|SetMovementMode (Variables|/Script/Engine.Character|GetCharacterMovement _asbp_third_person_character) "MOVE_Flying" 0)
  (bind _newtrack_0 (Timeline|Tractor PlayFromStart)
    (:Update
      (Transformation|SetActorLocation _asbp_third_person_character (Math|Vector|MakeVector (.x _returnvalue_2) (.y _returnvalue_2) (Math|Float|Lerp (.z (Transformation|GetWorldLocation (Variables|/Script/Engine.Character|GetCapsuleComponent _asbp_third_person_character))) (.z (Transformation|GetWorldLocation (Variables|Default|GetStaticMesh))) _newtrack_0)) false false))))

(event OnComponentEndOverlap(Box)
  (params (OverlappedComponent :type Primitive%20Component%20Object%20Reference) (OtherActor :type Actor%20Object%20Reference) (OtherComp :type Primitive%20Component%20Object%20Reference) (OtherBodyIndex :type Integer))
  (bind _returnvalue (Game|GetPlayerCharacter 0))
  (bind _returnvalue_2 (Transformation|GetActorLocation _returnvalue))
  (bind _asbp_third_person_character (Utilities|Casting|CastToBP_ThirdPersonCharacter OtherActor))
  (Pawn|Components|CharacterMovement|SetMovementMode (Variables|/Script/Engine.Character|GetCharacterMovement _asbp_third_person_character) "MOVE_Walking" 0)
  (bind _newtrack_0 (Timeline|Tractor Stop)
    (:Update
      (Transformation|SetActorLocation (stale OnComponentBeginOverlap(Box) _asbp_third_person_character) (Math|Vector|MakeVector (.x _returnvalue_2) (.y _returnvalue_2) (Math|Float|Lerp (.z (Transformation|GetWorldLocation (Variables|/Script/Engine.Character|GetCapsuleComponent (stale OnComponentBeginOverlap(Box) _asbp_third_person_character)))) (.z (Transformation|GetWorldLocation (Variables|Default|GetStaticMesh))) _newtrack_0)) false false))))

(event EventTick
  (params (DeltaSeconds :type Float%20%28single-precision%29))
  (Transformation|AddRelativeRotation (Variables|Default|GetStaticMesh) (Math|Rotator|MakeRotator 0.0 0.0 (* DeltaSeconds 1e+01)) false false))

(fn ConstructionScript
  (bind _interptomovement (Variables|Default|GetInterpToMovement))
  (Class|InterptoMovementComponent|AddControlPointPosition _interptomovement "0, 0, 0" true)
  (Class|InterptoMovementComponent|AddControlPointPosition _interptomovement (Variables|Default|GetMoveToPosition) true)
  (Variables|/Script/Engine.InterpToMovementComponent|SetBehaviourType _interptomovement (Variables|Default|GetBehaviour%20Type))
  (Variables|/Script/Engine.InterpToMovementComponent|SetDuration _interptomovement (Variables|Default|GetDuration)))