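; BP_Ring10 is a collectible ring prop that adds its CurrencyValue to the third-person character's Currency.
; Its Magnetized event interpolates the ring toward the player, speeding up with player velocity.
; On sphere overlap with the character, it writes the new total into the game instance's save data (zeroing several other PlayerData fields), plays a sound and destroys itself.
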(event OnComponentBeginOverlap(Sphere)
  (params (OverlappedComponent :type Primitive%20Component%20Object%20Reference) (OtherActor :type Actor%20Object%20Reference) (OtherComp :type Primitive%20Component%20Object%20Reference) (OtherBodyIndex :type Integer) (bFromSweep :type Boolean) (SweepResult :type Hit%20Result%20Structure%20%28by%20ref%29))
  (bind _asbp_third_person_character (Utilities|Casting|CastToBP_ThirdPersonCharacter OtherActor))
  ;[0.4323 0.4323 0.4323] Updating the amount of currency we have and setting it to that new value. Then storing it in the game instance that is holding the save game data for if we want to save it
  (bind _output_get (Variables|/Game/ThirdPerson/Blueprints/BP_ThirdPersonCharacter.BP_ThirdPersonCharacter_C|SetCurrency _asbp_third_person_character (+ (Variables|/Game/ThirdPerson/Blueprints/BP_ThirdPersonCharacter.BP_ThirdPersonCharacter_C|GetCurrency _asbp_third_person_character) (Variables|Default|GetCurrencyValue))))
  (Variables|/Game/Blueprints/Saves/BP_SaveGameData.BP_SaveGameData_C|SetPlayerData (Variables|/Game/Blueprints/Instance/BP_GameInstance.BP_GameInstance_C|GetSaveGameData (Variables|Default|GetAs%20BP%20Game%20Instance)) (Utilities|Struct|MakeStructure_PlayerSaveData 0 0 _output_get 0 "0.000000,0.000000,0.000000|0.000000,0.000000,0.000000|1.000000,1.000000,1.000000"))
  (Audio|PlaySoundatLocation "/Game/Assets/Audio/Sounds/SFX/SE_Ring_Mix.SE_Ring_Mix" (Transformation|GetActorLocation) "0, 0, 0" 0.5 1.0 0.0 "/Game/Assets/Audio/Attenuation/SoundAttenuation_Normal.SoundAttenuation_Normal" 0 0 0)
  (Actor|DestroyActor))

(event Custom|Magnetized
  (bind _returnvalue (Game|GetPlayerCharacter 0))
  ;[0.4323 0.4323 0.4323] Ring Attraction
  (Transformation|SetActorLocation (Math|Interpolation|VInterpTo (Transformation|GetActorLocation) (Transformation|GetActorLocation _returnvalue) (Utilities|Time|GetWorldDeltaSeconds) (+ 3.0 (/ (Math|Vector|VectorLength (Transformation|GetVelocity _returnvalue)) 1e+02))) false false))

(event EventBeginPlay
  ;[0.4323 0.4323 0.4323] Obtaining the game instance values so we can save them if we want to. This also helps load the values that were saved if there is a present save file.
  (bind _asbp_game_instance (Utilities|Casting|CastToBP_GameInstance (Game|GetGameInstance)))
  (Variables|Default|SetAs%20BP%20Game%20Instance _asbp_game_instance))

(fn ConstructionScript)