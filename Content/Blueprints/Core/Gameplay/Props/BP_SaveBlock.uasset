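; Save block prop that saves player data through BP_GameInstance whenever BP_ThirdPersonCharacter overlaps its box.
; The Anim_MoveBlock timeline moves the cube vertically by adding its track value as a world Z offset each update.
; The BlockWasHit flag prevents the animation restarting mid-play and clears when it finishes, but saving still runs on every overlap.
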(event OnComponentBeginOverlap(Box)
  (params (OverlappedComponent :type Primitive%20Component%20Object%20Reference) (OtherActor :type Actor%20Object%20Reference) (OtherComp :type Primitive%20Component%20Object%20Reference) (OtherBodyIndex :type Integer) (bFromSweep :type Boolean) (SweepResult :type Hit%20Result%20Structure%20%28by%20ref%29))
  (Utilities|Casting|CastToBP_ThirdPersonCharacter OtherActor)
  (Default|SavePlayerData (Variables|Default|GetAs%20BP%20Game%20Instance))
  (if (Variables|Default|GetBlockWasHit?)
    (Development|PrintString "True")
    (else
      (Variables|Default|SetBlockWasHit? true)
      (bind _newtrack_0 (Timeline|Anim_MoveBlock PlayFromStart)
        (:Update
          (Transformation|AddWorldOffset (Variables|Default|GetCube) (Math|Vector|MakeVector 0.0 0.0 _newtrack_0) false false))
        (:Finished
          (Variables|Default|SetBlockWasHit? false)
          (Development|PrintString "Reset"))))))

(event EventBeginPlay
  (bind _asbp_game_instance (Utilities|Casting|CastToBP_GameInstance (Game|GetGameInstance)))
  (Variables|Default|SetAs%20BP%20Game%20Instance _asbp_game_instance))

(event Collision|EventActorBeginOverlap
  (params (OtherActor :type Actor%20Object%20Reference)))

(event EventTick
  (params (DeltaSeconds :type Float%20%28single-precision%29)))

(fn ConstructionScript)