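; 2D platformer player character that handles health, damage reactions and death.
; Health starts at maximum on BeginPlay; incoming damage, ignored while defeated, lowers it within bounds and destroys the actor at zero.
; Non-lethal hits set a stunned flag, jump the animation instance to its stunned node, stop movement immediately, and clear the flag after a short delay.
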(event EventBeginPlay
  (Variables|Default|SetCurrentHealth (Variables|Default|GetMaxHealth)))

(event Collision|EventActorBeginOverlap
  (params (OtherActor :type Actor%20Object%20Reference)))

(event EventTick
  (params (DeltaSeconds :type Float%20%28single-precision%29)))

(event Game|Damage|EventAnyDamage
  (params (Damage :type Float%20%28single-precision%29) (DamageType :type Damage%20Type%20Object%20Reference) (InstigatedBy :type Controller%20Object%20Reference) (DamageCauser :type Actor%20Object%20Reference))
  (if (not (Variables|Default|GetIsDefeated))
    (Variables|Default|SetCurrentHealth (Math|Integer|Clamp(Integer) (- (Variables|Default|GetCurrentHealth) Damage) 0 (Variables|Default|GetMaxHealth)))
    (if (<= (Variables|Default|GetCurrentHealth) 0)
      (Actor|DestroyActor)
      (else
        (Variables|Default|SetIsStunnned true)
        (Class|PaperZDAnimInstance|JumptoNode (Class|PaperZDCharacter|GetAnimInstance) "Jump Stunned" "None")
        (Components|Movement|StopMovementImmediately (Variables|Character|GetCharacterMovement))
        (Utilities|FlowControl|Delay 0.2)
        (Variables|Default|SetIsStunnned false)))))

(fn ConstructionScript)