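; BP_LevelTransfer is a trigger actor that moves the player to another level when they walk into it.
; When the player character overlaps its Box, it calls FadeInTransitions, disables input and auto-walks the character to the ArrowMoveTo component's location.
; After a short delay it opens the Level reference, passing DestinationTag as the options string.
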(event OnComponentBeginOverlap(Box)
  (params (OverlappedComponent :type Primitive%20Component%20Object%20Reference) (OtherActor :type Actor%20Object%20Reference) (OtherComp :type Primitive%20Component%20Object%20Reference) (OtherBodyIndex :type Integer) (bFromSweep :type Boolean) (SweepResult :type Hit%20Result%20Structure%20%28by%20ref%29))
  (bind _returnvalue (Game|GetPlayerCharacter 0))
  (bind _returnvalue_2 (Game|GetPlayerController 0))
  (if (== OtherActor _returnvalue)
    (CallFunction|FadeinTransitions)
    (Input|DisableInput _returnvalue _returnvalue_2)
    (AI|Navigation|SimpleMovetoLocation _returnvalue_2 (Transformation|GetWorldLocation (Variables|Default|GetArrow_MoveTo)))
    (Utilities|FlowControl|Delay 2.0)
    (Game|OpenLevel(byObjectReference) (Variables|Default|GetLevel) true (Variables|Default|GetDestinationTag))))

(event EventBeginPlay)

(event Collision|EventActorBeginOverlap
  (params (OtherActor :type Actor%20Object%20Reference)))

(event EventTick
  (params (DeltaSeconds :type Float%20%28single-precision%29)))

(fn ConstructionScript)