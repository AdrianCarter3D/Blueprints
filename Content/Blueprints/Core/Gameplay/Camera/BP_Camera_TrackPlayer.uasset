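; Trigger-volume camera that takes over the view and follows the third-person player while they are inside its box.
; On overlap it blends the player controller's view to itself and starts a recursive short-Delay loop that rotates the camera to look at the character.
; Leaving the box blends the view back to the character and stops the loop.
; The construction script sizes the box from an exposed extent variable.
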(event OnComponentBeginOverlap(Box)
  (params (OverlappedComponent :type Primitive%20Component%20Object%20Reference) (OtherActor :type Actor%20Object%20Reference) (OtherComp :type Primitive%20Component%20Object%20Reference) (OtherBodyIndex :type Integer) (bFromSweep :type Boolean) (SweepResult :type Hit%20Result%20Structure%20%28by%20ref%29))
  (bind _asbp_third_person_character (Utilities|Casting|CastToBP_ThirdPersonCharacter OtherActor))
  (Game|Player|SetViewTargetwithBlend (Game|GetPlayerController 0) self 1.0 "VTBlend_Linear" 0.0 false)
  (Variables|Default|SetCanTrack? true)
  (CallFunction|TrackPlayer))

(event OnComponentEndOverlap(Box)
  (params (OverlappedComponent :type Primitive%20Component%20Object%20Reference) (OtherActor :type Actor%20Object%20Reference) (OtherComp :type Primitive%20Component%20Object%20Reference) (OtherBodyIndex :type Integer))
  (bind _asbp_third_person_character (Utilities|Casting|CastToBP_ThirdPersonCharacter OtherActor))
  (Game|Player|SetViewTargetwithBlend (Game|GetPlayerController 0) _asbp_third_person_character 1.0 "VTBlend_Linear" 0.0 false)
  (Variables|Default|SetCanTrack? false))

(event Custom|TrackPlayer
  (if (Variables|Default|GetCanTrack?)
    (Transformation|SetWorldRotation (Variables|Default|GetCamera) (Math|Rotator|FindLookatRotation (Transformation|GetWorldLocation (Variables|Default|GetCamera)) (Transformation|GetActorLocation (stale OnComponentBeginOverlap(Box) _asbp_third_person_character))) false false)
    (Utilities|FlowControl|Delay 0.005)
    (CallFunction|TrackPlayer)))

(fn ConstructionScript
  (Components|Box|SetBoxExtent (Variables|Default|GetBox) (Variables|Default|GetIn%20Box%20Extent) true))