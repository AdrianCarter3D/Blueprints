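; BP_StaticCamera is a trigger volume that switches the player's view to a fixed camera and triggers enemy spawning.
; Entering its Box blends the view to the referenced Camera and, the first time only, calls SpawnEnemy on its Spawners after a delay.
; A looping timer from BeginPlay polls for player overlap, blending to the camera and clearing itself once detected, without spawning.
; Leaving the Box does nothing.
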(event OnComponentBeginOverlap(Box)
  (params (OverlappedComponent :type Primitive%20Component%20Object%20Reference) (OtherActor :type Actor%20Object%20Reference) (OtherComp :type Primitive%20Component%20Object%20Reference) (OtherBodyIndex :type Integer) (bFromSweep :type Boolean) (SweepResult :type Hit%20Result%20Structure%20%28by%20ref%29))
  (if (== OtherActor (Game|GetPlayerCharacter 0))
    (Game|Player|SetViewTargetwithBlend (Game|GetPlayerController 0) (Variables|Default|GetCamera) 1.0 "VTBlend_Linear" 0.0 false)
    (Utilities|FlowControl|DoOnce false
      (:Completed
        (Utilities|FlowControl|Delay 1.0)
        (for _array_element (Variables|Default|GetSpawners)
          (Default|SpawnEnemy _array_element))))))

(event OnComponentEndOverlap(Box)
  (params (OverlappedComponent :type Primitive%20Component%20Object%20Reference) (OtherActor :type Actor%20Object%20Reference) (OtherComp :type Primitive%20Component%20Object%20Reference) (OtherBodyIndex :type Integer))
  (if (== OtherActor (Game|GetPlayerCharacter 0))
    _))

(event Custom|CheckOverlaponInit
  (if (Collision|IsOverlappingActor (Game|GetPlayerCharacter 0) :!class /Script/Engine.Actor)
    (Utilities|Time|ClearandInvalidateTimerbyHandle (Variables|Default|GetCheck%20Overlap%20on%20Inittimer))
    (Game|Player|SetViewTargetwithBlend (Game|GetPlayerController 0) (Variables|Default|GetCamera) 1.0 "VTBlend_Linear" 0.0 false)))

(event EventBeginPlay
  (bind _returnvalue (Utilities|Time|SetTimerbyEvent (EventDispatchers|CreateEvent :!event Custom|CheckOverlaponInit) 0.1 true))
  (Variables|Default|SetCheck%20Overlap%20on%20Inittimer _returnvalue))

(fn ConstructionScript)