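; Spline-rail camera actor that takes over the player's view inside a box volume sized in the construction script.
; Each tick, the spring arm moves to the spline point nearest the player, raised by a third of its arm length.
; It faces perpendicular to the spline direction at a fixed downward pitch.
; Any overlap begin blends the view to this camera; the third-person character leaving blends it back.
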(event OnComponentBeginOverlap(Box)
  (params (OverlappedComponent :type Primitive%20Component%20Object%20Reference) (OtherActor :type Actor%20Object%20Reference) (OtherComp :type Primitive%20Component%20Object%20Reference) (OtherBodyIndex :type Integer) (bFromSweep :type Boolean) (SweepResult :type Hit%20Result%20Structure%20%28by%20ref%29))
  (Game|Player|SetViewTargetwithBlend (Game|GetPlayerController 0) self 1.0 "VTBlend_Linear" 0.0 false))

(event OnComponentEndOverlap(Box)
  (params (OverlappedComponent :type Primitive%20Component%20Object%20Reference) (OtherActor :type Actor%20Object%20Reference) (OtherComp :type Primitive%20Component%20Object%20Reference) (OtherBodyIndex :type Integer))
  (bind _asbp_third_person_character (Utilities|Casting|CastToBP_ThirdPersonCharacter OtherActor))
  (Game|Player|SetViewTargetwithBlend (Game|GetPlayerController 0) _asbp_third_person_character 1.0 "VTBlend_Linear" 0.0 false))

(event EventTick
  (params (DeltaSeconds :type Float%20%28single-precision%29))
  (bind _returnvalue (Game|GetPlayerCharacter 0))
  (bind _spline (Variables|Default|GetSpline))
  (bind _springarm (Variables|Default|GetSpringArm))
  (bind _returnvalue_2 (Transformation|GetActorLocation _returnvalue))
  (bind _returnvalue_3 (Spline|FindLocationClosesttoWorldLocation _spline _returnvalue_2 "World"))
  (Transformation|SetWorldLocation _springarm (Math|Vector|MakeVector (.x _returnvalue_3) (.y _returnvalue_3) (+ (.z _returnvalue_3) (/ (Variables|/Script/Engine.SpringArmComponent|GetTargetArmLength _springarm) 3.0))) false false)
  (Transformation|SetWorldRotation _springarm (Math|Rotator|MakeRotator (.roll (Math|Rotator|FindLookatRotation (Transformation|GetWorldLocation (Variables|Default|GetCamera)) (Transformation|GetActorLocation (Game|GetPlayerCharacter 0)))) -3e+01 (+ (.yaw (Math|Conversions|RotationFromXVector (Spline|FindDirectionClosesttoWorldLocation _spline _returnvalue_2 "World"))) 9e+01)) false false))

(fn ConstructionScript
  (Components|Box|SetBoxExtent (Variables|Default|GetBox) (Variables|Default|GetIn%20Box%20Extent) true))