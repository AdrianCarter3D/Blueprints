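; BP_CameraZone is a trigger volume that switches the player's view to its own camera, for fixed-camera areas in the REHorror game.
; The construction script sizes the box from TriggerArea and places the camera from its location and rotation variables.
; When BP_REHorror_Character enters the box, player controller 0 blends to this actor over CameraBlendTime with the outgoing view locked.
; Leaving the box triggers nothing.
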(event OnComponentBeginOverlap(Box)
  (params (OverlappedComponent :type Primitive%20Component%20Object%20Reference) (OtherActor :type Actor%20Object%20Reference) (OtherComp :type Primitive%20Component%20Object%20Reference) (OtherBodyIndex :type Integer) (bFromSweep :type Boolean) (SweepResult :type Hit%20Result%20Structure%20%28by%20ref%29))
  (Utilities|Casting|CastToBP_REHorror_Character OtherActor)
  (Game|Player|SetViewTargetwithBlend (Game|GetPlayerController 0) self (Variables|Default|GetCameraBlendTime) "VTBlend_Linear" 0.0 true))

(event EventBeginPlay)

(event Collision|EventActorBeginOverlap
  (params (OtherActor :type Actor%20Object%20Reference)))

(event EventTick
  (params (DeltaSeconds :type Float%20%28single-precision%29)))

(fn ConstructionScript
  (Components|Box|SetBoxExtent (Variables|Default|GetBox) (Variables|Default|GetTriggerArea) true)
  (Transformation|SetRelativeLocationAndRotation (Variables|Default|GetCamera) (Variables|Default|GetCameraLocation) (Variables|Default|GetCameraRotation) false false))