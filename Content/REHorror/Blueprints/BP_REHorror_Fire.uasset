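; BP_REHorror_Fire is a fire light actor that simulates flickering firelight with a spot light and a point light.
; On BeginPlay, the FireFlicker timeline plays at a sped-up rate, and its track drives both intensities, with the point light scaled much brighter.
; The construction script applies exposed attenuation radius, color temperature and shadow settings to the spot light only.
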(event EventBeginPlay
  (Components|Timeline|SetPlayRate (Variables|Default|GetFireFlicker) 25.0)
  (bind _newtrack_0 (Timeline|FireFlicker PlayFromStart)
    (:Update
      (Rendering|Components|Light|SetIntensity (Variables|Default|GetSpotLight) (* _newtrack_0 2.0))
      (Rendering|Components|Light|SetIntensity (Variables|Default|GetPointLight) (* (* _newtrack_0 2.0) 12.0)))))

(event Collision|EventActorBeginOverlap
  (params (OtherActor :type Actor%20Object%20Reference)))

(event EventTick
  (params (DeltaSeconds :type Float%20%28single-precision%29)))

(fn ConstructionScript
  (Rendering|Lighting|SetAttenuationRadius (Variables|Default|GetSpotLight) (Variables|Default|GetSpotlight_Atten_Radius))
  (Class|LightComponent|SetTemperature (Variables|Default|GetSpotLight) (Variables|Default|GetLights_Temperature))
  (Rendering|Components|Light|SetCastShadows (Variables|Default|GetSpotLight) (Variables|Default|GetSpotlight_Shadow)))