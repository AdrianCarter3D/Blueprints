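; BP_REHorror_WallLight is a wall light for the REHorror game that can be configured per instance.
; The construction script applies variables for attenuation radius, temperature, shadow casting and intensity to its SpotLight component.
; A point-light attenuation node is left unconnected, so that setting has no effect here.
; The event graph holds only disabled placeholder events, so the Blueprint adds no runtime logic.
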(event EventBeginPlay)

(event Collision|EventActorBeginOverlap
  (params (OtherActor :type Actor%20Object%20Reference)))

(event EventTick
  (params (DeltaSeconds :type Float%20%28single-precision%29)))

(fn ConstructionScript
  (Rendering|Lighting|SetAttenuationRadius (Variables|Default|GetSpotLight) (Variables|Default|GetSpotlight_Atten_Radius))
  (Class|LightComponent|SetTemperature (Variables|Default|GetSpotLight) (Variables|Default|GetLights_Temperature))
  (Rendering|Components|Light|SetCastShadows (Variables|Default|GetSpotLight) (Variables|Default|GetSpotlight_Shadow))
  (Rendering|Components|Light|SetIntensity (Variables|Default|GetSpotLight) (Variables|Default|GetSpotlight_Intensity)))