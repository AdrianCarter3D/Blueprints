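; Interactable horror-game puzzle statue that turns a quarter turn around its yaw axis each time it is used.
; OnUsed passes a DoOnce gate, cycles RotationIndex through four states and plays the StatuePuzzle timeline to lerp the rotation.
; When the turn finishes, it stores the new rotation, asks GlassCasePrize to check the solution and resets the gate for the next use.
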(event EventBeginPlay
  (|CallParentFunction) ; This node is disabled and will not be called.\nDrag off pins to build functionality.
)

(event Collision|EventActorBeginOverlap
  (params (OtherActor :type Actor%20Object%20Reference))
  (|CallParentFunction OtherActor) ; This node is disabled and will not be called.\nDrag off pins to build functionality.
)

(event EventTick
  (params (DeltaSeconds :type Float%20%28single-precision%29))
  (|CallParentFunction DeltaSeconds) ; This node is disabled and will not be called.\nDrag off pins to build functionality.
)

(event EventOnUsed
  (params (Player :type BP%20RE%20Horror%20Character%20Object%20Reference))
  (Utilities|FlowControl|DoOnce false :!label _label
    (:Completed
      (switch int (Variables|Default|GetRotationIndex)
        (:0
          (Variables|Default|SetRotationIndex 1)
          (bind _rotate (Timeline|StatuePuzzle PlayFromStart)
            (:Update
              (Transformation|SetActorRotation (Math|Rotator|Lerp(Rotator) (Variables|Default|GetCurrentRotation) (Math|Rotator|MakeRotator (.Roll (Math|Rotator|BreakRotator (Variables|Default|GetCurrentRotation))) (.Pitch (Math|Rotator|BreakRotator (Variables|Default|GetCurrentRotation))) (+ (.Yaw (Math|Rotator|BreakRotator (Variables|Default|GetCurrentRotation))) 9e+01)) _rotate true)))
            (:Finished
              (Utilities|FlowControl|Sequence
                (:then_0
                  (Variables|Default|SetCurrentRotation (Transformation|GetActorRotation))
                  (Default|EventCheckSoluation (Variables|Default|GetGlassCase_Prize)))
                (:then_1
                  (goto _label Reset))))))
        (:1
          (Variables|Default|SetRotationIndex 2)
          (Timeline|StatuePuzzle PlayFromStart))
        (:2
          (Variables|Default|SetRotationIndex 3)
          (Timeline|StatuePuzzle PlayFromStart))
        (:3
          (Variables|Default|SetRotationIndex 0)
          (Timeline|StatuePuzzle PlayFromStart))))))

(fn ConstructionScript
  (|CallParentFunction))