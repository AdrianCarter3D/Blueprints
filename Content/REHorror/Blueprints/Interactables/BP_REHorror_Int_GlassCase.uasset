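; BP_REHorror_Int_GlassCase is a glass case that acts as the barrier for a statue rotation puzzle.
; Its Event_CheckSoluation event compares the RotationIndex of three referenced statues against a hard-coded combination.
; When all three match, the case destroys itself; it has no active BeginPlay, overlap or Tick logic, so the check relies on that event being called.
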(event Custom|Event_CheckSoluation
  (if (Math|Boolean|ANDBoolean (== (Variables|/Game/REHorror/Blueprints/Interactables/BP_REHorror_Int_Statue.BP_REHorror_Int_Statue_C|GetRotationIndex (Variables|Default|GetStatue1)) 1) (== (Variables|/Game/REHorror/Blueprints/Interactables/BP_REHorror_Int_Statue.BP_REHorror_Int_Statue_C|GetRotationIndex (Variables|Default|GetStatue2)) 2) (== (Variables|/Game/REHorror/Blueprints/Interactables/BP_REHorror_Int_Statue.BP_REHorror_Int_Statue_C|GetRotationIndex (Variables|Default|GetStatue3)) 3))
    (Actor|DestroyActor)))

(event EventBeginPlay
  (|CallParentFunction) ; This node is disabled and will not be called.\nDrag off pins to build functionality.
)

(event Collision|EventActorBeginOverlap
  (params (OtherActor :type Actor%20Object%20Reference))
  (|CallParentFunction OtherActor) ; This node is disabled and will not be called.\nDrag off pins to build functionality.
)

(event EventTick
  (params (DeltaSeconds :type Float%20%28single-precision%29))
  (|CallParentFunction DeltaSeconds) ; This node is disabled and will not be called.\nDrag off pins to build functionality.
)

(fn ConstructionScript
  (|CallParentFunction))