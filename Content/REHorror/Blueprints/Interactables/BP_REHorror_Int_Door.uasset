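; Interactable door for the REHorror game that teleports the player to its Arrow component behind a door-transition cutaway, with an optional key lock.
; On use, a required key is looked up in the items DataTable and checked against player inventory, either clearing the lock or showing a locked message.
; A DoOnce-guarded sequence fades the HUD, views a temporary transition actor spawned high above origin, waits, moves the player, then destroys it.
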(event EventBeginPlay
  (|CallParentFunction) ; This node is disabled and will not be called.\nDrag off pins to build functionality.
)

(event Collision|EventActorBeginOverlap
  (params (OtherActor :type Actor%20Object%20Reference))
  (|CallParentFunction OtherActor) ; This node is disabled and will not be called.\nDrag off pins to build functionality.
)

(event EventTick
  (params (DeltaSeconds :type Float%20%28single-precision%29))
  (|CallParentFunction DeltaSeconds) ; This node is disabled and will not be called.\nDrag off pins to build functionality.
)

(event EventOnUsed
  (params (Player :type BP%20RE%20Horror%20Character%20Object%20Reference))
  (bind _arrow (Variables|Default|GetArrow))
  (if (Variables|Door|GetRequiresKey?)
    (bind _returnvalue (Utilities|GetDataTableRow "/Game/REHorror/Core/DataTables/DT_REHorror_Items.DT_REHorror_Items" (Variables|Door|GetKeyItem))
      (:then
        (if (Utilities|Array|ContainsItem (Variables|/Game/REHorror/Blueprints/BP_REHorror_Character.BP_REHorror_Character_C|GetArray_Inventory Player) _returnvalue)
          (Variables|Door|SetRequiresKey? false)
          (Utilities|FlowControl|DoOnce false :!label _label
            (:Completed
              (Default|EventPlayBlackFadeinOut (Variables|/Game/REHorror/Blueprints/BP_REHorror_Character.BP_REHorror_Character_C|GetUI_HUD Player))
              (bind _returnvalue_2 (Game|SpawnActorfromClass "/Game/REHorror/Blueprints/Interactables/BP_REHorror_DoorTransition.BP_REHorror_DoorTransition_C" (Math|Transform|MakeTransform "0.000000,0.000000,20000.000000") "Undefined" "MultiplyWithRoot" 0 0))
              (Game|Player|SetViewTargetwithBlend (Game|GetPlayerController 0) _returnvalue_2 0.0 "VTBlend_Linear" 0.0 false)
              (Utilities|FlowControl|Delay 5.0)
              (Transformation|SetActorLocationAndRotation Player (Transformation|GetWorldLocation _arrow) (Variables|/Script/Engine.SceneComponent|GetRelativeRotation _arrow))
              (Default|EventPlayBlackFadeinOut (Variables|/Game/REHorror/Blueprints/BP_REHorror_Character.BP_REHorror_Character_C|GetUI_HUD Player))
              (Actor|DestroyActor _returnvalue_2)
              (goto _label Reset)))
          (else
            _)))
      (:RowNotFound
        _))
    (Default|EventShowText Player "It's locked...")
    (else
      (goto _label))))

(fn ConstructionScript
  (|CallParentFunction))