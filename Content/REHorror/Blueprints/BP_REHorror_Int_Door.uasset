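; BP_REHorror_Int_Door is an interactable door that moves the player behind a Resident Evil-style door transition.
; On OnUsed, it spawns a BP_REHorror_DoorTransition actor high above the world origin and switches player 0's view target to it.
; After a fixed five-second delay, it teleports the player to the Arrow component's world location, using that Arrow's relative rotation, then destroys the transition actor.
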(event EventBeginPlay
  (|CallParentFunction) ; This node is disabled and will not be called.\nDrag off pins to build functionality.
)

(event Collision|EventActorBeginOverlap
  (params (OtherActor :type Actor%20Object%20Reference))
  (|CallParentFunction OtherActor) ; This node is disabled and will not be called.\nDrag off pins to build functionality.
)

(event EventTick
  (params (DeltaSeconds :type Float%20%28single-precision%29))
  (|CallParentFunction DeltaSeconds) ; This node is disabled and will not be called.\nDrag off pins to build functionality.
)

(event EventOnUsed
  (params (Player :type BP%20RE%20Horror%20Character%20Object%20Reference))
  (bind _arrow (Variables|Default|GetArrow))
  (bind _returnvalue (Game|SpawnActorfromClass "/Game/REHorror/Blueprints/BP_REHorror_DoorTransition.BP_REHorror_DoorTransition_C" (Math|Transform|MakeTransform "0.000000,0.000000,20000.000000") "Undefined" "MultiplyWithRoot" 0 0))
  (Game|Player|SetViewTargetwithBlend (Game|GetPlayerController 0) _returnvalue 0.0 "VTBlend_Linear" 0.0 false)
  (Utilities|FlowControl|Delay 5.0)
  (Transformation|SetActorLocationAndRotation Player (Transformation|GetWorldLocation _arrow) (Variables|/Script/Engine.SceneComponent|GetRelativeRotation _arrow))
  (Actor|DestroyActor _returnvalue))

(fn ConstructionScript
  (|CallParentFunction))