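; BP_Hero is the player character, supporting free planar movement and a side-scroller mode that drops depth movement and enables jumping.
; Enhanced Input drives movement, which switches to Flying on ladders and records facing direction.
; Attacks play a PaperZD animation override, block movement until it ends, and damage actors overlapping the hitbox matching that direction.
; SavePlayerLocation re-calls itself each second, storing grounded positions in the GameInstance as SafeLocation.
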(event Custom|SavePlayerLocation
  (if (AI|Components|NavMovement|IsFalling (Variables|Character|GetCharacterMovement))
    _
    (else
      (bind _asbp_game_instance (Utilities|Casting|CastToBP_GameInstance (Game|GetGameInstance)))
      (Variables|/Game/Common/Blueprints/Instance/BP_GameInstance.BP_GameInstance_C|SetSafeLocation _asbp_game_instance (Transformation|GetActorLocation))))
  (Utilities|FlowControl|Delay 1.0)
  (CallFunction|SavePlayerLocation))

(event Input|EnhancedActionEvents|EnhancedInputActionIA_Move
  (params (ActionValue :type Vector%202D%20Structure) (ElapsedSeconds :type Float%20%28double-precision%29) (TriggeredSeconds :type Float%20%28double-precision%29) (InputAction :type Input%20Action%20Object%20Reference :default "/Game/Common/Blueprints/Input/Actions/IA_Move.IA_Move"))
  (:Triggered
    (if (not (Variables|Default|GetIsAttacking?))
      (Pawn|Input|AddMovementInput "1.000000,0.000000,0.000000" (.x ActionValue) false)
      (if (Variables|Default|GetSideScrollerMode?)
        _
        (else
          (Pawn|Input|AddMovementInput "0.000000,-1.000000,0.000000" (.y ActionValue) false)))
      (Variables|Default|SetDirectionality (Math|Vector2D|MakeVector2D (.x ActionValue) (.y ActionValue)))
      (if (Variables|Default|GetOnLadder)
        (Pawn|Components|CharacterMovement|SetMovementMode (Variables|Character|GetCharacterMovement) "MOVE_Flying" 0)
        (Pawn|Input|AddMovementInput (Transformation|GetActorUpVector (Game|GetPlayerCharacter 0)) 1.0 false)))))

(event Input|EnhancedActionEvents|EnhancedInputActionIA_Attack
  (params (ActionValue :type Boolean) (ElapsedSeconds :type Float%20%28double-precision%29) (TriggeredSeconds :type Float%20%28double-precision%29) (InputAction :type Input%20Action%20Object%20Reference :default "/Game/Common/Blueprints/Input/Actions/IA_Attack.IA_Attack"))
  (bind _directionality (Variables|Default|GetDirectionality))
  (bind (_x _y) (Math|Vector2D|BreakVector2D _directionality))
  (:Started
    (if (not (Variables|Default|GetIsAttacking?))
      (Audio|PlaySound2D 0 1.0 1.0 0.0 0 0)
      (Audio|PlaySound2D 0 1.0 1.0 0.0 0 0)
      (|PlayAnimationOverridewithCallbacks (Class|PaperZDCharacter|GetAnimInstance) "/Game/MythOfLegndrule/PaperZD/Attack.Attack" "DefaultSlot" 1.0 0.0
        (:then
          (Variables|Default|SetIsAttacking? true)
          (if (> (Math|Float|Absolute(Float) _x) (Math|Float|Absolute(Float) _y)) ; are we doing x or y movement?
            (if (> _x 0.0) ; are we going left or right
              (for _array_element (Collision|GetOverlappingActors (Variables|Default|GetHitBox_AttackRight) 0 :!class /Script/Engine.PrimitiveComponent)
                (Game|Damage|ApplyDamage _array_element (Math|Conversions|ToFloat(Integer) (Variables|Default|GetDamage)) 0 0))
              (else
                (for _array_element_2 (Collision|GetOverlappingActors (Variables|Default|GetHitBox_AttackLeft) 0 :!class /Script/Engine.PrimitiveComponent)
                  (Game|Damage|ApplyDamage _array_element_2 (Math|Conversions|ToFloat(Integer) (Variables|Default|GetDamage)) 0 0))))
            (elif (not (Variables|Default|GetSideScrollerMode?))
              (if (> _y 0.0) ; are we going up or down
                (for _array_element_3 (Collision|GetOverlappingActors (Variables|Default|GetHitBox_AttackForward) 0 :!class /Script/Engine.PrimitiveComponent)
                  (Game|Damage|ApplyDamage _array_element_3 (Math|Conversions|ToFloat(Integer) (Variables|Default|GetDamage)) 0 0))
                (else
                  (for _array_element_4 (Collision|GetOverlappingActors (Variables|Default|GetHitBox_AttackBack) 0 :!class /Script/Engine.PrimitiveComponent)
                    (Game|Damage|ApplyDamage _array_element_4 (Math|Conversions|ToFloat(Integer) (Variables|Default|GetDamage)) 0 0)))))))
        (:OnCompleted
          (Variables|Default|SetIsAttacking? false :!label _label))
        (:OnCancelled
          (goto _label))))))

(event Input|EnhancedActionEvents|EnhancedInputActionIA_Jump
  (params (ActionValue :type Boolean) (ElapsedSeconds :type Float%20%28double-precision%29) (TriggeredSeconds :type Float%20%28double-precision%29) (InputAction :type Input%20Action%20Object%20Reference :default "/Game/Common/Blueprints/Input/Actions/IA_Jump.IA_Jump"))
  (:Triggered
    (if (Variables|Default|GetSideScrollerMode?)
      (Character|Jump)))
  (:Completed
    (Character|StopJumping)))

(event EventBeginPlay
  (bind _asplayer_controller_hero (Utilities|Casting|CastToPlayerController_Hero (Pawn|GetController)))
  (Input|AddMappingContext (PlayerController|LocalPlayerSubsystems|GetEnhancedInputLocalPlayerSubsystem _asplayer_controller_hero) "/Game/Common/Blueprints/Input/InputMappingContext_Hero.InputMappingContext_Hero" 0 "(bIgnoreAllPressedKeysUntilRelease=True,bForceImmediately=False)")
  (Variables|Default|SetCurrentHealth (Variables|Default|GetMaxHealth)))

(event EventOnWalkingOffLedge
  (params (PreviousFloorImpactNormal :type Vector%20%28by%20ref%29 :default "0, 0, 0") (PreviousFloorContactNormal :type Vector%20%28by%20ref%29 :default "0, 0, 0") (PreviousLocation :type Vector%20%28by%20ref%29 :default "0, 0, 0") (TimeDelta :type Float%20%28single-precision%29)))

(event EventOnJumped)

(fn ConstructionScript)