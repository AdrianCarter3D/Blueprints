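; Player health component that drives a heart-based health widget, created on BeginPlay in every level except the opening one.
; Initialize, add-heart, damage and heal calls forward to the widget, which reports whether damage is fatal.
; Damage halts player movement; death also disables it, fires the death dispatcher and shows the Game Over widget with UI-only input.
; HealCall ignores its HealAmount input and passes zero.
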(event EventBeginPlay
  (bind _returnvalue (Game|GetCurrentLevelName true))
  (if (not (Utilities|Enum|Equal(Enum) _returnvalue "Level_TheMythOfLegndrule_Opening"))
    (bind _returnvalue_2 (UserInterface|CreateWidget "/Game/MythOfLegndrule/Widgets/Menus/Widget_Health.Widget_Health_C"))
    (bind _output_get (Variables|Default|SetWidgetHeatlhRef _returnvalue_2))
    (UserInterface|Viewport|AddtoViewport _output_get 0)
    (CallFunction|InitializeHealth)))

(event EventTick
  (params (DeltaSeconds :type Float%20%28single-precision%29)))

(fn InitializeHealth
  (Default|InitialiseHealth (Variables|Default|GetWidgetHeatlhRef) (Variables|Default|GetDefaultHeartCount) (Variables|Default|GetMaxHeartHealth) (Variables|Default|GetMaxHeartsPerRow)))

(fn AddHeartCall
  (Default|AddHeart (Variables|Default|GetWidgetHeatlhRef) (Variables|Default|GetFillHeartOnHeartContainer) (Variables|Default|GetMaxHeartsPerRow))
  (return false))

(fn DamageCall
  (params (Damage :type Integer))
  (bind _returnvalue (Game|GetPlayerController 0))
  (bind _returnvalue_2 (Game|GetPlayerCharacter 0))
  (bind _charactermovement (Variables|/Script/Engine.Character|GetCharacterMovement _returnvalue_2))
  (bind _bdied (Default|TakeDamage (Variables|Default|GetWidgetHeatlhRef) Damage (Variables|Default|GetMaxHeartHealth)))
  (if (not _bdied)
    (Components|Movement|StopMovementImmediately (Variables|/Script/Engine.Character|GetCharacterMovement (Game|GetPlayerCharacter 0)))
    (return false)
    (else
      (Development|PrintString "Dead")
      (Components|Movement|StopMovementImmediately _charactermovement)
      (Pawn|Components|CharacterMovement|DisableMovement _charactermovement)
      (Default|CallEventDispatcherDeath)
      (bind _returnvalue_3 (UserInterface|CreateWidget "/Game/MythOfLegndrule/Widgets/Menus/WBP_GameOver.WBP_GameOver_C"))
      (UserInterface|Viewport|AddtoViewport _returnvalue_3 0)
      (Variables|/Script/Engine.PlayerController|SetbShowMouseCursor _returnvalue true)
      (Input|SetInputModeUIOnly _returnvalue _returnvalue_3 "DoNotLock" false))))

(fn HealCall
  (params (HealAmount :type Integer))
  (Default|Heal (Variables|Default|GetWidgetHeatlhRef) 0 (Variables|Default|GetMaxHeartHealth))
  (return false))